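; Anim notify that force-destroys a spawned keyblade pawn belonging to the animated character.
; A macro scans all SpawnKeyblade_Pawn actors for the first whose ActorLabel matches the notify's label and whose PawnOwner is the mesh's owning TresCharPawnBase.
; A match is destroyed immediately, otherwise nothing happens, and the notify returns false either way.
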(fn ReceivedNotify
  (params (MeshComp :type Skeletal%20Mesh%20Component%20Object%20Reference) (Animation :type Anim%20Sequence%20Base%20Object%20Reference))
  (|SpawnKeybladePawnCheck MeshComp
    (:Match!
      (LocalVariables|SetOwner (.AsTres%20Char%20Pawn%20Base (Utilities|Casting|CastToTresCharPawnBase (Components|GetOwner MeshComp))))
      (Default|DESTROY (LocalVariables|GetTargetPawn))
      (return false))
    (:False
      (return false))))