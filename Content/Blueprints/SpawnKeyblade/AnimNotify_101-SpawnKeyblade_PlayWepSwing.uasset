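; Anim notify that plays a swing sound on a spawned Keyblade weapon during a character animation.
; It searches all SpawnKeyblade_Pawn actors for one whose ActorLabel matches and whose PawnOwner is the animated mesh's owner.
; On a match, it attaches the SwingID-selected sound from the weapon's swing assets to its mesh, forcing playback if needed.
; Both match and failure paths show on-screen debug messages through TresUIOpenInformation.
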(fn ReceivedNotify
  (params (MeshComp :type Skeletal%20Mesh%20Component%20Object%20Reference) (Animation :type Anim%20Sequence%20Base%20Object%20Reference))
  (bind _targetpawn (LocalVariables|GetTargetPawn))
  (bind _swing_id (Variables|Default|GetSwing%20ID))
  (bind _returnvalue (Math|Byte|MakeLiteralByte _swing_id))
  (bind _spawnedweapon (Variables|/Game/Blueprints/SpawnKeyblade/ACTOR/SpawnKeyblade_Pawn.SpawnKeyblade_Pawn_C|GetSpawnedWeapon _targetpawn))
  (bind _returnvalue_2 (Math|Conversions|ToInteger(Byte) _returnvalue))
  (bind _m_soundassets_swing (Variables|/Script/TresGame.TresWeaponBase|Getm_SoundAssets_Swing _spawnedweapon))
  (bind _references (Variables|/Script/SQEXSEAD.SQEXSEADSoundReferenceEnumSet|GetReferences _m_soundassets_swing))
  (bind _output (Utilities|Array|Get(acopy) _references _returnvalue_2))
  (bind (_sound _bfollow _attachpointname) (Utilities|Struct|BreakSQEXSEADSoundReference _output))
  (|SpawnKeybladePawnCheck MeshComp
    (:Match!
      (LocalVariables|SetOwner (.AsTres%20Char%20Pawn%20Base (Utilities|Casting|CastToTresCharPawnBase (Components|GetOwner MeshComp))))
      (bind _returnvalue_3 (Audio|SpawnSoundAttached _sound (Variables|/Script/TresGame.TresWeaponBase|GetMyMesh (Variables|/Game/Blueprints/SpawnKeyblade/ACTOR/SpawnKeyblade_Pawn.SpawnKeyblade_Pawn_C|GetSpawnedWeapon (LocalVariables|GetTargetPawn))) _attachpointname "0, 0, 0" "0, 0, 0" "SnapToTargetIncludingScale" true (Variables|Default|GetVolume) (Variables|Default|GetPitch)))
      (if (Audio|Components|Audio|IsPlaying _returnvalue_3)
        _
        (else
          (Audio|Components|Audio|Play _returnvalue_3 0.0)))
      (Class|TresGameBlueprintLibrary|TresUIOpenInformation (Utilities|Struct|MakeTresLocText (Utilities|String|ToString(Text) (Utilities|Text|FormatText "Sound Valid: {V} || Playing? {P} || {Name}" (Utilities|Text|ToText(Boolean) (Utilities|IsValid _sound)) (Utilities|Text|ToText(Boolean) (Audio|Components|Audio|IsPlaying _returnvalue_3)) (Utilities|Text|ToText(String) (Utilities|GetDisplayName _sound))))) true 5.0)
      (return false))
    (:False
      (Class|TresGameBlueprintLibrary|TresUIOpenInformation (Utilities|Struct|MakeTresLocText (Utilities|String|ToString(Text) (Utilities|Text|FormatText "What do you MEAN, still false!?!"))) true 2.0)
      (return false))))