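; Anim notify state that spawns a SpawnKeyblade_Pawn to provide a configurable Keyblade weapon during an animation.
; On begin, it searches existing helper pawns for a matching ActorLabel, then either skips spawning or destroys the older one, per the duplicate setting.
; It spawns the pawn via SpawnAIFromClass, tags it, copies in the owner, notify duration, socket, visibility, FX, material and lifetime settings, then calls START.
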(fn ReceivedNotifyBegin
  (params (MeshComp :type Skeletal%20Mesh%20Component%20Object%20Reference) (Animation :type Anim%20Sequence%20Base%20Object%20Reference) (TotalDuration :type Float%20%28single-precision%29))
  (LocalVariables|SetMesh MeshComp)
  (LocalVariables|SetOwner (.AsTres%20Char%20Pawn%20Base (Utilities|Casting|CastToTresCharPawnBase (Components|GetOwner MeshComp))))
  (bind _outactors (Actor|GetAllActorsOfClass MeshComp "/Game/Blueprints/SpawnKeyblade/ACTOR/SpawnKeyblade_Pawn.SpawnKeyblade_Pawn_C"))
  (for _array_element _outactors
    (if (Utilities|Name|Equal(Name) (Variables|/Game/Blueprints/SpawnKeyblade/ACTOR/SpawnKeyblade_Pawn.SpawnKeyblade_Pawn_C|GetActor%20-%20Label _array_element) (Variables|Default|GetActor%20-%20Label))
      (switch Utilities|FlowControl|Switch|SwitchonSpawnKeyblade_OnCopyDetectedSetting (Variables|Default|GetActor%20-%20Duplicate%20Setting)
        (:NewEnumerator0
          (LocalVariables|SetIS-Copy true))
        (:NewEnumerator1
          (Default|DESTROY _array_element)))))
  (if (LocalVariables|GetIS-Copy)
    _
    (else
      (bind _returnvalue (AI|SpawnAIFromClass MeshComp "/Game/Blueprints/SpawnKeyblade/ACTOR/SpawnKeyblade_Pawn.SpawnKeyblade_Pawn_C" 0 "0, 0, 0" "0, 0, 0" false))
      (Variables|/Script/Engine.Actor|SetTags _returnvalue (Utilities|Array|MakeArray (Variables|Default|GetActor%20-%20Label)))
      (bind _asspawn_keyblade_pawn (Utilities|Casting|CastToSpawnKeyblade_Pawn _returnvalue))
      (|SetVariables _asspawn_keyblade_pawn TotalDuration)
      (Default|START _asspawn_keyblade_pawn)))
  (return false))