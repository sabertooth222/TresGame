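; Anim notify state that spawns particle effects on a spawned Keyblade's weapon mesh during an animation.
; Begin and End find the SpawnKeyblade_Pawn matching the actor label and the mesh's owning pawn.
; Begin attaches each configured effect with transform, speed and optional color, recording only those detached on spawn in the pawn's arrays.
; End looks up every effect's template there and destroys the first matching component, without removing array entries.
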(fn ReceivedNotifyBegin
  (params (MeshComp :type Skeletal%20Mesh%20Component%20Object%20Reference) (Animation :type Anim%20Sequence%20Base%20Object%20Reference) (TotalDuration :type Float%20%28single-precision%29))
  (bind _targetpawn (LocalVariables|GetTargetPawn))
  (|SpawnKeybladePawnCheck_3 MeshComp
    (:Match!
      (for _array_element (Variables|Default|GetAttachEffects)
        (bind _returnvalue (Class|GameplayStatics|SqExSpawnEmitterAttached (.Effect (Utilities|Struct|BreakSpawnKeyblade_FXTemplate-Struct _array_element)) (Variables|/Script/TresGame.TresWeaponBase|GetMyMesh (Variables|/Game/Blueprints/SpawnKeyblade/ACTOR/SpawnKeyblade_Pawn.SpawnKeyblade_Pawn_C|GetSpawnedWeapon (LocalVariables|GetTargetPawn))) (.AttachSocket (Utilities|Struct|BreakSpawnKeyblade_FXTemplate-Struct _array_element)) (.Location (Utilities|Struct|BreakSpawnKeyblade_FXTemplate-Struct _array_element)) (.Rotation (Utilities|Struct|BreakSpawnKeyblade_FXTemplate-Struct _array_element)) 0 "KeepRelativeOffset" false 0.0))
        (Transformation|SetRelativeScale3D _returnvalue (.Scale (Utilities|Struct|BreakSpawnKeyblade_FXTemplate-Struct _array_element)))
        (Variables|/Script/Engine.ParticleSystemComponent|SetCustomTimeDilation _returnvalue (.Speed (Utilities|Struct|BreakSpawnKeyblade_FXTemplate-Struct _array_element)))
        (if (.ChangeColor? (Utilities|Struct|BreakSpawnKeyblade_FXTemplate-Struct _array_element))
          (for _array_element_2 (Variables|/Script/Engine.ParticleSystemComponent|GetInstanceParameters _returnvalue)
            (Utilities|Struct|SetmembersinParticleSysParam _array_element_2 (.NewColor (Utilities|Struct|BreakSpawnKeyblade_FXTemplate-Struct _array_element)))))
        (if (.DetachonSpawn? (Utilities|Struct|BreakSpawnKeyblade_FXTemplate-Struct _array_element))
          (Transformation|DetachFromComponent _returnvalue "KeepRelative" "KeepRelative" "KeepRelative" true)
          (Utilities|Array|Add (Variables|/Game/Blueprints/SpawnKeyblade/ACTOR/SpawnKeyblade_Pawn.SpawnKeyblade_Pawn_C|GetExternalSpawnedFX _targetpawn) _returnvalue)
          (Utilities|Array|Add (Variables|/Game/Blueprints/SpawnKeyblade/ACTOR/SpawnKeyblade_Pawn.SpawnKeyblade_Pawn_C|GetExternalSpawnedFX_ParticleTemplates _targetpawn) (.Effect (Utilities|Struct|BreakSpawnKeyblade_FXTemplate-Struct _array_element)))))
      (return false))
    (:False
      (return false))))

(fn ReceivedNotifyEnd
  (params (MeshComp :type Skeletal%20Mesh%20Component%20Object%20Reference) (Animation :type Anim%20Sequence%20Base%20Object%20Reference))
  (bind _targetpawn (LocalVariables|GetTargetPawn))
  (|SpawnKeybladePawnCheck_2 MeshComp
    (:Match!
      (for _array_element (Variables|Default|GetAttachEffects)
        (Components|DestroyComponent (Utilities|Array|Get(acopy) (Variables|/Game/Blueprints/SpawnKeyblade/ACTOR/SpawnKeyblade_Pawn.SpawnKeyblade_Pawn_C|GetExternalSpawnedFX _targetpawn) (Utilities|Array|FindItem (Variables|/Game/Blueprints/SpawnKeyblade/ACTOR/SpawnKeyblade_Pawn.SpawnKeyblade_Pawn_C|GetExternalSpawnedFX_ParticleTemplates _targetpawn) (.Effect (Utilities|Struct|BreakSpawnKeyblade_FXTemplate-Struct _array_element)))) _targetpawn))
      (return false))
    (:False
      (return false))))