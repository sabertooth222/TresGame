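; Anim notify state that shows weapon trails on a spawned Keyblade pawn during an animation window.
; Macros scan all SpawnKeyblade_Pawn actors for one matching ActorLabel and the mesh's owner, caching it as TargetPawn.
; Begin starts TRAILFX between the vfx_top and vfx_bottom sockets, and End stops it.
; Tick retries the lookup and also ends trails when the stored animation name, set to "None", differs from the owner's last played one.
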(fn ReceivedNotifyBegin
  (params (MeshComp :type Skeletal%20Mesh%20Component%20Object%20Reference) (Animation :type Anim%20Sequence%20Base%20Object%20Reference) (TotalDuration :type Float%20%28single-precision%29))
  (|SpawnKeybladePawnCheck_3 MeshComp
    (:Match!
      (Effects|Particles|Trails|BeginTrails (Variables|/Game/Blueprints/SpawnKeyblade/ACTOR/SpawnKeyblade_Pawn.SpawnKeyblade_Pawn_C|GetTRAILFX (LocalVariables|GetTargetPawn)) "vfx_top" "vfx_bottom" "ETrailWidthMode_FromFirst" 1.0)
      (return false))
    (:False
      (return false))))

(fn ReceivedNotifyEnd
  (params (MeshComp :type Skeletal%20Mesh%20Component%20Object%20Reference) (Animation :type Anim%20Sequence%20Base%20Object%20Reference))
  (|SpawnKeybladePawnCheck_2 MeshComp
    (:Match!
      (Effects|Particles|Trails|EndTrails (Utilities|Array|Get(acopy) (Variables|/Game/Blueprints/SpawnKeyblade/ACTOR/SpawnKeyblade_Pawn.SpawnKeyblade_Pawn_C|GetTRAILFX (LocalVariables|GetTargetPawn))))
      (return false))
    (:False
      (return false))))

(fn ReceivedNotifyTick
  (params (MeshComp :type Skeletal%20Mesh%20Component%20Object%20Reference) (Animation :type Anim%20Sequence%20Base%20Object%20Reference) (FrameDeltaTime :type Float%20%28single-precision%29))
  (Utilities|FlowControl|Sequence
    (:then_0
      (if (or (not (LocalVariables|GetIS-MATCH)) (not (LocalVariables|GetIS-GETALLDONE)))
        (|SpawnKeybladePawnCheck_2 MeshComp
          (:False
            (return false)))))
    (:then_1
      (if (and (LocalVariables|GetIS-GETALLDONE) (LocalVariables|GetIS-MATCH))
        (if (Utilities|Name|NotEqual(Name) (LocalVariables|GetGetAnimName) (Class|TresCharPawnBase|AnimGetLastPlayAnimName (.AsTres%20Char%20Pawn%20Base (Utilities|Casting|CastToTresCharPawnBase (Components|GetOwner MeshComp))) "None"))
          (Effects|Particles|Trails|EndTrails (Variables|/Game/Blueprints/SpawnKeyblade/ACTOR/SpawnKeyblade_Pawn.SpawnKeyblade_Pawn_C|GetTRAILFX (LocalVariables|GetTargetPawn)))
          (return false))))))