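; Goofy shotlock actor: when Sora's Guard animation plays, it freezes all enemies and drops Goofy from above the lock-on target.
; Tick finds or spawns Goofy, who gets a falling animset, capsule collision, lowered gravity and a GoofShotlock blackboard flag.
; His first actor overlap restores animations, gravity and enemy time, then destroys him if spawned.
; The animation swap overwrites the shared animset entries, using a saved copy to restore them.
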(event Custom|GoofyFall
  (bind _returnvalue (Class|TresGameBlueprintLibrary|GetTresPlayerControllerBase))
  (bind _goofy (Variables|Default|GetGoofy))
  (bind _psora (Variables|Default|GetPSora))
  (bind _goofy_2 (Variables|Default|GetGoofy))
  (bind _returnvalue_2 (Class|TresPlayerControllerLowerBase|GetTresCameraManager _returnvalue))
  (bind _m_lockontarget (Variables|/Script/TresGame.TresCameraManager|Getm_LockonTarget _returnvalue_2))
  (bind _returnvalue_3 (Components|GetOwner _m_lockontarget))
  (Components|Activation|SetActive (Variables|/Script/TresGame.TresCharPawnBase|GetMyMovement (Variables|Default|GetGoofy)) false false)
  (bind _returnvalue_4 (AddComponent|AddCapsuleComponent (Variables|Default|GetGoofy) false))
  (Components|Capsule|SetCapsuleSize _returnvalue_4 9e+01 45.0 true)
  (Variables|Default|Setgoof%20collision _returnvalue_4)
  (if (>= (Class|TresCharPawnBase|GetHitPoint (Variables|Default|GetGoofy)) 0)
    _
    (else
      (Class|TresCharPawnBase|SetHitPoint _goofy_2 (Math|Float|Truncate (* (Class|TresCharPawnBase|GetMaxHitPoint _goofy_2) 0.4)))))
  (Class|TresCharPawnBase|AnimStop (Variables|Default|GetGoofy) 0.0 "FullBody")
  (Class|TresCharPawnBase|SetGravityScale (Variables|Default|GetGoofy) 0.8)
  (bind _returnvalue_5 (AddComponent|AddCapsuleComponent _returnvalue_3 false))
  (bind _output_get (Variables|Default|Setenemy%20coll _returnvalue_5))
  (Components|Capsule|SetCapsuleSize _output_get 4e+01 45.0 true)
  (if (Utilities|IsValid _m_lockontarget)
    (Transformation|SetActorLocation (Variables|Default|GetGoofy) (+ (Transformation|GetActorLocation _returnvalue_3) (* (Transformation|GetActorUpVector _returnvalue_3) 700)) false false)
    (else
      (Transformation|SetActorLocation (Variables|Default|GetGoofy) (+ (Transformation|GetActorLocation _psora) (* (Transformation|GetActorForwardVector _psora) 400) (* (Transformation|GetActorUpVector _psora) 500)) false false)))
  (AI|Components|Blackboard|SetValueasBool (AI|GetBlackboard _goofy) (Utilities|Name|MakeLiteralName "GoofShotlock") true)
  (Components|Activation|SetActive (Variables|/Script/TresGame.TresCharPawnBase|GetMyMovement _goofy) true false)
  (Collision|BindEventtoOnActorBeginOverlap (Variables|Default|GetGoofy) (delegate Custom|CustomEvent_1)))

(event Custom|GoofyAnimChange
  (if (Variables|Default|GetGoofAnimSetFailSafe)
    _
    (else
      (Variables|Default|SetGoofAnimSetFailSafe true)
      (Variables|Default|SetGoof%20OG%20anims (Variables|/Script/TresGame.TresAnimSet|GetAnims (Variables|Default|Getn_ex002_animset)))))
  (for (_array_element _array_index) (Variables|/Script/TresGame.TresAnimSet|GetAnims (Variables|Default|Getn_ex002_animset))
    (Variables|Default|Setanim _array_element)
    (Variables|Default|Setanim%20index _array_index)
    (if (Utilities|Name|Equal(Name) (.AnimName (Utilities|Struct|BreakTresAnimAssetUnit (Variables|Default|Getanim))) (Utilities|Name|MakeLiteralName "JumpNormalDownLoop"))
      (Utilities|Array|SetArrayElem (Variables|/Script/TresGame.TresAnimSet|GetAnims (Variables|Default|Getn_ex002_animset)) (Variables|Default|Getanim%20index) (Utilities|Struct|MakeTresAnimAssetUnit "JumpNormalDownLoop" "/Game/Character/npc/n_ex002/anm/rt/body/GooofyFallPTV.GooofyFallPTV"))
      (else
        (Utilities|Array|SetArrayElem (Variables|/Script/TresGame.TresAnimSet|GetAnims (Variables|Default|Getn_ex002_animset)) (Variables|Default|Getanim%20index) (Utilities|Struct|MakeTresAnimAssetUnit "dummy" "/Game/Character/npc/n_ex002/anm/rt/body/GoofyFallingPT1V4.GoofyFallingPT1V4"))))))

(event Custom|CustomEvent_1
  (params (OverlappedActor :type Actor%20Object%20Reference) (OtherActor :type Actor%20Object%20Reference))
  (bind _goofy (Variables|Default|GetGoofy))
  (CallFunction|GoofyAnimReset)
  (bind _outactors (Actor|GetAllActorsOfClass "/Script/TresGame.TresEnemyPawnBase"))
  (for _array_element _outactors
    (Variables|/Script/Engine.Actor|SetCustomTimeDilation _array_element 1.0))
  (Variables|Default|SetCurrentlyFalling false)
  (Class|TresCharPawnBase|SetGravityScale _goofy 1.0)
  (Class|TresCharPawnBase|SetStopAI (Variables|Default|GetGoofy) false)
  (Collision|UnbindEventfromOnActorBeginOverlap _goofy (delegate Custom|CustomEvent_1))
  (Components|DestroyComponent (Variables|Default|Getgoof%20collision))
  (if (Variables|Default|GetSpawnedGoofy)
    (Actor|DestroyActor (Variables|Default|GetGoofy))))

(event Custom|GoofyAnimReset
  (if (Variables|Default|GetGoofAnimSetFailSafe)
    (Variables|/Script/TresGame.TresAnimSet|SetAnims (Variables|Default|Getn_ex002_animset) (Variables|Default|GetGoof%20OG%20anims))))

(event Custom|CustomEvent_0
  (params (OverlappedComponent :type Primitive%20Component%20Object%20Reference) (OtherActor :type Actor%20Object%20Reference) (OtherComp :type Primitive%20Component%20Object%20Reference) (OtherBodyIndex :type Integer) (bFromSweep :type Boolean) (SweepResult :type Hit%20Result%20Structure%20%28by%20ref%29))
  (bind _goofy (Variables|Default|GetGoofy))
  (CallFunction|GoofyAnimReset)
  (Variables|Default|SetCurrentlyFalling false)
  (Class|TresCharPawnBase|SetGravityScale _goofy 1.0)
  (Class|TresCharPawnBase|SetStopAI _goofy false)
  (Collision|UnbindEventfromOnComponentBeginOverlap (Utilities|Array|Get(acopy) (Variables|/Script/TresGame.TresBodyCollComponent|Getm_BodyColls (Variables|/Script/TresGame.TresCharPawnBase|GetMyBodyColl (Variables|Default|GetGoofy))) 3) (delegate Custom|CustomEvent_0))
  (if (Variables|Default|GetSpawnedGoofy)
    (Actor|DestroyActor (Variables|Default|GetGoofy))))

(event EventTick
  (params (DeltaSeconds :type Float%20%28single-precision%29))
  (if (not (Variables|Default|GetCurrentlyFalling))
    (if (Utilities|IsValid (Variables|Default|GetPSora))
      _
      (else
        (bind _outactors (Actor|GetAllActorsOfClass "/Script/TresGame.TresPlayerPawnBase"))
        (for _array_element _outactors
          (Variables|Default|SetPSora _array_element))))
    (if (Utilities|IsValid (Variables|Default|GetGoofy))
      _
      (else
        (bind _outactors_2 (Actor|GetAllActorsOfClass "/Script/TresGame.TresNpcPawn_n_ex002"))
        (if (> (Utilities|Array|Length _outactors_2) 0)
          (for _array_element_2 _outactors_2
            (Variables|Default|SetGoofy _array_element_2))
          (Variables|Default|SetSpawnedGoofy false)
          (else
            (bind _returnvalue (AI|SpawnAIFromClass "/Game/Blueprints/npc/n_ex002/n_ex002_Pawn.n_ex002_Pawn_C" "/Game/Blueprints/npc/n_ex002/BT/n_ex002_BT.n_ex002_BT" "0, 0, 0" "0, 0, 0" false))
            (bind _astres_npc_pawn_n_ex_002 (Utilities|Casting|CastToTresNpcPawn_n_ex002 _returnvalue))
            (Variables|Default|SetGoofy _astres_npc_pawn_n_ex_002)
            (Variables|Default|SetSpawnedGoofy true)))))
    (if (Utilities|Name|Equal(Name) (Class|TresCharPawnBase|AnimGetLastPlayAnimName (Variables|Default|GetPSora) "FullBody") (Utilities|Name|MakeLiteralName "Guard"))
      (bind _outactors_3 (Actor|GetAllActorsOfClass "/Script/TresGame.TresEnemyPawnBase"))
      (for _array_element_3 _outactors_3
        (Variables|/Script/Engine.Actor|SetCustomTimeDilation _array_element_3 0.0))
      (CallFunction|GoofyAnimChange)
      (CallFunction|GoofyFall)
      (Variables|Default|SetCurrentlyFalling true))))

(fn ConstructionScript)