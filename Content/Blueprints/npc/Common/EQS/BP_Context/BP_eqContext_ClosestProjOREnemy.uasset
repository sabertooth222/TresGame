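; EQS context for NPC queries that provides the closest threat to the querier: an opposing-team pawn in its AI attack state or an opposing-team projectile.
; It scans all TresCharPawnBase pawns, then all TresProjectileBase actors, against one shared ClosestDistance, so whichever is nearer wins.
; ClosestDistance and ClosestEnemy are not reset within the function before the scans.
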(fn ProvideSingleActor
  (params (QuerierObject :type Object%20Object%20Reference) (QuerierActor :type Actor%20Object%20Reference))
  (bind _astres_char_pawn_base (Utilities|Casting|CastToTresCharPawnBase QuerierActor))
  (LocalVariables|SetQuerier _astres_char_pawn_base)
  (bind _outactors (Actor|GetAllActorsOfClass "/Script/TresGame.TresCharPawnBase"))
  (for _array_element _outactors
    (if (!= (Class|TresPawnBase|GetTeamNo _array_element) (Class|TresPawnBase|GetTeamNo _astres_char_pawn_base))
      (if (Utilities|Enum|Equal(Enum) (Class|TresCharPawnBase|GetStateID _array_element) "TSID_STATE_AI_ATTACK")
        (Math|Float|CompareFloat (Transformation|GetDistanceTo _array_element (LocalVariables|GetQuerier)) (LocalVariables|GetClosestDistance)
          (:<
            (LocalVariables|SetClosestDistance (Transformation|GetDistanceTo _array_element (LocalVariables|GetQuerier)))
            (LocalVariables|SetClosestEnemy _array_element))))))
  (bind _outactors_2 (Actor|GetAllActorsOfClass "/Script/TresGame.TresProjectileBase"))
  (for _array_element_2 _outactors_2
    (if (!= (Class|TresPawnBase|GetTeamNo _array_element_2) (Class|TresPawnBase|GetTeamNo (LocalVariables|GetQuerier)))
      (Math|Float|CompareFloat (Transformation|GetDistanceTo _array_element_2 (LocalVariables|GetQuerier)) (LocalVariables|GetClosestDistance)
        (:<
          (LocalVariables|SetClosestDistance (Transformation|GetDistanceTo _array_element_2 (LocalVariables|GetQuerier)))
          (LocalVariables|SetClosestEnemy _array_element_2)))))
  (return (LocalVariables|GetClosestEnemy)))