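; An EQS context for Kairi that supplies the hostile projectiles currently live in the world to environment queries.
; It gathers every TresProjectileBase actor and keeps those whose team number differs from the querying pawn's and whose particle component is still active.
; The active-particle check serves as the test for whether a projectile is live.
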(fn ProvideActorsSet
  (params (QuerierObject :type Object%20Object%20Reference) (QuerierActor :type Actor%20Object%20Reference))
  (Utilities|Array|Clear (Variables|Default|GetEnemyProjectiles))
  (bind _astres_char_pawn_base (Utilities|Casting|CastToTresCharPawnBase QuerierActor))
  (bind _outactors (Actor|GetAllActorsOfClass "/Script/TresGame.TresProjectileBase"))
  (for _array_element _outactors
    (if (and (!= (Class|TresPawnBase|GetTeamNo _array_element) (Class|TresPawnBase|GetTeamNo _astres_char_pawn_base)) (Components|Activation|IsActive (Variables|/Script/TresGame.TresProjectileBase|GetMyParticle _array_element)))
      (Utilities|Array|Add (Variables|Default|GetEnemyProjectiles) _array_element)))
  (return (Variables|Default|GetEnemyProjectiles)))