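; Test actor that spawns the Mini_shorthand particle emitter at its own location and animates its rotation with a timeline.
; On BeginPlay it stores the spawned emitter and its starting world rotation, then plays Timeline_0.
; Each update lerps a full turn of roll from the track and adds it to the starting roll, keeping the starting yaw and zeroing pitch.
; An alternative CombineRotators approach is left unconnected.
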(event EventBeginPlay
  (bind _returnvalue (Effects|SpawnEmitteratLocation "/Game/Effects/magicmickey/mini_shorthand.mini_shorthand" (Transformation|GetActorLocation) "0,47.000000,0.000000"))
  (bind _output_get (Variables|Default|Setparticle _returnvalue))
  (Variables|Default|Setrot (Transformation|GetWorldRotation _output_get))
  (bind _newtrack_0 (Timeline|Timeline_0 Play)
    (:Update
      (Transformation|SetWorldRotation (Variables|Default|Getparticle) (Math|Rotator|MakeRotator (+ (Math|Float|Lerp 0.0 3.6e+02 _newtrack_0) (.Roll (Math|Rotator|BreakRotator (Variables|Default|Getrot)))) 0.0 (.Yaw (Math|Rotator|BreakRotator (Variables|Default|Getrot)))) false false))))

(fn ConstructionScript)