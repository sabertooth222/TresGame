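; One-shot helper actor that fires a projectile for a player, ally or enemy pawn on BeginPlay, then destroys itself.
; Target comes from player lock-on, optional enemy tracking (closest, random, soft angle/distance) or the AI blackboard's TargetActor.
; Spawn transform derives from pawn, mesh socket or target offsets, optionally aimed at the target.
; It spawns through a TresProjectileGenComponent, reusable by name tag, then configures homing movement.
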(event Custom|END
  (Actor|DestroyActor))

(event EventBeginPlay
  (Utilities|PawnTypeMacro
    (:NewParam2
      (Utilities|SpawnTypeMacro
        (:OutputPin
          (if (Utilities|Name|Equal(Name) (Variables|Default|GetName%20of%20Projectile) "None")
            (Utilities|IsValid (Variables|Default|GetProj%20Gen%20Comp%20Ref) :!label _label
              (:Is%20Valid
                (if (== (Utilities|Array|FindItem (Variables|/Script/TresGame.TresProjectileGenComponent|Getm_Projctiles (stale _returnvalue)) (Variables|Default|GetProjectile)) -1)
                  (Variables|/Script/TresGame.TresProjectileGenComponent|Setm_Projctiles (stale _returnvalue) (Utilities|Array|MakeArray (Variables|Default|GetProjectile)) :!label _label_2)))
              (:Is%20Not%20Valid
                (bind _returnvalue (AddComponent|AddTresProjectileGenComponent (Variables|Default|GetPawn) true (Variables|Default|GetGenComp%20Transform)))
                (bind _output_get (Variables|Default|SetProj%20Gen%20Comp%20Ref _returnvalue))
                (Variables|/Script/Engine.ActorComponent|SetComponentTags _output_get (Utilities|Array|MakeArray (Variables|Default|GetName%20of%20Projectile)))
                (goto _label_2)))
            (if (and (Variables|Default|GetProjectile%20-%20Look%20At%20Valid%20Target?) (Utilities|IsValid (Variables|Default|GetTarget)))
              (|LookAtCode))
            (bind _returnvalue_2 (Class|TresProjectileGenComponent|SpawnProjectilewithPos (Variables|Default|GetProj%20Gen%20Comp%20Ref) 0 (Variables|Default|GetProjectile%20Location) (Math|Rotator|GetRotationXVector (Variables|Default|GetProjectile%20Rotation))))
            (bind _output_get_2 (Variables|Default|SetProjectileBase _returnvalue_2))
            (if (Variables|Default|GetDebug:%20Use%20Original%20TresMove%20Component)
              (Variables|/Script/TresGame.TresProjectileMovementComponent|Setm_HomingTargetComponent (Variables|/Script/TresGame.TresProjectileBase|GetMyMovement (Variables|Default|GetProjectileBase)) (.AsTres%20Lockon%20Target%20Component (Utilities|Casting|CastToTresLockonTargetComponent (Variables|Default|GetTarget))))
              (Components|Activation|Activate (Variables|/Script/TresGame.TresProjectileBase|GetMyMovement (Variables|Default|GetProjectileBase)) true)
              (else
                (bind _returnvalue_3 (AddComponent|AddProjectileMovementComponent _output_get_2))
                (Variables|/Script/Engine.ProjectileMovementComponent|SetbIsHomingProjectile _returnvalue_3 (Variables|Default|GetProjectile%20-%20Is%20Homing?))
                (Variables|/Script/Engine.ProjectileMovementComponent|SetHomingTargetComponent _returnvalue_3 (Variables|Default|GetTarget))
                (Variables|/Script/Engine.ProjectileMovementComponent|SetHomingAccelerationMagnitude _returnvalue_3 (Variables|Default|GetProjectile%20-%20Homing%20Acceleration))
                (Variables|/Script/Engine.ProjectileMovementComponent|SetbInitialVelocityInLocalSpace _returnvalue_3 (Variables|Default|GetProjectile%20-%20Local%20Space%20Velocity))
                (Variables|/Script/Engine.ProjectileMovementComponent|SetbRotationFollowsVelocity _returnvalue_3 (Variables|Default|GetProjectile%20-%20Rotation%20Follows%20Velocity))
                (Variables|/Script/Engine.MovementComponent|SetVelocity _returnvalue_3 (Variables|Default|GetProjectile:%20Velocity))
                (Components|Activation|Activate _returnvalue_3 true)))
            (Actor|DestroyActor)
            (else
              (bind _array_element (Utilities|ForEachLoopwithBreak (Actor|GetComponentsByClass (Variables|Default|GetPawn) "/Script/TresGame.TresProjectileGenComponent") :!label _label_3)
                (:LoopBody
                  (Utilities|IsValid _array_element
                    (:Is%20Valid
                      (if (Utilities|Array|ContainsItem (Variables|/Script/Engine.ActorComponent|GetComponentTags _array_element) (Variables|Default|GetName%20of%20Projectile))
                        (Variables|Default|SetProj%20Gen%20Comp%20Ref _array_element)
                        (goto _label_3 Break)))))
                (:Completed
                  (goto _label))))))))))

(fn ConstructionScript)