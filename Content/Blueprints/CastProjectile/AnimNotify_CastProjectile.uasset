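; Anim notify that casts a projectile from the animating TresCharPawnBase by spawning a CastProjectile_Actor.
; It forwards its projectile, socket, spawn offset, movement, homing and target-tracking settings to that actor, which receives the owning pawn as well.
; It then unconditionally draws a debug sphere and thin cone at the pawn location plus spawn offset, with the resulting world X negated, orienting the cone by the adjustment rotation.
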(fn ReceivedNotify
  (params (MeshComp :type Skeletal%20Mesh%20Component%20Object%20Reference) (Animation :type Anim%20Sequence%20Base%20Object%20Reference))
  (bind _returnvalue (Components|GetOwner MeshComp))
  (bind _spawn___adjust_x_position (Variables|Default|GetSpawn%20-%20Adjust%20X-Position))
  (bind _spawn___adjust_y_position (Variables|Default|GetSpawn%20-%20Adjust%20Y-Position))
  (bind _spawn___adjust_z_position (Variables|Default|GetSpawn%20-%20Adjust%20Z-Position))
  (bind _debug_sphere___duration (Variables|Default|GetDebug%20Sphere%20-%20Duration))
  (bind _astres_char_pawn_base (Utilities|Casting|CastToTresCharPawnBase _returnvalue))
  (bind _returnvalue_2 (Transformation|GetActorLocation _astres_char_pawn_base))
  (bind _returnvalue_3 (+ _returnvalue_2 "0, 0, 0" "" (Math|Vector|MakeVector _spawn___adjust_x_position _spawn___adjust_y_position _spawn___adjust_z_position)))
  (bind (_x _y _z) (Math|Vector|BreakVector _returnvalue_3))
  (bind _returnvalue_4 (* _x 2.0))
  (bind _returnvalue_5 (- _x _returnvalue_4))
  (Game|SpawnActorfromClass "/Game/Blueprints/CastProjectile/CastProjectile_Actor.CastProjectile_Actor_C" (|CollapseGraph_0) "Undefined" 0 _astres_char_pawn_base (Variables|Default|GetProjectile) (Variables|Default|GetProjectile%20Name) (Variables|Default|GetPawn%20Type) (Variables|Default|GetSpawn%20Type) (Variables|Default|GetSpawn:%20Socket%20-%20Socket%20Name) (Variables|Default|GetDebug%20-%20Delay%20Before%20Installing%20UE4Move) (Variables|Default|GetDebug%20-%20Delay%20Before%20Deactivate%20TresMove) (Variables|Default|GetTracking%20-%20Ignore%20Lockon%20Target?) (Variables|Default|GetTracking%20-%20Enable%20Tracking?) (Variables|Default|GetTracking%20-%20Tracking%20Type) (Variables|Default|GetTracking%20-%20Max%20Distance) (Variables|Default|GetTracking:%20Soft%20Target%20-%20Max%20Angle%20of%20Cone) (Variables|Default|GetProjectile%20-%20Initial%20Speed) (Variables|Default|GetProjectile%20-%20Max%20Speed) (Variables|Default|GetProjectile%20-%20Gravity) (Variables|Default|GetRotation%20Follows%20Velocity?) (Variables|Default|GetDebug%20-%20Local%20Space%20Velocity?) (Variables|Default|GetLook%20at%20Valid%20Target?) (Variables|Default|GetProjectile%20-%20Enable%20Homing?) (Variables|Default|GetProjectile%20-%20Homing%20Acceleration%20Magnitude) (Variables|Default|GetSpawn%20-%20Adjust%20X-Position) (Variables|Default|GetSpawn%20-%20Adjust%20Y-Position) (Variables|Default|GetSpawn%20-%20Adjust%20Z-Position) (Variables|Default|GetSpawn%20-%20Adjust%20X-Rotation) (Variables|Default|GetSpawn%20-%20Adjust%20Y-Rotation) (Variables|Default|GetSpawn%20-%20Adjust%20Z-Rotation) (Variables|Default|GetSpawn:%20Enemy%20-%20No-Enemy%20X-Position) (Variables|Default|GetSpawn:%20Enemy%20-%20No-Enemy%20Y-Position) (Variables|Default|GetSpawn:%20Enemy%20-%20No-Enemy%20Z-Position) (Variables|Default|GetDebug%20-%20Use%20Original%20Tres%20Homing) (Variables|Default|GetDebug%20-%20Projectile%20Velocity) 0)
  (Rendering|Debug|DrawDebugSphere (Math|Vector|MakeVector _returnvalue_5 _y _z) 3e+01 12 (Variables|Default|GetDebug%20Sphere%20-%20Color) _debug_sphere___duration 0.5)
  (Class|KismetSystemLibrary|DrawDebugConeinDegrees (Math|Vector|MakeVector _returnvalue_5 _y _z) (Math|Vector|GetRightVector (Math|Rotator|MakeRotator (Variables|Default|GetSpawn%20-%20Adjust%20X-Rotation) (Variables|Default|GetSpawn%20-%20Adjust%20Y-Rotation) (Variables|Default|GetSpawn%20-%20Adjust%20Z-Rotation))) 1e+02 1.0 1.0 12 "(R=0.035952,G=0.000000,B=0.489583,A=1.000000)" _debug_sphere___duration 2.0)
  (return false))