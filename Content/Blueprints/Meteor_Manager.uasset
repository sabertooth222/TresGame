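; Meteor shower manager that rains projectiles straight down around the average location of all enemies, captured once at BeginPlay.
; It adds a projectile generator component to the player pawn and drives it with a fast looping timer, spawning at random points in a raised flat box.
; After an initial burst, timer pauses and delays stagger the spawns until a fixed count destroys component and actor.
; BeginPlay also opens a "test" subtitle.
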(event Custom|CustomEvent_0
  (bind _returnvalue (Math|Vector|MakeVector 1e+03 1e+03 0.0))
  (bind _projspawntimer (Variables|Default|GetProjSpawnTimer))
  (bind _donald_location (Variables|Default|GetDonald_Location))
  (bind _enemyaverage (Variables|Default|GetEnemyAverage))
  (bind _projspawntimer_2 (Variables|Default|GetProjSpawnTimer))
  (bind (_x _y _z) (Math|Vector|BreakVector _donald_location))
  (bind _returnvalue_2 (Math|Random|RandomPointinBoundingBox _enemyaverage _returnvalue))
  (bind (_x_2 _y_2 _z_2) (Math|Vector|BreakVector _returnvalue_2))
  (if (> (Variables|Default|GetProjectileCount) 10)
    (Utilities|Time|PauseTimerbyHandle _projspawntimer)
    (Utilities|FlowControl|Delay 0.05)
    (Utilities|Time|UnpauseTimerbyHandle _projspawntimer))
  (bind _returnvalue_3 (Class|TresProjectileGenComponent|SpawnProjectilewithPos (Variables|Default|GetProjGenComp) 0 (Math|Vector|MakeVector _x_2 _y_2 (+ _z_2 1e+03)) (Math|Vector|GetUnitDirection(Vector) _donald_location (Math|Vector|MakeVector _x _y (- _z 1e+03)))))
  (Components|Activation|SetActive (Variables|/Script/TresGame.TresProjectileBase|GetMyParticle _returnvalue_3) true false)
  (Variables|Default|SetProjectileCount (+ (Variables|Default|GetProjectileCount) 1))
  (if (>= (Variables|Default|GetProjectileCount) 40)
    (Utilities|Time|PauseTimerbyHandle (Variables|Default|GetProjSpawnTimer))
    (Components|DestroyComponent (Variables|Default|GetProjGenComp))
    (Actor|DestroyActor)
    (elif (> (Variables|Default|GetProjectileCount) 10)
      (Utilities|Time|PauseTimerbyHandle _projspawntimer_2)
      (Utilities|FlowControl|Delay (Math|Random|RandomFloatinRange 0.0 0.1))
      (Utilities|Time|UnpauseTimerbyHandle _projspawntimer_2))))

(event EventBeginPlay
  (bind _returnvalue (Class|TresGameBlueprintLibrary|GetTresPlayerPawnBase))
  (Class|TresGameBlueprintLibrary|TresUIOpenSubtitle (Utilities|Struct|MakeTresLocText "" "" (Variables|Default|GetNewVar_1) "test") "Cutscene")
  (Variables|Default|SetDonald_Location (Transformation|GetActorLocation _returnvalue))
  (bind _returnvalue_2 (AddComponent|AddTresProjectileGenComponent _returnvalue false))
  (Variables|Default|SetProjGenComp _returnvalue_2)
  (bind _outactors (Actor|GetAllActorsOfClass "/Script/TresGame.TresEnemyPawnBase"))
  (bind _returnvalue_3 (Class|GameplayStatics|GetActorArrayAverageLocation _outactors))
  (Variables|Default|SetEnemyAverage _returnvalue_3)
  (bind _returnvalue_4 (Utilities|Time|SetTimerbyEvent (delegate Custom|CustomEvent_0) 0.001 true))
  (Variables|Default|SetProjSpawnTimer _returnvalue_4))

(fn ConstructionScript)