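; One-shot actor that plays a form-change visual on the first N_ex023_Pawn in the level, reverting it to base-form textures.
; On BeginPlay a timeline drives the FormChangeSlide scalar on three of the pawn's skeletal mesh dynamic materials.
; At the halfway point, where the effect peaks and hides the swap, a one-time flag triggers per-slot functions that set the base textures.
; The actor destroys itself when the timeline finishes.
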(event EventBeginPlay
  (bind _outactors (Actor|GetAllActorsOfClass "/Game/Blueprints/npc/n_ex023/n_ex023_pawn.n_ex023_Pawn_C"))
  (Variables|Default|SetNPCPawn (Utilities|Array|Get(acopy) _outactors))
  (bind _alpha (Timeline|Formchange%20Slider PlayFromStart)
    (:Update
      ;[0.5528 1 0.4499] Slides each mat from 0 to 1 using the timeline over 1 second
      (bind _asmaterial_instance_dynamic (Utilities|Casting|CastToMaterialInstanceDynamic (Rendering|Material|GetMaterial (Actor|GetComponentbyClass (Variables|Default|GetNPCPawn) "/Script/TresGame.TresSkeletalMeshComponent") 9)))
      (bind _asmaterial_instance_dynamic_2 (Utilities|Casting|CastToMaterialInstanceDynamic (Rendering|Material|GetMaterial (Actor|GetComponentbyClass (Variables|Default|GetNPCPawn) "/Script/TresGame.TresSkeletalMeshComponent") 10)))
      (bind _asmaterial_instance_dynamic_3 (Utilities|Casting|CastToMaterialInstanceDynamic (Rendering|Material|GetMaterial (Actor|GetComponentbyClass (Variables|Default|GetNPCPawn) "/Script/TresGame.TresSkeletalMeshComponent") 8)))
      (Rendering|Material|SetScalarParameterValue _asmaterial_instance_dynamic "FormChangeSlide" _alpha :!class /Script/Engine.MaterialInstanceDynamic)
      ;[0.6262 0.3719 1] Waits until the alpha slide gets to .5 (which is the "max" effect, the effect goes down after .5 until it gets to 1, where the effect is non-existent) - this code changes the textures at 0.5 (the game also changes the textures from texture 0 to texture 1 automatically, not sure how exactly that works)
      (if (and (>= _alpha 0.5) (Variables|Default|GetStillFormChanged))
        (Variables|Default|SetStillFormChanged false)
        ;[0.4973 0.9502 1] Switches textures to base form
        (|revertmat9_2 (Rendering|Material|GetMaterial (Actor|GetComponentbyClass (Variables|Default|GetNPCPawn) "/Script/TresGame.TresSkeletalMeshComponent") 9))
        (|revertmat10_2 (Rendering|Material|GetMaterial (Actor|GetComponentbyClass (Variables|Default|GetNPCPawn) "/Script/TresGame.TresSkeletalMeshComponent") 10))
        (|revertmat8_2 (Rendering|Material|GetMaterial (Actor|GetComponentbyClass (Variables|Default|GetNPCPawn) "/Script/TresGame.TresSkeletalMeshComponent") 8))))
    (:Finished
      (Actor|DestroyActor))))

(fn ConstructionScript)