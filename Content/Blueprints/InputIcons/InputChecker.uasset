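; InputChecker tracks the player's most recent input device type and whether gamepad Confirm/Cancel are swapped.
; On BeginPlay and every Tick, GetInputMethod sets SwapConfirmCancel from the GamePadDecideType setting in the TresGameInstance.
; It then polls every key in KeyLastInputMap on player controller 0 and, for any just pressed, stores that key's device type in LastInputType.
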(event EventTick
  (params (DeltaSeconds :type Float%20%28single-precision%29))
  (CallFunction|GetInputMethod))

(event EventBeginPlay
  (CallFunction|GetInputMethod))

(fn ConstructionScript)

(fn GetInputMethod
  (bind _returnvalue (Class|TresGameBlueprintLibrary|GetTresPlayerControllerBase))
  ;[1 1 1] Confirm/Cancel Swap
  (Variables|Default|SetSwapConfirmCancel (== (Variables|/Script/TresGame.TresGameSettings|GetGamePadDecideType (Variables|/Script/TresGame.TresGameInstance|Getm_pGameSettings (.AsTres%20Game%20Instance (Utilities|Casting|CastToTresGameInstance (Game|GetGameInstance))))) 1))
  ;[1 1 1] Get LastInput
  (bind _keys (Utilities|Map|Keys (Variables|Default|GetKeyLastInputMap)))
  (for _array_element _keys
    (if (Game|Player|WasInputKeyJustPressed _returnvalue _array_element)
      (Variables|Default|SetLastInputType (Class|PlayerController|SqEXGetLastInputKeyDeviceType _returnvalue _array_element)))))