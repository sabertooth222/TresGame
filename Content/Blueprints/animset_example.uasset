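; Animation notify that switches or resets an animset through an Animset_managewr actor when the notify fires.
; It looks up the first manager in the world and calls AnimReset if Reset is set, otherwise AnimSetChange with its AnimsetChange value.
; A missing manager is spawned at the origin only for changes; a reset still indexes the empty array.
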(fn ReceivedNotify
  (params (MeshComp :type Skeletal%20Mesh%20Component%20Object%20Reference) (Animation :type Anim%20Sequence%20Base%20Object%20Reference))
  (bind _outactors (Actor|GetAllActorsOfClass "/Game/Blueprints/animset_managewr.animset_managewr_C"))
  (if (< (Utilities|Array|Length _outactors) 1)
    (if (Variables|Default|GetReset?)
      (Default|AnimReset (Utilities|Array|Get(acopy) _outactors) :!label _label)
      (else
        (bind _returnvalue (Game|SpawnActorfromClass "/Game/Blueprints/animset_managewr.animset_managewr_C" (Math|Transform|MakeTransform "0, 0, 0") "Undefined" 0 0))
        (Default|AnimSetChange _returnvalue (Variables|Default|GetAnimsetChange))))
    (elif (Variables|Default|GetReset?)
      (goto _label)
      (else
        (Default|AnimSetChange (Utilities|Array|Get(acopy) _outactors) (Variables|Default|GetAnimsetChange))))))