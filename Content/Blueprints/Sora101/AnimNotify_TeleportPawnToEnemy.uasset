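; Anim notify that teleports the owning pawn toward an enemy during an animation.
; The player uses the camera's lock-on target; otherwise it picks the living, lockable, non-invincible enemy with the lowest distance-times-angle score within range and view angle.
; The destination is offset from the target or capped at teleport range, or straight ahead if targetless teleporting is allowed.
; A line trace shortens the jump at obstacles, and rotation is kept.
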(fn ReceivedNotify
  (params (MeshComp :type Skeletal%20Mesh%20Component%20Object%20Reference) (Animation :type Anim%20Sequence%20Base%20Object%20Reference))
  (bind _astres_pawn_base (Utilities|Casting|CastToTresPawnBase (Components|GetOwner MeshComp)))
  (LocalVariables|SetPawn _astres_pawn_base)
  (|GetTargetEnemy)
  (Transformation|Teleport)
  (return false))