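; Behavior Tree task, apparently a test, that switches on debug displays through TresGameCheatManager when it executes.
; It prints a debug string, then, if Blueprint debug mode is active, calls cheat functions for HUD, AI, EQS, text render, status log and GPU analysis before finishing successfully.
; Otherwise it shows a "not debug mode" subtitle and never calls FinishExecute.
; Several disconnected debug calls remain in the graph.
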(event EventReceiveExecute
  (params (OwnerActor :type Actor%20Object%20Reference))
  (Development|ExecuteConsoleCommand "")
  (Class|TresGameBlueprintLibrary|TresDebugPrintString "help" true false 5.0 "(R=0.058054,G=1.000000,B=0.484891,A=1.000000)" false)
  (bind _returnvalue (Class|TresGameBlueprintLibrary|IsTresBluePrintDebugMode))
  (if _returnvalue
    (bind _astres_game_cheat_manager (Utilities|Casting|CastToTresGameCheatManager (Variables|/Script/Engine.PlayerController|GetCheatManager (Class|TresGameBlueprintLibrary|GetTresPlayerControllerBase))))
    (Class|TresGameCheatManager|DebugUISetHudDrawDeubg _astres_game_cheat_manager true)
    (Class|TresGameCheatManager|DebugShowAIDebug _astres_game_cheat_manager true)
    (Class|TresGameCheatManager|DebugShowEQSDebug _astres_game_cheat_manager true)
    (Class|TresGameCheatManager|DebugSetVisibleDebugTextRender _astres_game_cheat_manager true)
    (Class|TresGameCheatManager|DebugUIShowAllHud _astres_game_cheat_manager)
    (Class|TresGameCheatManager|DebugUISetActionCommand _astres_game_cheat_manager 5)
    (Class|TresGameCheatManager|DebugBPEMSetEnabledStatusLog _astres_game_cheat_manager true)
    (Class|TresGameCheatManager|AllAIDebugDisplay _astres_game_cheat_manager)
    (Class|TresGameCheatManager|DebugDiffAnalysisGPU _astres_game_cheat_manager)
    (AI|BehaviorTree|FinishExecute true)
    (else
      (Class|TresGameBlueprintLibrary|TresUIOpenSubtitle (Utilities|Struct|MakeTresLocText "" "" (Variables|Default|GetNewVar_0) "not debug mode") "Cutscene"))))