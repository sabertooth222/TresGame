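; Anim notify that moves a TresAIPawnBase toward its blackboard TargetActor during an animation.
; The destination interpolates by a set percentage toward the target, offset along the target's forward and right axes and world Z.
; If distance to the target is within the minimum and maximum range, it spawns a BP_MovetoDest helper to perform the timed move, with floor-snap and yaw options.
; The branch for playing a new animation during the move is disconnected.
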(fn ReceivedNotify
  (params (MeshComp :type Skeletal%20Mesh%20Component%20Object%20Reference) (Animation :type Anim%20Sequence%20Base%20Object%20Reference))
  (bind _destination_offset (Variables|Default|GetDestination%20Offset))
  (bind (_x _y _z) (Math|Vector|BreakVector _destination_offset))
  (bind _astres_aipawn_base (Utilities|Casting|CastToTresAIPawnBase (Components|GetOwner MeshComp)))
  (bind _output_get (LocalVariables|SetAIPawn _astres_aipawn_base))
  (bind _astres_char_pawn_base (Utilities|Casting|CastToTresCharPawnBase (AI|Components|Blackboard|GetValueasObject (AI|GetBlackboard _output_get) (Utilities|Name|MakeLiteralName "TargetActor"))))
  (LocalVariables|SetTarget _astres_char_pawn_base)
  (LocalVariables|SetDestination (Math|Vector|Lerp(Vector) (Transformation|GetActorLocation (LocalVariables|GetAIPawn)) (+ (Math|Vector|MakeVector (.X (Math|Vector|BreakVector (Transformation|GetActorLocation (LocalVariables|GetTarget)))) (.Y (Math|Vector|BreakVector (Transformation|GetActorLocation (LocalVariables|GetTarget)))) (+ (.Z (Math|Vector|BreakVector (Transformation|GetActorLocation (LocalVariables|GetTarget)))) _z)) (* (Transformation|GetActorForwardVector (LocalVariables|GetTarget)) _y) (* (Transformation|GetActorRightVector (LocalVariables|GetTarget)) _x)) (/ (Variables|Default|GetPercentage%20of%20distance%20to%20target.) 1e+02)))
  (Math|Float|CompareFloat (Transformation|GetDistanceTo (LocalVariables|GetAIPawn) (LocalVariables|GetTarget)) (Variables|Default|GetMinimum%20Distance)
    (:>
      _)
    (:==
      _))
  (Math|Float|CompareFloat (Transformation|GetDistanceTo (LocalVariables|GetAIPawn) (LocalVariables|GetTarget)) (Variables|Default|GetMaximum%20Distance)
    (:==
      _)
    (:<
      _))
  (bind _returnvalue (Game|SpawnActorfromClass "/Game/Blueprints/notifies/BP_MovetoDest.BP_MovetoDest_C" (Math|Transform|MakeTransform "0, 0, 0") "Undefined" 0 0))
  (Default|MoveUp _returnvalue (LocalVariables|GetAIPawn) (LocalVariables|GetDestination) (Variables|Default|GetTime%20To%20Arrive) (Variables|Default|GetStay%20On%20Ground) (Variables|Default|GetRotate%20With%20Movement))
  (return false))