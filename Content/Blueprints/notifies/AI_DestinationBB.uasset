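; Anim notify that moves the owning AI pawn to the Destination vector stored in its blackboard.
; It spawns a BP_MovetoDest helper at the world origin, which drives the move using the notify's arrival time, floor-snap and rotation settings.
; It does nothing unless the owner is an AI pawn and the blackboard TargetActor is a character pawn, though that target is not passed to the move.
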(fn ReceivedNotify
  (params (MeshComp :type Skeletal%20Mesh%20Component%20Object%20Reference) (Animation :type Anim%20Sequence%20Base%20Object%20Reference))
  (bind _astres_aipawn_base (Utilities|Casting|CastToTresAIPawnBase (Components|GetOwner MeshComp)))
  (bind _output_get (LocalVariables|SetAIPawn _astres_aipawn_base))
  (bind _astres_char_pawn_base (Utilities|Casting|CastToTresCharPawnBase (AI|Components|Blackboard|GetValueasObject (AI|GetBlackboard _output_get) (Utilities|Name|MakeLiteralName "TargetActor"))))
  (LocalVariables|SetTarget _astres_char_pawn_base)
  (LocalVariables|SetDestination (AI|Components|Blackboard|GetValueasVector (AI|GetBlackboard _output_get) (Utilities|Name|MakeLiteralName "Destination")))
  (bind _returnvalue (Game|SpawnActorfromClass "/Game/Blueprints/notifies/BP_MovetoDest.BP_MovetoDest_C" (Math|Transform|MakeTransform "0, 0, 0") "Undefined" 0 0))
  (Default|MoveUp _returnvalue (LocalVariables|GetAIPawn) (LocalVariables|GetDestination) (Variables|Default|GetTime%20To%20Arrive) (Variables|Default|GetStay%20On%20Ground) (Variables|Default|GetRotate%20With%20Movement))
  (return false))