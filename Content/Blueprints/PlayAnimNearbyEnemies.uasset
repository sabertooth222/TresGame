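; Anim notify that plays an animation on the player pawn when enough enemies are nearby.
; It gathers all TresEnemyPawnBase actors, skipping the scan if there are fewer than NearbyEnemies, and counts those within Distance of player 0.
; When the count reaches the threshold, it calls AnimPlaySequence with configurable slot, blend, loop, play rate and root-transform settings, then exits.
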(fn ReceivedNotify
  (params (MeshComp :type Skeletal%20Mesh%20Component%20Object%20Reference) (Animation :type Anim%20Sequence%20Base%20Object%20Reference))
  (LocalVariables|SetPlayerPawn (Class|TresGameBlueprintLibrary|GetTresPlayerPawnBase))
  (bind _outactors (Actor|GetAllActorsOfClass "/Script/TresGame.TresEnemyPawnBase"))
  (if (>= (Utilities|Array|Length _outactors) (Variables|Default|GetNearby%20Enemies))
    (bind _array_element (Utilities|Array|ForEachLoopwithBreak _outactors :!label _label)
      (:LoopBody
        (if (<= (Transformation|GetDistanceTo (LocalVariables|GetPlayerPawn) _array_element) (Variables|Default|GetDistance))
          (bind _result (Math|Integer|IncrementInt (LocalVariables|GetValidNearbyEnemies))
            (:%20%20
              (if (== _result (Variables|Default|GetNearby%20Enemies))
                (Utilities|FlowControl|Sequence
                  (:then_0
                    (Class|TresCharPawnBase|AnimPlaySequence (LocalVariables|GetPlayerPawn) (Variables|Default|GetAnimation) (LocalVariables|GetName) (Variables|Default|GetBlend%20Time) (Variables|Default|GetLoop) (Variables|Default|GetEffect%20Group) (Variables|Default|GetPlay%20Rate) (Variables|Default|GetRoot%20Translation) (Variables|Default|GetRoot%20Rotation) (Variables|Default|GetRoot%20Trans%20Scale%20XY) (Variables|Default|GetRoot%20Trans%20Scale%20Z))
                    (return false))
                  (:then_1
                    (goto _label Break)))))))))))