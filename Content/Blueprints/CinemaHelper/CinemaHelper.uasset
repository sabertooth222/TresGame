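; CinemaHelper is a self-deduplicating helper actor that exposes events for playing and skipping cutscenes.
; PlaySequence plays a level sequence, blending from a once-cached view target and back on finish, optionally hiding the HUD.
; SkipCutscene stops the sequence and restores actor visibility, music and HUD.
; Other events handle subtitles, info popups, sound, visibility and BGM, using slots and volume gathered five seconds after BeginPlay.
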(fn ConstructionScript)

(fn NewFunction0)

(event Custom|Transition%20To%20Cutscene
  (params (Animated%20Camera%20Actor%20Ref :type Actor%20Object%20Reference) (BlendTime :type Float%20%28single-precision%29) (BlendFunc :type EViewTargetBlendFunction%20Enum :default "VTBlend_Linear") (BlendExp :type Float%20%28single-precision%29) (bLockOutgoing :type Boolean))
  (bind _returnvalue (Class|TresGameBlueprintLibrary|GetLocalPlayerController))
  ;[0.05248 0.002314 0.7604 0.23] Camera Blending
  (Utilities|FlowControl|Sequence
    (:then_0
      (Utilities|FlowControl|DoOnce false ; We need to save the view target only ONCE. this is VITAL to blending BACK to sora.\nIn order for the blending to work properly, sora must be loaded into the scene first,\nso don't try to play a level sequence on event begin play without a delay, otherwise\nwe won't be able to blend back to sora.
        (:Completed
          (Variables|Niko'sSequencerLogicVariables|SetCached%20View%20Target (Pawn|GetViewTarget _returnvalue)))))
    (:then_1
      (Game|Player|SetViewTargetwithBlend _returnvalue Animated%20Camera%20Actor%20Ref BlendTime BlendFunc BlendExp bLockOutgoing))))

(event Custom|Transition%20To%20Gameplay
  (params (BlendTime :type Float%20%28single-precision%29) (BlendFunc :type EViewTargetBlendFunction%20Enum :default "VTBlend_Linear") (BlendExp :type Float%20%28single-precision%29) (bLockOutgoing :type Boolean))
  ;[0.05248 0.002314 0.7604 0.23] Camera Blending
  (Game|Player|SetViewTargetwithBlend (Class|TresGameBlueprintLibrary|GetLocalPlayerController) (Variables|Niko'sSequencerLogicVariables|GetCached%20View%20Target) BlendTime BlendFunc BlendExp bLockOutgoing))

(event Custom|Play%20Sequence
  (params (LevelSequence :type Level%20Sequence%20Object%20Reference) (To%20Cutscene%20Blend%20Time :type Float%20%28single-precision%29) (Back%20To%20Gameplay%20Blend%20Time :type Float%20%28single-precision%29) (Hide%20HUD? :type Boolean) (HUD%20Show%20Delay%20%28if%20hide%20hud%20is%20true%29 :type Float%20%28single-precision%29) (%28Other%20Settings%29 :type Movie%20Scene%20Sequence%20Playback%20Settings%20Structure))
  ;[0.05248 0.002314 0.7604 0.23] Play Sequence Event
  (if Hide%20HUD?
    (Class|TresGameBlueprintLibrary|TresUIHideHudCommand)
    (Class|TresGameBlueprintLibrary|TresUIHideHudUx)
    (Class|TresGameBlueprintLibrary|TresUIHideHudStatus)
    (Class|TresGameBlueprintLibrary|TresUIHideHudShining))
  (bind _outactor (Sequencer|Player|CreateLevelSequencePlayer LevelSequence %28Other%20Settings%29))
  (Sequencer|Player|Stop (Variables|/Script/LevelSequence.LevelSequenceActor|GetSequencePlayer _outactor) :!class /Script/MovieScene.MovieSceneSequencePlayer)
  (Class|MovieSceneSequencePlayer|JumptoPosition (Variables|/Script/LevelSequence.LevelSequenceActor|GetSequencePlayer _outactor) 0.0)
  (Sequencer|Player|Play (Variables|/Script/LevelSequence.LevelSequenceActor|GetSequencePlayer _outactor) :!class /Script/MovieScene.MovieSceneSequencePlayer)
  (CallFunction|TransitiontoCutscene (CallFunction|GetCinemaHelper) _outactor To%20Cutscene%20Blend%20Time "VTBlend_Linear" 0.5 false)
  ;[0.05248 0.002314 0.7604 0.23] On Sequence Finished Delegate Event
  (EventDispatchers|BindEventtoOnFinished (Variables|/Script/LevelSequence.LevelSequenceActor|GetSequencePlayer _outactor) (delegate Custom|SequencerEvent%20|%20OnFinished)))

(event Custom|SequencerEvent%20|%20OnFinished
  ;[0.05248 0.002314 0.7604 0.23] On Sequence Finished Delegate Event
  (CallFunction|TransitiontoGameplay (stale Custom|Play%20Sequence Back%20To%20Gameplay%20Blend%20Time) "VTBlend_Linear" 0.5 false)
  (if (stale Custom|Play%20Sequence Hide%20HUD?)
    (Utilities|FlowControl|Delay (+ (stale Custom|Play%20Sequence Back%20To%20Gameplay%20Blend%20Time) (stale Custom|Play%20Sequence HUD%20Show%20Delay%20%28if%20hide%20hud%20is%20true%29)))
    (Class|TresGameBlueprintLibrary|TresUIShowHudCommand)
    (Class|TresGameBlueprintLibrary|TresUIShowHudStatus)
    (Class|TresGameBlueprintLibrary|TresUIShowHudUx)))

(event Custom|Sub
  (params (Subtitles :type String) (Subtitle%20Time :type Float%20%28single-precision%29) (Sound :type Sound%20Base%20Object%20Reference))
  (Utilities|Time|ClearandInvalidateTimerbyHandle (Variables|CinemaHelperMainVariables|GetSubClearEvent))
  (Class|TresGameBlueprintLibrary|TresUIOpenSubtitle (Utilities|Struct|MakeTresLocText Subtitles) "Cutscene")
  (Audio|PlaySound2D Sound)
  (bind _returnvalue (Utilities|Time|SetTimerbyEvent (delegate Custom|Clear%20Sub) Subtitle%20Time))
  (Variables|CinemaHelperMainVariables|SetSubClearEvent _returnvalue))

(event Custom|PlaySound
  (params (Sound :type Sound%20Base%20Object%20Reference))
  (Audio|PlaySound2D Sound))

(event Custom|GetPlayer
  (Variables|CinemaHelperMainVariables|SetPawn (Class|TresGameBlueprintLibrary|GetTresPlayerPawnBase)))

(event Custom|SkipCutscene
  (params (Level%20Sequence :type Level%20Sequence%20Actor%20Object%20Reference) (Delay :type Float%20%28single-precision%29) (FadeTime :type Float%20%28single-precision%29) (Play%20Old%20Music :type Boolean) (Play%20New%20Music :type Boolean) (New%20Music :type Sound%20Base%20Object%20Reference))
  (|SequenceSkip-FirstHalf_2 Level%20Sequence Delay)
  (|CinemaStuff-Code_2 Delay FadeTime Play%20Old%20Music Play%20New%20Music New%20Music)
  (Class|TresGameBlueprintLibrary|BPTresStartFadein :InLayer "SQEX_FADE_LAYER_FG" :InFadeTime 1.0)
  (Utilities|FlowControl|Delay 1.0)
  (Class|TresGameBlueprintLibrary|TresEndCinematicMode false false)
  (Class|TresGameBlueprintLibrary|TresUIShowHudCommand)
  (Class|TresGameBlueprintLibrary|TresUIShowHudStatus))

(event Custom|PlayNewMusic
  (params (New%20BGM :type Sound%20Base%20Object%20Reference) (FadeTime :type Float%20%28single-precision%29))
  (bind _event_bgmslot (Variables|CinemaHelperMainVariables|GetEvent%20BGMSlot))
  (Class|SQEXSEADBGMSlotController|Set _event_bgmslot New%20BGM)
  (Class|SQEXSEADBGMSlotController|SetVolume _event_bgmslot (Math|Conversions|ToFloat(Byte) (Variables|CinemaHelperMainVariables|GetVolume)) FadeTime)
  (Class|SQEXSEADBGMSlotController|Play (Variables|CinemaHelperMainVariables|GetEvent%20BGMSlot)))

(event Custom|StopMusic
  (params (FadeTime :type Float%20%28single-precision%29))
  (Class|SQEXSEADStatics|StopAllBGMOptionalFade FadeTime))

(event Custom|StopSound
  (params (FadeTime :type Float%20%28single-precision%29))
  (Class|SQEXSEADStatics|StopAllCategorySounds FadeTime))

(event Custom|HideScene
  (params (Is%20Hidden :type Boolean))
  (bind _outactors (Class|TresGameBlueprintLibrary|GetAllActorsOfTag "/Script/Engine.Pawn" "Scene"))
  (for _array_element _outactors
    (Rendering|SetActorHiddenInGame _array_element Is%20Hidden)))

(event Custom|ShowPlayer
  (bind _outactors (Actor|GetAllActorsOfClass "/Script/TresGame.TresPlayerPawnBase"))
  (for _array_element _outactors
    (Rendering|SetVisibility (Variables|/Script/TresGame.TresCharPawnBase|GetMyMesh _array_element) true false)
    (Rendering|SetActorHiddenInGame _array_element false)))

(event Custom|PlayOldMusic
  (params (FadeTime :type Float%20%28single-precision%29))
  (bind _current_bgmslot (Variables|CinemaHelperMainVariables|GetCurrent%20BGMSlot))
  (Class|SQEXSEADBGMSlotController|SetVolume _current_bgmslot (Math|Conversions|ToFloat(Byte) (Variables|CinemaHelperMainVariables|GetVolume)) FadeTime)
  (Class|SQEXSEADBGMSlotController|Play _current_bgmslot))

(event Custom|HidePlayer
  (params (Is%20Hidden :type Boolean))
  (bind _outactors (Actor|GetAllActorsOfClass "/Script/TresGame.TresPlayerPawnBase"))
  (for _array_element _outactors
    (|CollapseGraph_0_2 _array_element Is%20Hidden)))

(event Custom|Info
  (params (Localized%20Text :type String) (OptionalDisplayTime :type Float%20%28single-precision%29))
  (Class|TresGameBlueprintLibrary|TresUIOpenInformation (Utilities|Struct|MakeTresLocText Localized%20Text) true OptionalDisplayTime))

(event Custom|Clear%20Sub
  (Class|TresGameBlueprintLibrary|TresUICloseSubtitle))

(event Custom|HideParty
  (params (Is%20Hidden :type Boolean))
  (bind _outactors (Actor|GetAllActorsOfClass "/Script/TresGame.TresAIPawnBase"))
  (Utilities|IsValid (Utilities|Array|Get(acopy) _outactors)
    (:Is%20Valid
      (for _array_element _outactors
        (Rendering|SetActorHiddenInGame _array_element Is%20Hidden)
        (Class|TresGameBlueprintLibrary|SetAllComponentVisible _array_element (not Is%20Hidden))))))

(event EventBeginPlay
  (|DupeCleanup
    (:OutputPin
      (Utilities|FlowControl|Delay 5.0)
      (Variables|CinemaHelperMainVariables|SetPawn (Class|TresGameBlueprintLibrary|GetTresPlayerPawnBase))
      (bind _returnvalue (Class|SQEXSEADStatics|GetPlayingBGMSlotController))
      (Variables|CinemaHelperMainVariables|SetCurrent%20BGMSlot _returnvalue)
      (bind _returnvalue_2 (Class|TresSoundStatics|TresGetWorldStaticBGMAsset _returnvalue "FIELD"))
      (Variables|CinemaHelperMainVariables|SetOld%20Music%20FIELD _returnvalue_2)
      (bind _returnvalue_3 (Class|TresSoundStatics|TresGetWorldStaticBGMAsset _returnvalue "BATTLE"))
      (Variables|CinemaHelperMainVariables|SetOld%20Music%20BATTLE _returnvalue_3)
      (bind _returnvalue_4 (Class|SQEXSEADStatics|CreateBGMSlot "Event" (Utilities|Struct|MakeSQEXSEAD_BGMOptions 50 "Stop")))
      (Variables|CinemaHelperMainVariables|SetEvent%20BGMSlot _returnvalue_4)
      (Variables|CinemaHelperMainVariables|SetVolume (Variables|/Script/TresGame.TresGameSettings|GetSoundBgmVolume (Variables|/Script/TresGame.TresGameInstance|Getm_pGameSettings (.AsTres%20Game%20Instance (Utilities|Casting|CastToTresGameInstance (Game|GetGameInstance)))))))))