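; FormChecker1 is a helper that checks whether the player's Sora is in a specific form, judged by material state.
; FormCheck switches on the player's unique ID to pick that Sora variant's material slot and expected texture.
; TextureCheck reads that slot's dynamic material instance, returning true only if FormChangeTex0 matches and AntiVolume is zero.
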(fn ConstructionScript)

(fn FormCheck
  (switch Utilities|FlowControl|Switch|SwitchonETresPlayerUniqueID (Class|TresPawnBase|GetPlayerUniqueID (Variables|Default|Getplayer))
    (:SORA_KH3
      (bind _baseform_ (CallFunction|TextureCheck (Variables|Default|Getplayer) 9 "/Game/Character/pc/p_ex001/mdl/mat0/p_ex001_0d00.p_ex001_0d00"))
      (return _baseform_))
    (:SORA_KH3CA
      (bind _baseform__2 (CallFunction|TextureCheck (Variables|Default|Getplayer) 4 "/Game/Character/pc/p_ca001/mdl/mat0/FormChangeTex/p_ca001_0f00.p_ca001_0f00"))
      (return _baseform__2))
    (:SORA_KH3MI
      (bind _baseform__3 (CallFunction|TextureCheck (Variables|Default|Getplayer) 7 "/Game/Character/pc/p_mi001/mdl/mat0/FormChangeTex/p_mi001_0d00.p_mi001_0d00"))
      (return _baseform__3))
    (:SORA_KH3TS
      (bind _baseform__4 (CallFunction|TextureCheck (Variables|Default|Getplayer) 1 "/Game/Character/pc/p_ts001/mdl/mat0/p_ts001_0d00.p_ts001_0d00"))
      (return _baseform__4))
    (:SORA_KH3BX
      (bind _baseform__5 (CallFunction|TextureCheck (Variables|Default|Getplayer) 7 "/Game/Character/pc/p_ex001/mdl/mat0/p_ex001_0d00.p_ex001_0d00"))
      (return _baseform__5))
    (:SORA_KH2
      (bind _baseform__6 (CallFunction|TextureCheck (Variables|Default|Getplayer) 8 "/Game/Character/pc/p_ex011/mdl/mat0/p_ex011_1d00.p_ex011_1d00"))
      (return _baseform__6))
    (:SORA_KH3DL
      (bind _baseform__7 (CallFunction|TextureCheck (Variables|Default|Getplayer) 7 "/Game/Character/pc/p_dl001/mdl/mat0/p_dl001_0d00.p_dl001_0d00"))
      (return _baseform__7))))

(fn TextureCheck
  (params (Char :type Tres%20Char%20Pawn%20Base%20Object%20Reference) (ElementIndex :type Integer) (Texture :type Texture%202D%20Object%20Reference))
  (bind _asmaterial_instance_dynamic (Utilities|Casting|CastToMaterialInstanceDynamic (Rendering|Material|GetMaterial (Variables|/Script/TresGame.TresCharPawnBase|GetMyMesh Char) ElementIndex)))
  (bind _returnvalue (Rendering|Material|GetTextureParameterValue _asmaterial_instance_dynamic "FormChangeTex0" :!class /Script/Engine.MaterialInstanceDynamic))
  (if (== _returnvalue Texture)
    (bind _returnvalue_2 (Rendering|Material|GetScalarParameterValue _asmaterial_instance_dynamic "AntiVolume" :!class /Script/Engine.MaterialInstanceDynamic))
    (if (== _returnvalue_2 0.0)
      (return true)
      (else
        (return false)))
    (else
      (return false))))