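; Fire dive projectile that damages its target enemy on impact.
; When the sphere hits TargetEnemy it spawns two hit effects, applies damage and destroys itself; a custom hit event does the same without damage.
; The Destroyed event spawns an emitter only when no hit was registered.
; BeginPlay is empty, leaving speed setup, player reference initialization, target arrow attachment and the firing effect disconnected.
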(event OnComponentHit(Sphere)
  (params (HitComponent :type Primitive%20Component%20Object%20Reference) (OtherActor :type Actor%20Object%20Reference) (OtherComp :type Primitive%20Component%20Object%20Reference) (NormalImpulse :type Vector :default "0, 0, 0") (Hit :type Hit%20Result%20Structure%20%28by%20ref%29))
  (bind _returnvalue (Transformation|GetActorLocation))
  (bind _targetenemy (Variables|Default|GetTargetEnemy))
  ;[0 1 1 0.5] On projectile hit
  (if (== OtherActor _targetenemy)
    (Variables|Default|SetIs_Hit true)
    (Effects|SpawnEmitteratLocation (Variables|Default|GetHit_Effect_1) _returnvalue)
    (Effects|SpawnEmitteratLocation (Variables|Default|GetHit_Effect_2) _returnvalue)
    (Game|Damage|ApplyDamage _targetenemy 1e+01 (Variables|Default|GetController) self "/Script/Engine.DamageType")
    (Actor|DestroyActor)))

(event Custom|CustomEvent
  (params (HitComponent :type Primitive%20Component%20Object%20Reference) (OtherActor :type Actor%20Object%20Reference) (OtherComp :type Primitive%20Component%20Object%20Reference) (NormalImpulse :type Vector) (Hit :type Hit%20Result%20Structure%20%28by%20ref%29))
  (bind _returnvalue (Transformation|GetActorLocation))
  (Variables|Default|SetIs_Hit true)
  (Effects|SpawnEmitteratLocation (Variables|Default|GetHit_Effect_1) _returnvalue)
  (Effects|SpawnEmitteratLocation (Variables|Default|GetHit_Effect_2) _returnvalue)
  (Actor|DestroyActor))

(event EventBeginPlay)

(event EventDestroyed
  ;[1 0 0 0.5] Spawn particle effect when projectile is destroyed (but not due to a hit)
  (if (not (Variables|Default|GetIs_Hit))
    (Effects|SpawnEmitteratLocation 0 (Transformation|GetActorLocation) (Transformation|GetActorRotation))))

(fn ConstructionScript)