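; Short-lived enemy magnet attack that drags team 0 characters inward and spins them around its owner.
; Tick pulls pawns overlapping the outer capsule toward the actor; those also inside the revolve capsule become revolvers.
; Captured players lose input and most actions, other pawns have AI stopped, and a timeline rotates them about the owner at its height.
; A timer of about 1.5 seconds releases everyone captured and destroys the actor.
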(event Custom|CustomEvent_0
  (bind _returnvalue (Class|TresGameBlueprintLibrary|GetTresPlayerControllerBase))
  (for _array_element (Variables|Default|GetRevolvers)
    (Utilities|Casting|CastToTresPlayerPawnBase _array_element
      (:then
        (Input|ResetIgnoreMoveInput _returnvalue)
        (Input|ResetIgnoreLookInput _returnvalue)
        (CallFunction|RestrictPlayerMagnet false))
      (:CastFailed
        (Class|TresCharPawnBase|SetStopAI _array_element false))))
  (Actor|DestroyActor))

(event Custom|Revolve
  (bind _returnvalue (Components|GetOwner))
  (bind _returnvalue_2 (Transformation|GetActorLocation _returnvalue))
  (bind (_x _y _z) (Math|Vector|BreakVector _returnvalue_2))
  (Timeline|Timeline_0 Play
    (:Update
      (for _array_element (Variables|Default|GetRevolvers)
        (Transformation|SetActorLocation _array_element (Math|Vector|MakeVector (+ (.X (Math|Vector|BreakVector (Math|Vector|RotateVectorAroundAxis (- (Transformation|GetActorLocation _array_element) _returnvalue_2) 1e+01 "0, 0,1.000000"))) _x) (+ (.Y (Math|Vector|BreakVector (Math|Vector|RotateVectorAroundAxis (- (Transformation|GetActorLocation _array_element) _returnvalue_2) 1e+01 "0, 0,1.000000"))) _y) _z) false false)))))

(event EventBeginPlay
  (bind _outactors (Actor|GetAllActorsOfClass "/Script/TresGame.TresCharPawnBase"))
  (for _array_element _outactors
    (if (== (Class|TresPawnBase|GetTeamNo _array_element) 0)
      (Utilities|Array|Add (Variables|Default|GetPlayerTeam) _array_element)))
  (Utilities|Time|SetTimerbyEvent (delegate Custom|CustomEvent_0) 1.494)
  (CallFunction|Revolve))

(event EventTick
  (params (DeltaSeconds :type Float%20%28single-precision%29))
  (bind _returnvalue (Class|TresGameBlueprintLibrary|GetTresPlayerControllerBase))
  (Variables|Default|SetTimeElapsed (+ DeltaSeconds (Variables|Default|GetTimeElapsed)))
  (for (_array_element _array_index) (Variables|Default|GetPlayerTeam)
    (if (Collision|IsOverlappingActor (Variables|Default|GetCapsule) _array_element :!class /Script/Engine.PrimitiveComponent)
      (Class|TresCharMovementComponent|RequestDirectVelocity (Class|TresCharPawnBase|GetTresCharMovementComponent _array_element) (Math|Vector|MakeVector (* (.X (Math|Vector|BreakVector (Math|Vector|GetUnitDirection(Vector) (Transformation|GetActorLocation _array_element) (Transformation|GetActorLocation)))) 1.25e+03) (* (.Y (Math|Vector|BreakVector (Math|Vector|GetUnitDirection(Vector) (Transformation|GetActorLocation _array_element) (Transformation|GetActorLocation)))) 1.25e+03) (* (.Z (Math|Vector|BreakVector (Math|Vector|GetUnitDirection(Vector) (Transformation|GetActorLocation _array_element) (Transformation|GetActorLocation)))) 1.25e+03)))
      (if (Collision|IsOverlappingActor (Variables|Default|GetRevolveCapsule) _array_element :!class /Script/Engine.PrimitiveComponent)
        (Utilities|Array|Add (Variables|Default|GetRevolvers) _array_element)
        (Utilities|Casting|CastToTresPlayerPawnBase _array_element
          (:then
            (Input|SetIgnoreMoveInput _returnvalue true)
            (Input|SetIgnoreLookInput _returnvalue true)
            (CallFunction|RestrictPlayerMagnet true))
          (:CastFailed
            (Class|TresCharPawnBase|SetStopAI _array_element true)))
        (Utilities|Array|RemoveIndex (Variables|Default|GetPlayerTeam) _array_index)))))

(fn ConstructionScript)

(fn RestrictPlayerMagnet
  (params (Restrict? :type Boolean))
  (bind _returnvalue (Class|TresGameBlueprintLibrary|GetTresPlayerControllerBase))
  (bind _returnvalue_2 (not Restrict?))
  (Class|TresPlayerControllerBase|SetRestrictStyle _returnvalue Restrict?)
  (Class|TresPlayerControllerBase|SetRestrictFriend _returnvalue Restrict?)
  (Class|TresPlayerControllerBase|SetRestrictLink _returnvalue Restrict?)
  (Class|TresPlayerControllerBase|SetRestrictAttack _returnvalue Restrict?)
  (Class|TresPlayerControllerBase|SetRestrictAttraction _returnvalue Restrict?)
  (Class|TresPlayerControllerBase|SetRestrictShootLock _returnvalue Restrict?)
  (Class|TresPlayerControllerBase|SetRestrictDiveFall _returnvalue Restrict?)
  (Class|TresPlayerControllerBase|SetRestrictJump _returnvalue Restrict?)
  (Class|TresPlayerControllerBase|SetAbilityAthleticFlow _returnvalue (not Restrict?))
  (Class|TresPlayerControllerBase|SetRestrictGuard _returnvalue Restrict?)
  (Class|TresPlayerControllerBase|SetRestrictMagic _returnvalue Restrict?)
  (Class|TresPlayerControllerBase|SetRestrictItem _returnvalue Restrict?)
  (Class|TresPlayerControllerBase|SetRestrictWeapon _returnvalue false)
  (Class|TresPlayerControllerBase|SetRestrictSituation _returnvalue false)
  (Class|TresPlayerControllerBase|SetAbility2ndJump _returnvalue _returnvalue_2)
  (Class|TresPlayerControllerBase|SetAbilityAirSlide _returnvalue _returnvalue_2)
  (return))