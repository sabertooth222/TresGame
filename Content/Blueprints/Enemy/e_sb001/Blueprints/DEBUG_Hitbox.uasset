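; Debug actor for the e_sb001 enemy that prints its horizontal distance to the player on screen.
; BeginPlay caches an E_sb001_Pawn found in the level, keeping the last one, and Tick shows the distance to player pawn 0 as a cutscene subtitle.
; An unwired branch, which never runs, would add static meshes at the first weapon's attack collision shapes, unhide that collision and destroy the debug actor.
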(event EventBeginPlay
  (bind _outactors (Actor|GetAllActorsOfClass "/Game/Blueprints/Enemy/e_sb001/e_sb001_Pawn.e_sb001_Pawn_C"))
  (for _array_element _outactors
    (Variables|Default|Setesb001 _array_element)))

(event EventTick
  (params (DeltaSeconds :type Float%20%28single-precision%29))
  (Class|TresGameBlueprintLibrary|TresUIOpenSubtitle (Utilities|Struct|MakeTresLocText "" "" (Variables|Default|GetNewVar_0) (Utilities|String|ToString(Float) (Transformation|GetHorizontalDistanceTo (Variables|Default|Getesb001) (Class|TresGameBlueprintLibrary|GetTresPlayerPawnBase)))) "Cutscene"))

(fn ConstructionScript)