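; One-shot helper actor that switches an e_sb001 pawn to dual keyblade weapons, W_so200 in the right hand and W_so210 in the left.
; On BeginPlay it destroys the pawn's equipped weapons, then spawns both replacements, copies the pawn's data table set and base params onto each weapon and its attack collision, and snaps them to the hand sockets.
; It writes the pair back into the pawn's equipment list and destroys itself after a short delay.
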(event EventBeginPlay
  (bind _e_sb001_pawn (Variables|Default|Gete_sb001_pawn))
  (bind _e_sb001_pawn_2 (Variables|Default|Gete_sb001_pawn))
  (bind _m_pdatatableset (Variables|/Script/TresGame.TresPawnBase|Getm_pDataTableSet _e_sb001_pawn))
  (bind _m_pdatatableset_2 (Variables|/Script/TresGame.TresPawnBase|Getm_pDataTableSet _e_sb001_pawn_2))
  (for _array_element (Variables|/Script/TresGame.TresEquipmentComponent|Getm_WeaponEquips (Variables|/Script/TresGame.TresCharPawnBase|GetMyEquipment (Variables|Default|Gete_sb001_pawn)))
    (Actor|DestroyActor (stale _astres_weapon_base)))
  (bind _returnvalue (Game|SpawnActorfromClass "/Game/Blueprints/Player/p_ex001/w_so200_Wep.w_so200_Wep_C" (Math|Transform|MakeTransform "0, 0, 0") "Undefined" (Variables|Default|Gete_sb001_pawn) 0))
  (bind _output_get (Variables|Default|SetWeapon (.AsTres%20Weapon%20Keyblade%20Base (Utilities|Casting|CastToTresWeaponKeybladeBase _returnvalue))))
  (Variables|/Script/TresGame.TresWeaponBase|Setm_pOwnerDataTableSet (Variables|Default|GetWeapon) _m_pdatatableset)
  (Variables|/Script/TresGame.TresPawnBase|Setm_pBaseParam (Variables|Default|GetWeapon) (Variables|/Script/TresGame.TresPawnBase|Getm_pBaseParam (Variables|Default|Gete_sb001_pawn)))
  (Variables|/Script/TresGame.TresAtkCollComponent|Setm_pOwnerDataTableSet (Variables|/Script/TresGame.TresWeaponBase|GetMyAtkColl _output_get) _m_pdatatableset)
  (Variables|/Script/TresGame.TresAtkCollComponent|Setm_pOwnerBaseParam (Variables|/Script/TresGame.TresWeaponBase|GetMyAtkColl _output_get) (Variables|/Script/TresGame.TresPawnBase|Getm_pBaseParam (Variables|Default|Gete_sb001_pawn)))
  (Transformation|AttachComponentToComponent _output_get (Variables|/Script/TresGame.TresCharPawnBase|GetMyMesh (Variables|Default|Gete_sb001_pawn)) "R_wep_skt" "SnapToTarget" "SnapToTarget" "KeepRelative" true)
  (Variables|/Script/TresGame.TresWeaponBase|SetMyPawn (Variables|Default|GetWeapon) (Variables|Default|Gete_sb001_pawn))
  (Variables|Default|SetRWeapon (Variables|Default|GetWeapon))
  (bind _returnvalue_2 (Game|SpawnActorfromClass "/Game/Blueprints/Player/p_ex001/w_so210_Wep.w_so210_Wep_C" (Math|Transform|MakeTransform "0, 0, 0") "Undefined" (Variables|Default|Gete_sb001_pawn) 0))
  (bind _output_get_2 (Variables|Default|SetWeapon (.AsTres%20Weapon%20Keyblade%20Base (Utilities|Casting|CastToTresWeaponKeybladeBase _returnvalue_2))))
  (Variables|/Script/TresGame.TresWeaponBase|Setm_pOwnerDataTableSet (Variables|Default|GetWeapon) _m_pdatatableset_2)
  (Variables|/Script/TresGame.TresPawnBase|Setm_pBaseParam (Variables|Default|GetWeapon) (Variables|/Script/TresGame.TresPawnBase|Getm_pBaseParam (Variables|Default|Gete_sb001_pawn)))
  (Variables|/Script/TresGame.TresAtkCollComponent|Setm_pOwnerDataTableSet (Variables|/Script/TresGame.TresWeaponBase|GetMyAtkColl _output_get_2) _m_pdatatableset_2)
  (Variables|/Script/TresGame.TresAtkCollComponent|Setm_pOwnerBaseParam (Variables|/Script/TresGame.TresWeaponBase|GetMyAtkColl _output_get_2) (Variables|/Script/TresGame.TresPawnBase|Getm_pBaseParam (Variables|Default|Gete_sb001_pawn)))
  (Transformation|AttachComponentToComponent _output_get_2 (Variables|/Script/TresGame.TresCharPawnBase|GetMyMesh (Variables|Default|Gete_sb001_pawn)) "L_wep_skt" "SnapToTarget" "SnapToTarget" "KeepRelative" true)
  (Variables|/Script/TresGame.TresWeaponBase|SetMyPawn (Variables|Default|GetWeapon) (Variables|Default|Gete_sb001_pawn))
  (Variables|/Script/TresGame.TresEquipmentComponent|Setm_WeaponEquips (Variables|/Script/TresGame.TresCharPawnBase|GetMyEquipment (Variables|Default|Gete_sb001_pawn)) (Utilities|Array|MakeArray (Variables|Default|GetRWeapon) (Variables|Default|GetWeapon)))
  (Utilities|FlowControl|Delay 0.2)
  (Actor|DestroyActor self))

(fn ConstructionScript)