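; Manager actor for the Sora boss's twin-copies phase, spawning DF and LF pawns on either side of the boss.
; On BeginPlay it starts a cinematic level sequence, stops the twins' AI, and hides the boss, making it invincible and untargetable.
; When the sequence finishes, a delay precedes ending cinematic mode and restarting boss AI.
; Once both twins are destroyed, it sets the boss blackboard's "CanAttack?" and destroys itself, without unhiding the boss.
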(event Custom|CustomEvent_0
  (params (DestroyedActor :type Actor%20Object%20Reference))
  (Variables|Default|SetDeathCount (+ (Variables|Default|GetDeathCount) 1))
  (if (> (Variables|Default|GetDeathCount) 1)
    (AI|Components|Blackboard|SetValueasBool (AI|GetBlackboard (Variables|Default|GetSoraBoss_Pawn')) (Utilities|Name|MakeLiteralName "CanAttack?") true)
    (Class|TresGameBlueprintLibrary|TresUIOpenSubtitle (Utilities|Struct|MakeTresLocText "" "" (Variables|Default|GetNewVar_0) "Can attack = true") "Cutscene")
    (Actor|DestroyActor self)))

(event Custom|camera_onFinished
  (Class|TresGameBlueprintLibrary|TresUIOpenSubtitle (Utilities|Struct|MakeTresLocText "" "" (Variables|Default|GetNewVar_0) "cameraend") "Cutscene")
  (Utilities|FlowControl|Delay 5.0)
  (Class|TresGameBlueprintLibrary|TresEndCinematicMode false false)
  (Class|TresGameBlueprintLibrary|ResetTresCameraNormal false)
  (Class|TresCharPawnBase|SetStopAI (Variables|Default|GetSoraBoss_Pawn') false))

(event EventBeginPlay
  (bind _soraboss_pawn_ (Variables|Default|GetSoraBoss_Pawn'))
  (bind _soraboss_pawn__2 (Variables|Default|GetSoraBoss_Pawn'))
  (bind _returnvalue (Transformation|GetActorRotation _soraboss_pawn__2))
  (bind _returnvalue_2 (Transformation|GetActorLocation _soraboss_pawn__2))
  (bind _returnvalue_3 (Transformation|GetActorRightVector _soraboss_pawn__2))
  (bind _returnvalue_4 (* _returnvalue_3 -200))
  (bind _returnvalue_5 (* _returnvalue_3 200))
  (bind _returnvalue_6 (+ _returnvalue_2 _returnvalue_5))
  (bind _returnvalue_7 (+ _returnvalue_2 _returnvalue_4))
  (Class|TresGameBlueprintLibrary|ResetTresCameraNormal false)
  (Class|TresGameBlueprintLibrary|TresStartCinematicMode false true true true false false false false false false false false false)
  (bind _outactor (Sequencer|Player|CreateLevelSequencePlayer "/Game/Blueprints/Enemy/e_sb001/Camera/levelsequence_test.levelsequence_test"))
  (Sequencer|Player|Play (Variables|/Script/LevelSequence.LevelSequenceActor|GetSequencePlayer _outactor) :!class /Script/MovieScene.MovieSceneSequencePlayer)
  (EventDispatchers|BindEventtoOnFinished (Variables|/Script/LevelSequence.LevelSequenceActor|GetSequencePlayer _outactor) (delegate Custom|camera_onFinished))
  (bind _returnvalue_8 (AI|SpawnAIFromClass "/Game/Blueprints/Enemy/e_sb001_DF/e_sb001DF_Pawn.e_sb001DF_Pawn_C" 0 _returnvalue_6 _returnvalue false))
  (bind _ase_sb_001df_pawn (Utilities|Casting|CastToe_sb001DF_Pawn _returnvalue_8)
    (:then
      (bind _output_get (Variables|Default|SetDF_Pawn _ase_sb_001df_pawn))
      (Transformation|SetActorLocation _output_get _returnvalue_6 false false)
      (Effects|SpawnEmitterAttached "/Game/Effects/dlc01/wep/w_so220/par/vw_so220_brs_blk00.vw_so220_brs_blk00" (Variables|/Script/Engine.Actor|GetRootComponent _output_get) "None")
      (bind _returnvalue_9 (AI|SpawnAIFromClass "/Game/Blueprints/Enemy/e_sb001_LF/e_sb001LF_Pawn.e_sb001LF_Pawn_C" 0 _returnvalue_7 _returnvalue false))
      (bind _ase_sb_001lf_pawn (Utilities|Casting|CastToe_sb001LF_Pawn _returnvalue_9)
        (:then
          (bind _output_get_2 (Variables|Default|SetLF_Pawn _ase_sb_001lf_pawn))
          (Transformation|SetActorLocation _output_get_2 _returnvalue_7 false false)
          (Effects|SpawnEmitterAttached "/Game/Effects/dlc01/wep/w_so220/par/vw_so220_brs_lgt00.vw_so220_brs_lgt00" (Variables|/Script/Engine.Actor|GetRootComponent _output_get_2) "None")
          (Utilities|FlowControl|Delay 0.1)
          (Class|TresCharPawnBase|SetStopAI (Variables|Default|GetDF_Pawn) true)
          (Game|BindEventtoOnDestroyed (Variables|Default|GetDF_Pawn) (delegate Custom|CustomEvent_0))
          (Game|BindEventtoOnDestroyed (Variables|Default|GetLF_Pawn) (delegate Custom|CustomEvent_0))
          (Variables|Default|SetHidden? true)
          (Class|TresCharMovementComponent|SetMovementMode (Variables|/Script/TresGame.TresCharPawnBase|GetMyMovement (Variables|Default|GetSoraBoss_Pawn')) "MOVE_Flying")
          (Effects|SpawnEmitteratLocation "/Game/Effects/dlc01/wep/w_so220/par/vw_so220_fin_plr_s0.vw_so220_fin_plr_s0" (Transformation|GetActorLocation (Variables|Default|GetSoraBoss_Pawn')))
          (Collision|SetActorEnableCollision _soraboss_pawn_ (not (Variables|Default|GetHidden?)))
          (Class|TresCharPawnBase|SetConditionInvincible _soraboss_pawn_ (Variables|Default|GetHidden?))
          (for _array_element (Actor|GetAttachedActors (Variables|Default|GetSoraBoss_Pawn'))
            (Rendering|SetActorHiddenInGame _array_element (Variables|Default|GetHidden?)))
          (for _array_element_2 (Actor|GetComponentsByClass (Variables|Default|GetSoraBoss_Pawn') "/Script/TresGame.TresLockonTargetComponent")
            (Variables|/Script/TresGame.TresLockonTargetComponent|Setm_bPermissionLockOn _array_element_2 (not (Variables|Default|GetHidden?)))
            (Variables|/Script/TresGame.TresLockonTargetComponent|Setm_bPermissionMoveFlow _array_element_2 (not (Variables|Default|GetHidden?)))
            (Variables|/Script/TresGame.TresLockonTargetComponent|Setm_bPermissionShootFlow _array_element_2 (not (Variables|Default|GetHidden?))))
          (Rendering|SetActorHiddenInGame (Variables|Default|GetSoraBoss_Pawn') (Variables|Default|GetHidden?)))
        (:CastFailed
          (Class|TresGameBlueprintLibrary|TresUIOpenSubtitle (Utilities|Struct|MakeTresLocText "" "" (Variables|Default|GetNewVar_0) "lf cast fail") "Cutscene"))))
    (:CastFailed
      (Class|TresGameBlueprintLibrary|TresUIOpenSubtitle (Utilities|Struct|MakeTresLocText "" "" (Variables|Default|GetNewVar_0) "df cast fail") "Cutscene"))))

(fn ConstructionScript)