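; CutsceneFixActor makes Matinee cutscenes use the current player character's mesh in place of listed character IDs.
; Every tick while the player pawn is in the cinematic state, it scans the interp groups of all MatineeActors.
; Groups whose MCharacterMesh appears in CharacterIDs count as player groups.
; Their MCharacterMesh is overwritten with the first seven characters of the player's skeletal mesh name, which serve as the character ID.
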(event EventTick
  (params (DeltaSeconds :type Float%20%28single-precision%29))
  (bind _returnvalue (Class|TresGameBlueprintLibrary|GetTresPlayerPawnBase))
  (if (Utilities|Enum|Equal(Enum) (Class|TresCharPawnBase|GetStateID _returnvalue) "TSID_STATE_CINEMATIC")
    (bind _outactors (Actor|GetAllActorsOfClass "/Script/Engine.MatineeActor"))
    (for _array_element _outactors
      (for _array_element_2 (Variables|/Script/Engine.InterpData|GetInterpGroups (Variables|/Script/Engine.MatineeActor|GetMatineeData _array_element))
        (bind _containspid (CallFunction|IsPlayerGroup (.AsTres%20Interp%20Group (Utilities|Casting|CastToTresInterpGroup _array_element_2))))
        (if _containspid
          (Variables|/Script/TresGame.TresInterpGroup|Setm_CharacterMesh (.AsTres%20Interp%20Group (Utilities|Casting|CastToTresInterpGroup _array_element_2)) (Utilities|String|Left (Utilities|GetObjectName (Variables|/Script/Engine.SkinnedMeshComponent|GetSkeletalMesh (Variables|/Script/TresGame.TresCharPawnBase|GetMyMesh _returnvalue))) 7)))))))

(fn ConstructionScript)

(fn IsPlayerGroup
  (params (InterpGroup :type Tres%20Interp%20Group%20Object%20Reference))
  (return (Utilities|Array|ContainsItem (LocalVariables|GetCharacterIDs) (Variables|/Script/TresGame.TresInterpGroup|Getm_CharacterMesh InterpGroup))))