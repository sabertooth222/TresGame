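; Helper actor that plays a camera animation through the CameraManager and manages its timed end.
; PlayCustomAnim maps a settings struct to a play space and playback parameters, returning the anim, duration and end type.
; AnimationEndType starts a timer that, on expiry, optionally stops all camera anims, then destroys the actor.
; PlayCameraRandom and PlaySQEXAnim are empty, and no event here calls PlayCustomAnim.
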(event Custom|PlayCameraRandom)

(event Custom|AnimationEndType
  (bind _returnvalue (Utilities|Time|SetTimerbyEvent (delegate Custom|DurationEnd) (Variables|Default|GetCurrent%20Camera%20Anim%20Duration)))
  (Variables|Default|SetTimerUntilDurationEnd _returnvalue))

(event Custom|DurationEnd
  (if (Variables|Default|GetStopAnimationAtDurationEnd)
    (CallFunction|StopCameraAnim))
  (Actor|DestroyActor))

(event Custom|StopCameraAnim
  (Class|PlayerCameraManager|StopAllCameraAnims (Variables|Default|GetCamera%20Manager) (Variables|Default|GetStop%20Immediately?)))

(event EventBeginPlay)

(event Collision|EventActorBeginOverlap
  (params (OtherActor :type Actor%20Object%20Reference)))

(event EventTick
  (params (DeltaSeconds :type Float%20%28single-precision%29)))

(fn ConstructionScript)