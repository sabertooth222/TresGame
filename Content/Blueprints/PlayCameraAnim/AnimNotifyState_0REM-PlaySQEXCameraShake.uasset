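; Anim notify state that plays a camera shake on the local Tres camera manager for the span of an animation notify.
; On begin it takes either a SQEX preset or a custom shake class and plays it in camera-local space at the set scale.
; The preset helper shows only one assigned shake, Shake_super_kokizami_1sec.
; On end it immediately stops all camera shakes on that manager, not just its own.
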(fn ReceivedNotifyBegin
  (params (MeshComp :type Skeletal%20Mesh%20Component%20Object%20Reference) (Animation :type Anim%20Sequence%20Base%20Object%20Reference) (TotalDuration :type Float%20%28single-precision%29))
  (bind _returnvalue (Class|TresGameBlueprintLibrary|GetLocalTresCameraManager MeshComp))
  (switch Utilities|FlowControl|Switch|SwitchonCameraAnim_TypeOfCameraShake (Variables|Default|GetCamera%20Shake%20Type)
    (:NewEnumerator0
      (|SQEXCameraShake))
    (:NewEnumerator1
      (LocalVariables|SetFinal%20Camera%20Shake (Variables|Default|GetCustom%20Camera%20Shake))))
  (Class|TresGameBlueprintLibrary|ClientPlayCameraShake _returnvalue (LocalVariables|GetFinal%20Camera%20Shake) _returnvalue (Variables|Default|GetScale) "CameraLocal" "0, 0, 0")
  (return false))

(fn ReceivedNotifyEnd
  (params (MeshComp :type Skeletal%20Mesh%20Component%20Object%20Reference) (Animation :type Anim%20Sequence%20Base%20Object%20Reference))
  (CameraShake|StopAllCameraShakes (Class|TresGameBlueprintLibrary|GetLocalTresCameraManager MeshComp) true)
  (return false))