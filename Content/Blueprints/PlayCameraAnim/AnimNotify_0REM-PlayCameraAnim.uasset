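; Anim notify that plays or stops Tres camera animations from an animation, optionally only when the performance (Keyblade cinematic combo) camera is enabled.
; A function switch plays a RandomCameraAnim setting as a SQUARE ENIX or custom camera, spawns a WIP smart-camera actor, or stops chosen or all animations.
; An optional spawned state-check actor handles camera reset on state changes such as hurt or combo; both stop modes end existing checkers.
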(fn ReceivedNotify
  (params (MeshComp :type Skeletal%20Mesh%20Component%20Object%20Reference) (Animation :type Anim%20Sequence%20Base%20Object%20Reference))
  (LocalVariables|SetPawn (.AsTres%20Char%20Pawn%20Base (Utilities|Casting|CastToTresCharPawnBase (Components|GetOwner MeshComp))))
  (LocalVariables|SetCamera%20Manager (Class|TresGameBlueprintLibrary|GetLocalTresCameraManager))
  (LocalVariables|SetPlayer%20Controller (Class|TresGameBlueprintLibrary|GetLocalTresPlayerControllerBase))
  (if (Variables|Default|GetPlay%20Only%20If%20Keyblade%20Cinematic%20/%20Combo%20Cam%20Enabled)
    (if (and (Class|TresGameBlueprintLibrary|TresIsGameEnablePerformanceCamera) (Class|TresGameBlueprintLibrary|TresIsConfigEnablePerformanceCamera))
      _
      (else
        (return false))))
  (if (not (Variables|Default|GetReset%20Camera?))
    _
    (else
      _))
  (switch Utilities|FlowControl|Switch|SwitchonPlayCameraAnim_Function (Variables|Default|GetNotify%20Function)
    (:NewEnumerator0
      (bind _output_get (LocalVariables|SetFinalCameraAnimSetting (|RandomCameraAnim)))
      (switch Utilities|FlowControl|Switch|SwitchonCameraAnim_MainChoice (.CameraAnimationType (Utilities|Struct|BreakPlayCameraAnimSettings _output_get))
        (:NewEnumerator0
          (bind _sqex_camera_anim (CallFunction|CameraAnimFetchSQEXCamera (.SquareEnixCamera (Utilities|Struct|BreakPlayCameraAnimSettings _output_get))))
          (LocalVariables|SetFinalCameraAnim _sqex_camera_anim))
        (:NewEnumerator1
          (LocalVariables|SetFinalCameraAnim (.CustomCamera-Animation (Utilities|Struct|BreakPlayCameraAnimSettings _output_get)))))
      (if (.bSuccess (Utilities|Casting|CastToTresCameraAnim (Class|TresCameraManager|GetActiveCamera (LocalVariables|GetCamera%20Manager))))
        (LocalVariables|SetEvent%20Camera (.AsTres%20Camera%20Anim (Utilities|Casting|CastToTresCameraAnim (Class|TresCameraManager|GetActiveCamera (LocalVariables|GetCamera%20Manager))))))
      (bind _active_event_camera (CallFunction|PlaySQEXCamera (LocalVariables|GetPawn) (LocalVariables|GetEvent%20Camera) (.EventCameraLabel (Utilities|Struct|BreakPlayCameraAnimSettings _output_get)) (LocalVariables|GetFinalCameraAnim) (.AttachEventCamera? (Utilities|Struct|BreakPlayCameraAnimSettings _output_get)) (.AttachCameraTarget (Utilities|Struct|BreakPlayCameraAnimSettings _output_get)) (.IfNoEnemyLock-OnAttachtoPlayer? (Utilities|Struct|BreakPlayCameraAnimSettings _output_get)) (.DoesAnimationLoop? (Utilities|Struct|BreakPlayCameraAnimSettings _output_get)) (.EventCameraTakeover? (Utilities|Struct|BreakPlayCameraAnimSettings _output_get)) (.EventCameraAuto-End? (Utilities|Struct|BreakPlayCameraAnimSettings _output_get)) (.EventCameraTakeoverATEND? (Utilities|Struct|BreakPlayCameraAnimSettings _output_get)) (CallFunction|SQEXCameraSetParameters (.StartingParametersInterpolationBlendetc (Utilities|Struct|BreakPlayCameraAnimSettings _output_get))) (CallFunction|SQEXCameraSetParameters (.EndingParameters (Utilities|Struct|BreakPlayCameraAnimSettings _output_get))) (.PlayRate (Utilities|Struct|BreakPlayCameraAnimSettings _output_get)) (.Scale (Utilities|Struct|BreakPlayCameraAnimSettings _output_get)) (.CameraDuration (Utilities|Struct|BreakPlayCameraAnimSettings _output_get))))
      (LocalVariables|SetActiveEventCamera _active_event_camera))
    (:NewEnumerator4
      (Game|SpawnActorfromClass "/Game/Blueprints/PlayCameraAnim/PlaySmartCameraAnim_Actor.PlaySmartCameraAnim_Actor_C" (Math|Transform|MakeTransform "0, 0, 0" "0, 0, 0" "1,1,1") "Undefined" 0 (LocalVariables|GetPawn) (LocalVariables|GetPlayer%20Controller) (LocalVariables|GetCamera%20Manager) (Variables|Default|GetSmart%20-%20Stop%20Camera%20Anim%20on%20Duration%20End?) (Variables|Default|GetSmart%20-%20Stop%20Camera%20Immediately?) 0))
    (:NewEnumerator3
      (for _array_element (Variables|Default|GetCamera%20Animation)
        (Class|PlayerCameraManager|StopAllInstancesOfCameraAnim (LocalVariables|GetCamera%20Manager) _array_element false))
      (|ClearStateCheckers :!label _label
        (:Completed
          _)))
    (:NewEnumerator2
      (Class|PlayerCameraManager|StopAllCameraAnims (LocalVariables|GetCamera%20Manager) false)
      (goto _label)))
  (if (Variables|Default|GetReset%20Camera%20on%20New%20State?%20%28Hurt,%20Combo,%20etc%29)
    (Game|SpawnActorfromClass "/Game/Blueprints/PlayCameraAnim/PlayCameraAnim_StateCheck_Actor.PlayCameraAnim_StateCheck_Actor_C" (Math|Transform|MakeTransform "0, 0, 0" "0, 0, 0" "1,1,1") "Undefined" 0 (LocalVariables|GetPawn) (Variables|Default|GetReset%20-%20End%20Camera%20Function) (LocalVariables|GetFinalCameraAnimSetting) (LocalVariables|GetActiveEventCamera) (Variables|Default|GetReset%20-%20End%20Immediately?%20%28UE4%29) (Variables|Default|GetReset%20-%20Enable%20Takeover?%20%28SQEX%29) (Variables|Default|GetReset%20-%20End%20Camera%20Parameters%20%28SQEX%29) (Variables|Default|GetReset%20-%20Reset%20for%20PlayAnims?%20%28%20SHEX,%20RCEX,%20etc%29) 0))
  (return false))