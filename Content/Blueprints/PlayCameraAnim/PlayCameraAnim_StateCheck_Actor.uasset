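; Helper actor that watches a pawn during a played camera animation and ends that event camera early when the pawn changes action.
; On BeginPlay it destroys other instances of itself, then binds to the pawn's state event and optionally ticks to detect animation changes.
; A listed state or changed animation ends the SQEX camera and destroys the actor.
; A camera-duration timer only destroys the actor.
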(event Custom|OnCtorState_Event_0
  (params (StateID :type ETresStateID%20Enum :default "TSID_STATE_EMPTY"))
  (|StateChecker StateID
    (:NEW%20VALID%20STATE
      (CallFunction|ENDCAM))))

(event Custom|ENDCAM
  (CallFunction|SQEXCameraEndCameraEarly (Variables|Default|GetPawn) (Variables|Default|GetEnd%20Camera%20Function) (Variables|Default|GetImmediate?%20%28UE4%29) (Variables|Default|GetTakeover?%20%28SQEX%29) (Utilities|Struct|BreakPlayCameraAnimSettings (Variables|Default|GetFinalCameraAnimSetting)) (Variables|Default|GetCamera%20Params) (Variables|Default|GetActiveEventCamera))
  (Actor|DestroyActor))

(event Custom|END
  (Actor|DestroyActor))

(event Custom|ENDTIMER
  (CallFunction|END))

(event EventBeginPlay
  (|CloneCheck
    (:Completed
      (Variables|Default|SetCurrent%20Anim (Class|TresCharPawnBase|AnimGetLastPlayAnimName (Variables|Default|GetPawn) "None"))
      (if (Variables|Default|GetInclude%20PlayAnim%20Check)
        (Actor|Tick|SetActorTickEnabled true))
      (EventDispatchers|AssignOnCtorState (Variables|Default|GetPawn) (delegate Custom|OnCtorState_Event_0))
      (Utilities|Time|SetTimerbyEvent (delegate Custom|ENDTIMER) (Utilities|Struct|BreakPlayCameraAnimSettings (Variables|Default|GetFinalCameraAnimSetting))))))

(event EventTick
  (params (DeltaSeconds :type Float%20%28single-precision%29))
  (if (Utilities|Name|NotEqual(Name) (Class|TresCharPawnBase|AnimGetLastPlayAnimName (Variables|Default|GetPawn) "None") (Variables|Default|GetCurrent%20Anim))
    (CallFunction|ENDCAM)
    (Actor|Tick|SetActorTickEnabled false)))

(fn ConstructionScript)