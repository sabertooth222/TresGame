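; Test actor for moving and rotating clock particle effects, spawning separate Mini_clock and Mini_shorthand emitters at its location on BeginPlay.
; A timeline rotates and nudges the actor each update while rolling the shorthand emitter through a full turn from its initial roll, keeping its initial yaw.
; Tick moves both emitters to the actor's location rather than attaching them.
; Several disconnected experiments, including an attached-emitter variant, never run.
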(event EventBeginPlay
  (bind _returnvalue (Effects|SpawnEmitteratLocation "/Game/Effects/magicmickey/mini_clock.mini_clock" (Transformation|GetActorLocation) "0,47.000000, 0"))
  (Variables|Default|SetNewVar_0 _returnvalue)
  (bind _returnvalue_2 (Effects|SpawnEmitteratLocation "/Game/Effects/magicmickey/mini_shorthand.mini_shorthand" (Transformation|GetActorLocation) "0,47.000000,0.000000"))
  (bind _output_get (Variables|Default|Setparticle _returnvalue_2))
  (Variables|Default|Setrot (Transformation|GetWorldRotation _output_get))
  (bind _newtrack_0 (Timeline|Timeline_0 Play)
    (:Update
      (Class|Actor|AddActorWorldRotation "0,1.000000, 0")
      (Transformation|AddActorLocalOffset "1.000000,1.000000, 0" false false)
      (Transformation|SetWorldRotation (Variables|Default|Getparticle) (Math|Rotator|MakeRotator (+ (Math|Float|Lerp 0.0 3.6e+02 _newtrack_0) (.Roll (Math|Rotator|BreakRotator (Variables|Default|Getrot)))) 0.0 (.Yaw (Math|Rotator|BreakRotator (Variables|Default|Getrot)))) false false))))

(event EventTick
  (params (DeltaSeconds :type Float%20%28single-precision%29))
  (Transformation|SetWorldLocation (Variables|Default|GetNewVar_0) (Transformation|GetActorLocation) false false))

(fn ConstructionScript)