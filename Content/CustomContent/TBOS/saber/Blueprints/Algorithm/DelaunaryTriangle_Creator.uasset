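; Dungeon generator actor that builds a Delaunay triangulation over room center positions on BeginPlay to feed corridor pathing.
; Runs Bowyer-Watson in 2D: super triangle, circumcircle tests per inserted point, then removal of triangles touching the super triangle.
; Passes triangles to a spawned MinimumSpanningTree actor.
; If the super-triangle check fails, sorts rooms along a line and sends chained edges straight to DungeonMaster instead.
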(event EventBeginPlay
  (for _array_element (Variables|Default|GetRoomCenters)
    (Utilities|Array|Add (Variables|Default|GetRoomCenter_Vectors) (Math|Conversions|ToVector2D(Vector) (Transformation|GetActorLocation _array_element))))
  (bind (_output _supertriangle_failed) (CallFunction|Bowyer-WatsonAlgorithm (Variables|Default|GetRoomCenter_Vectors)))
  (if _supertriangle_failed
    (bind _returnedges (CallFunction|StraightLine-Algorithm))
    (Default|PathAlgorithmFinished (Variables|Default|GetDungeonMaster) _returnedges)
    (else
      (bind _returnvalue (Game|SpawnActorfromClass "/Game/CustomContent/TBOS/saber/Blueprints/Algorithm/MinimumSpanningTree.MinimumSpanningTree_C" (Math|Transform|MakeTransform "0, 0, 0") "Undefined" 0 (Variables|Default|GetDungeonMaster) 0))
      (Default|CreateMinSpanTree _returnvalue _output))))

(fn ConstructionScript)

(fn FindSuperTriangle
  (params (Points :type Array%20of%20Vector%202D%20Structures))
  ;[1 1 1] Init ridiculous min/max
  (LocalVariables|SetMinX 1e+06)
  (LocalVariables|SetMinY 1e+06)
  (LocalVariables|SetMaxX -1e+06)
  (LocalVariables|SetMaxY -1e+06)
  ;[1 1 1] Find the super-encompassing triangle around all of our points
  (for _array_element Points
    (LocalVariables|SetMinX (Math|Float|Min(Float) (.x _array_element) (LocalVariables|GetMinX)))
    (LocalVariables|SetMinY (Math|Float|Min(Float) (.y _array_element) (LocalVariables|GetMinY)))
    (LocalVariables|SetMaxX (Math|Float|Max(Float) (.x _array_element) (LocalVariables|GetMaxX)))
    (LocalVariables|SetMaxY (Math|Float|Max(Float) (.y _array_element) (LocalVariables|GetMaxY))))
  ;[1 1 1] Finds distance between min/max x + y...and multiplies it by 10...for some reason
  (LocalVariables|Setdx (- (LocalVariables|GetMaxX) (LocalVariables|GetMinX)))
  (LocalVariables|Setdy (- (LocalVariables|GetMaxY) (LocalVariables|GetMinY)))
  (return (Utilities|Struct|MakeTriangle (Math|Vector2D|MakeVector2D (- (LocalVariables|GetMinX) (LocalVariables|Getdx)) (- (LocalVariables|GetMinY) (* (LocalVariables|Getdy) 3.0))) (Math|Vector2D|MakeVector2D (- (LocalVariables|GetMinX) (LocalVariables|Getdx)) (+ (LocalVariables|GetMaxY) (LocalVariables|Getdy))) (Math|Vector2D|MakeVector2D (+ (LocalVariables|GetMaxX) (* (LocalVariables|Getdx) 3.0)) (+ (LocalVariables|Getdy) (LocalVariables|GetMaxY))))))

(fn AddVertex
  (params (%20 :type Vector%202D%20Structure) (triangles :type Array%20of%20Triangle%20Structures))
  (bind _new_edges_2 (LocalVariables|Getnew%20edges%202))
  ;[0 0.6953 1] initialize
  (LocalVariables|SetVertex %20)
  (Utilities|Array|Clear (LocalVariables|Getnew%20triangles%20))
  (Utilities|Array|Clear (LocalVariables|Getedges))
  (for _array_element triangles
    (bind _is_ (CallFunction|IsinCircumcircle? (LocalVariables|GetVertex) _array_element))
    ;[1 1 1] First iteration will be true since every point should be inside super triangle
    (if _is_ ; inCircumcircle?
      (Utilities|Array|Add (LocalVariables|Getedges) (Utilities|Struct|MakeLine (.A (Utilities|Struct|BreakTriangle _array_element)) (.B (Utilities|Struct|BreakTriangle _array_element))))
      (Utilities|Array|Add (LocalVariables|Getedges) (Utilities|Struct|MakeLine (.A (Utilities|Struct|BreakTriangle _array_element)) (.C (Utilities|Struct|BreakTriangle _array_element))))
      (Utilities|Array|Add (LocalVariables|Getedges) (Utilities|Struct|MakeLine (.B (Utilities|Struct|BreakTriangle _array_element)) (.C (Utilities|Struct|BreakTriangle _array_element))))
      (else
        (Utilities|Array|Add (LocalVariables|Getnew%20triangles%20) _array_element))))
  (Utilities|Array|Clear (LocalVariables|Getnew%20edges%202))
  (Utilities|Array|Clear (LocalVariables|GetNOT%20FUCKIN%20UNIQUE%20EDGES2))
  (for _array_element_2 (LocalVariables|Getedges) ; get unique edges
    (if (or (Utilities|Array|ContainsItem _new_edges_2 _array_element_2) (Utilities|Array|ContainsItem _new_edges_2 (Utilities|Struct|MakeLine (.B (Utilities|Struct|BreakLine _array_element_2)) (.A (Utilities|Struct|BreakLine _array_element_2)))))
      (Utilities|Array|Add (LocalVariables|GetNOT%20FUCKIN%20UNIQUE%20EDGES2) _array_element_2)
      (Utilities|Array|RemoveItem (LocalVariables|Getnew%20edges%202) (Utilities|Struct|MakeLine (.B (Utilities|Struct|BreakLine _array_element_2)) (.A (Utilities|Struct|BreakLine _array_element_2))))
      (Utilities|Array|RemoveItem (LocalVariables|Getnew%20edges%202) _array_element_2)
      (elif (not (or (Utilities|Array|ContainsItem (LocalVariables|GetNOT%20FUCKIN%20UNIQUE%20EDGES2) _array_element_2) (Utilities|Array|ContainsItem (LocalVariables|GetNOT%20FUCKIN%20UNIQUE%20EDGES2) (Utilities|Struct|MakeLine (.B (Utilities|Struct|BreakLine _array_element_2)) (.A (Utilities|Struct|BreakLine _array_element_2))))))
        (Utilities|Array|Add (LocalVariables|Getnew%20edges%202) _array_element_2))))
  (for _array_element_3 (LocalVariables|Getnew%20edges%202)
    (Utilities|Array|Add (LocalVariables|Getnew%20triangles%20) (Utilities|Struct|MakeTriangle (.A (Utilities|Struct|BreakLine _array_element_3)) (.B (Utilities|Struct|BreakLine _array_element_3)) (LocalVariables|GetVertex))))
  (return (LocalVariables|Getnew%20triangles%20)))

(fn IsinCircumcircle?
  (params (vertex :type Vector%202D%20Structure) (triangle :type Triangle%20Structure))
  (bind (_x _y) (Math|Vector2D|BreakVector2D (.a triangle)))
  (bind (_x_2 _y_2) (Math|Vector2D|BreakVector2D (.c triangle)))
  (bind (_x_3 _y_3) (Math|Vector2D|BreakVector2D (.b triangle)))
  (LocalVariables|SetVertex%20X (.x vertex))
  (LocalVariables|SetVertex%20Y (.y vertex))
  (LocalVariables|Setax _x)
  (LocalVariables|Setay _y)
  (LocalVariables|Setbx _x_3)
  (LocalVariables|Setby _y_3)
  (LocalVariables|Setcx _x_2)
  (LocalVariables|Setcy _y_2)
  (LocalVariables|SetD (+ (* (LocalVariables|Getax) (- (LocalVariables|Getby) (LocalVariables|Getcy))) (* (LocalVariables|Getbx) (- (LocalVariables|Getcy) (LocalVariables|Getay))) (* (LocalVariables|Getcx) (- (LocalVariables|Getay) (LocalVariables|Getby)))))
  (LocalVariables|Setux (/ (/ (+ (* (+ (Math|Float|Square (LocalVariables|Getax)) (Math|Float|Square (LocalVariables|Getay))) (- (LocalVariables|Getby) (LocalVariables|Getcy))) (* (+ (Math|Float|Square (LocalVariables|Getbx)) (Math|Float|Square (LocalVariables|Getby))) (- (LocalVariables|Getcy) (LocalVariables|Getay))) (* (+ (Math|Float|Square (LocalVariables|Getcx)) (Math|Float|Square (LocalVariables|Getcy))) (- (LocalVariables|Getay) (LocalVariables|Getby)))) (LocalVariables|GetD)) 2.0))
  (LocalVariables|Setuy (/ (/ (+ (* (+ (Math|Float|Square (LocalVariables|Getax)) (Math|Float|Square (LocalVariables|Getay))) (- (LocalVariables|Getcx) (LocalVariables|Getbx))) (* (+ (Math|Float|Square (LocalVariables|Getbx)) (Math|Float|Square (LocalVariables|Getby))) (- (LocalVariables|Getax) (LocalVariables|Getcx))) (* (+ (Math|Float|Square (LocalVariables|Getcx)) (Math|Float|Square (LocalVariables|Getcy))) (- (LocalVariables|Getbx) (LocalVariables|Getax)))) (LocalVariables|GetD)) 2.0))
  (bind _distance (CallFunction|Vector2dDistance (Math|Vector2D|MakeVector2D (LocalVariables|Getax) (LocalVariables|Getay)) (Math|Vector2D|MakeVector2D (LocalVariables|Getux) (LocalVariables|Getuy))))
  (return (<= (Math|Vector2D|Vector2DLength (Math|Vector2D|MakeVector2D (- (LocalVariables|Getux) (LocalVariables|GetVertex%20X)) (- (LocalVariables|Getuy) (LocalVariables|GetVertex%20Y)))) _distance)))

(fn Bowyer-WatsonAlgorithm
  (params (Points :type Array%20of%20Vector%202D%20Structures))
  (LocalVariables|SetPoints2 Points)
  ;[1 0.01813 0] todo: create better super triangle
  (bind _triangle (CallFunction|FindSuperTriangle (LocalVariables|GetPoints2)))
  (if (== (Math|Vector|DotProduct (Math|Vector|GetUnitDirection(Vector) (Math|Conversions|ToVector(Vector2D) (.A (Utilities|Struct|BreakTriangle _triangle))) (Math|Conversions|ToVector(Vector2D) (.B (Utilities|Struct|BreakTriangle _triangle)))) (Math|Vector|GetUnitDirection(Vector) (Math|Conversions|ToVector(Vector2D) (.A (Utilities|Struct|BreakTriangle _triangle))) (Math|Conversions|ToVector(Vector2D) (.C (Utilities|Struct|BreakTriangle _triangle))))) 0.0)
    (return 0 true)
    (else
      (bind _output_get (LocalVariables|SetSuper%20triangle2 _triangle))
      (Rendering|Debug|DrawDebugLine (Math|Conversions|ToVector(Vector2D) (.A (Utilities|Struct|BreakTriangle _output_get))) (Math|Conversions|ToVector(Vector2D) (.B (Utilities|Struct|BreakTriangle _output_get))) "(R=0.000000,G=1.000000,B=0.277538,A=1.000000)" 5e+02 0.0)
      (Rendering|Debug|DrawDebugLine (Math|Conversions|ToVector(Vector2D) (.B (Utilities|Struct|BreakTriangle _output_get))) (Math|Conversions|ToVector(Vector2D) (.C (Utilities|Struct|BreakTriangle _output_get))) "(R=0.000000,G=1.000000,B=0.168679,A=1.000000)" 5e+02 0.0)
      (Rendering|Debug|DrawDebugLine (Math|Conversions|ToVector(Vector2D) (.A (Utilities|Struct|BreakTriangle _output_get))) (Math|Conversions|ToVector(Vector2D) (.C (Utilities|Struct|BreakTriangle _output_get))) "(R=0.000000,G=1.000000,B=0.256586,A=1.000000)" 5e+02 0.0)
      (LocalVariables|SetTriangles2 (Utilities|Array|MakeArray _output_get))
      (for _array_element (LocalVariables|GetPoints2)
        (bind _triangles_out (CallFunction|AddVertex _array_element (LocalVariables|GetTriangles2)))
        (LocalVariables|SetTriangles2 _triangles_out))
      (for _array_element_2 (LocalVariables|GetTriangles2)
        (if (not (Math|Boolean|ORBoolean (Math|Vector|Equal(Vector) (.A (Utilities|Struct|BreakTriangle _array_element_2)) (.A (Utilities|Struct|BreakTriangle (LocalVariables|GetSuper%20triangle2))) 0.0) (Math|Vector|Equal(Vector) (.A (Utilities|Struct|BreakTriangle _array_element_2)) (.B (Utilities|Struct|BreakTriangle (LocalVariables|GetSuper%20triangle2))) 0.0) (Math|Vector|Equal(Vector) (.A (Utilities|Struct|BreakTriangle _array_element_2)) (.C (Utilities|Struct|BreakTriangle (LocalVariables|GetSuper%20triangle2))) 0.0) (Math|Vector|Equal(Vector) (.B (Utilities|Struct|BreakTriangle _array_element_2)) (.A (Utilities|Struct|BreakTriangle (LocalVariables|GetSuper%20triangle2))) 0.0) (Math|Vector|Equal(Vector) (.B (Utilities|Struct|BreakTriangle _array_element_2)) (.B (Utilities|Struct|BreakTriangle (LocalVariables|GetSuper%20triangle2))) 0.0) (Math|Vector|Equal(Vector) (.B (Utilities|Struct|BreakTriangle _array_element_2)) (.C (Utilities|Struct|BreakTriangle (LocalVariables|GetSuper%20triangle2))) 0.0) (Math|Vector|Equal(Vector) (.C (Utilities|Struct|BreakTriangle _array_element_2)) (.A (Utilities|Struct|BreakTriangle (LocalVariables|GetSuper%20triangle2))) 0.0) (Math|Vector|Equal(Vector) (.C (Utilities|Struct|BreakTriangle _array_element_2)) (.B (Utilities|Struct|BreakTriangle (LocalVariables|GetSuper%20triangle2))) 0.0) (Math|Vector|Equal(Vector) (.C (Utilities|Struct|BreakTriangle _array_element_2)) (.C (Utilities|Struct|BreakTriangle (LocalVariables|GetSuper%20triangle2))) 0.0)))
          (Utilities|Array|Add (LocalVariables|GetNew%20triangles%202) _array_element_2)))
      ;[1 1 1] Check that none of the points are on the super triangle
      (return (LocalVariables|GetNew%20triangles%202) false))))

(fn StraightLine-Algorithm
  (bind _roomcenter_vectors (Variables|Default|GetRoomCenter_Vectors))
  (bind _roomcenter_vectors_2 (Variables|Default|GetRoomCenter_Vectors))
  (bind _roomcenter_vectors_3 (Variables|Default|GetRoomCenter_Vectors))
  (bind _returnvalue (Utilities|Array|LastIndex _roomcenter_vectors))
  (bind _output (Utilities|Array|Get(acopy) _roomcenter_vectors))
  (LocalVariables|SetLineVector (Math|Vector|GetUnitDirection(Vector) (Math|Conversions|ToVector(Vector2D) (Utilities|Array|Get(acopy) _roomcenter_vectors_2)) (Math|Conversions|ToVector(Vector2D) (Utilities|Array|Get(acopy) _roomcenter_vectors_2 1))))
  ;[1 1 1] Sorts points onto a straightline linearly
  (for _index (range 0 _returnvalue)
    (bind _output_get (LocalVariables|SetMinIndex _index))
    (for _index_2 (range (+ _output_get 1) _returnvalue)
      (if (< (Math|Vector2D|DotProduct(2D) (- (Utilities|Array|Get(acopy) _roomcenter_vectors _index_2) _output) (Math|Conversions|ToVector2D(Vector) (LocalVariables|GetLineVector))) (Math|Vector2D|DotProduct(2D) (- (Utilities|Array|Get(acopy) _roomcenter_vectors (LocalVariables|GetMinIndex)) _output) (Math|Conversions|ToVector2D(Vector) (LocalVariables|GetLineVector))))
        (LocalVariables|SetMinIndex _index_2)))
    (if (!= _index (LocalVariables|GetMinIndex))
      (LocalVariables|SetSwapA (Utilities|Array|Get(acopy) _roomcenter_vectors _index))
      (LocalVariables|SetSwapB (Utilities|Array|Get(acopy) _roomcenter_vectors (LocalVariables|GetMinIndex)))
      (Utilities|Array|SetArrayElem _roomcenter_vectors (LocalVariables|GetMinIndex) (LocalVariables|GetSwapA))
      (Utilities|Array|SetArrayElem _roomcenter_vectors _index (LocalVariables|GetSwapB))))
  (for (_array_element _array_index) _roomcenter_vectors_3
    (if (!= _array_index (Utilities|Array|LastIndex _roomcenter_vectors_3))
      (bind _distance (CallFunction|Vector2dDistance _array_element (Utilities|Array|Get(acopy) _roomcenter_vectors_3 (+ _array_index 1))))
      (Utilities|Array|Add (LocalVariables|GetEdges) (Utilities|Struct|MakeEdge+Distance _array_element (Utilities|Array|Get(acopy) _roomcenter_vectors_3 (+ _array_index 1)) _distance))))
  (return (LocalVariables|GetEdges)))