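; Dungeon path algorithm that turns Delaunay triangles into a minimum spanning tree with extra loops, then passes the edges to DungeonMaster.
; Unique triangle edges are sorted, converted to point indices and run through Kruskal's algorithm using a union-find with union by rank.
; Single-connection nodes then gain a short unused Delaunay edge, preferring other dead ends before any node.
; Debug lines, spheres and text labels visualise the result.
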(event Custom|Create_MinSpanTree
  (params (Triangles :type Array%20of%20Triangle%20Structures))
  (bind _nodeconnections (Variables|Default|GetNodeConnections))
  (bind _nodeconnections_2 (Variables|Default|GetNodeConnections))
  ;[1 1 1] Converts Triangles to Individual *Unique* Lines
  (CallFunction|CreateEdges Triangles)
  (CallFunction|SortEdgesArray (Variables|Default|GetEdges))
  ;[1 1 1] Converts Edges to Indexed points Rather than Vector Points
  (CallFunction|CreateMSTEdges (Variables|Default|GetEdges))
  ;[1 1 1] Kruskal's
  (bind _cost1 (CallFunction|Kruskal's))
  ;[1 1 1] Converts Final MST back to vectors rather than indexed points
  (for _array_element (Variables|Default|GetMST_Edges)
    (Utilities|Array|Add (Variables|Default|GetFinal_Edges) (Utilities|Struct|MakeEdge+Distance (Utilities|Array|Get(acopy) (Variables|Default|GetUnique_VectorMap) (.VectorA_Index (Utilities|Struct|BreakMST_Edge _array_element))) (Utilities|Array|Get(acopy) (Variables|Default|GetUnique_VectorMap) (.VectorB_Index (Utilities|Struct|BreakMST_Edge _array_element))) (.Weight (Utilities|Struct|BreakMST_Edge _array_element)))))
  (for _array_element_2 (Variables|Default|GetFinal_Edges)
    (Rendering|Debug|DrawDebugLine (Math|Conversions|ToVector(Vector2D) (.A (Utilities|Struct|BreakEdge+Distance _array_element_2))) (Math|Conversions|ToVector(Vector2D) (.B (Utilities|Struct|BreakEdge+Distance _array_element_2))) "(R=0.000000,G=1.000000,B=0.095112,A=1.000000)" 5e+02 15.0))
  ;[1 1 1] Converts Edges Array into Unused Delaunay Edges
  (for _array_element_3 (Variables|Default|GetFinal_Edges)
    (Utilities|Array|RemoveItem (Variables|Default|GetEdges) _array_element_3))
  ;[1 1 1] Maps Each MST Node to amount of connections it has (which we need to solve which nodes should get extra loops
  (for _array_element_4 (Variables|Default|GetFinal_Edges)
    (if (.ReturnValue (Utilities|Map|Find (Variables|Default|GetNodeConnections) (.A (Utilities|Struct|BreakEdge+Distance _array_element_4))))
      (Utilities|Map|Add (Variables|Default|GetNodeConnections) (.A (Utilities|Struct|BreakEdge+Distance _array_element_4)) (+ (.Value (Utilities|Map|Find (Variables|Default|GetNodeConnections) (.A (Utilities|Struct|BreakEdge+Distance _array_element_4)))) 1))
      (else
        (Utilities|Map|Add (Variables|Default|GetNodeConnections) (.A (Utilities|Struct|BreakEdge+Distance _array_element_4)) 1)))
    (if (.ReturnValue (Utilities|Map|Find (Variables|Default|GetNodeConnections) (.B (Utilities|Struct|BreakEdge+Distance _array_element_4))))
      (Utilities|Map|Add (Variables|Default|GetNodeConnections) (.B (Utilities|Struct|BreakEdge+Distance _array_element_4)) (+ (.Value (Utilities|Map|Find (Variables|Default|GetNodeConnections) (.B (Utilities|Struct|BreakEdge+Distance _array_element_4)))) 1))
      (else
        (Utilities|Map|Add (Variables|Default|GetNodeConnections) (.B (Utilities|Struct|BreakEdge+Distance _array_element_4)) 1))))
  (bind _keys (Utilities|Map|Keys _nodeconnections))
  (for (_array_element_5 _array_index) _keys
    (if (== (.Value (Utilities|Map|Find _nodeconnections _array_element_5)) 1)
      (Rendering|Debug|DrawDebugSphere (Math|Conversions|ToVector(Vector2D) _array_element_5) 5e+01 12 "(R=1.000000,G=0.548421,B=0.000000,A=1.000000)" 5e+02 2.0))
    (bind _returnvalue (AddComponent|AddTextRenderComponent false (Math|Transform|MakeTransform (Math|Vector|MakeVector (.X (Math|Vector2D|BreakVector2D _array_element_5)) (.Y (Math|Vector2D|BreakVector2D _array_element_5)) 5e+01) "0, 0, 0" "5.000000,5.000000,5.000000")))
    (Rendering|Components|TextRender|SetText _returnvalue (Utilities|Text|ToText(String) (Utilities|String|ToString(Integer) _array_index)))
    (Rendering|Components|TextRender|SetTextRenderColor _returnvalue (Math|Color|MakeColor 0 0 255 255)))
  ;[0.2708 1 0.9901] Add Extra Connections
  (bind _output_get (CallFunction|FindExtraLoops))
  (for _array_element_6 (Variables|Default|GetExtra_LoopEdges)
    (Rendering|Debug|DrawDebugLine (Math|Conversions|ToVector(Vector2D) (.A (Utilities|Struct|BreakEdge+Distance _array_element_6))) (Math|Conversions|ToVector(Vector2D) (.B (Utilities|Struct|BreakEdge+Distance _array_element_6))) "(R=0.320038,G=1.000000,B=0.940233,A=1.000000)" 5e+02 11.0))
  (bind _values (Utilities|Map|Values _nodeconnections_2))
  (for (_array_element_7 _array_index_2) _values
    (if (== _array_element_7 1)
      (bind _keys_2 (Utilities|Map|Keys _nodeconnections_2))
      (Rendering|Debug|DrawDebugSphere (Math|Conversions|ToVector(Vector2D) (Utilities|Array|Get(acopy) _keys_2 _array_element_7)) 5e+01 12 "(R=0.001347,G=0.000000,B=1.000000,A=1.000000)" 5e+02 2.0)))
  (for _array_element_8 (Variables|Default|GetExtra_LoopEdges)
    (Utilities|Array|Add (Variables|Default|GetFinal_Edges) _array_element_8))
  (Default|PathAlgorithmFinished (Variables|Default|GetDungeonMaster) (Variables|Default|GetFinal_Edges)))

(event EventBeginPlay)

(fn ConstructionScript)

(fn CreateEdges
  (params (Triangles :type Array%20of%20Triangle%20Structures))
  (for _array_element Triangles
    (LocalVariables|SetLineA (.A (Utilities|Struct|BreakTriangle _array_element)))
    (LocalVariables|SetLineB (.B (Utilities|Struct|BreakTriangle _array_element)))
    (LocalVariables|SetLineC (.C (Utilities|Struct|BreakTriangle _array_element)))
    (bind (_returnedges _unique_) (CallFunction|CheckifUniqueEdge (LocalVariables|GetUniqueEdges) (Utilities|Struct|MakeLine (LocalVariables|GetLineA) (LocalVariables|GetLineB))))
    (LocalVariables|SetUniqueEdges _returnedges)
    (if _unique_
      (bind _distance (CallFunction|Vector2dDistance (LocalVariables|GetLineA) (LocalVariables|GetLineB)))
      (Utilities|Array|Add (Variables|Default|GetEdges) (Utilities|Struct|MakeEdge+Distance (LocalVariables|GetLineA) (LocalVariables|GetLineB) _distance)))
    (bind (_returnedges_2 _unique__2) (CallFunction|CheckifUniqueEdge (LocalVariables|GetUniqueEdges) (Utilities|Struct|MakeLine (LocalVariables|GetLineA) (LocalVariables|GetLineC))))
    (LocalVariables|SetUniqueEdges _returnedges_2)
    (if _unique__2
      (bind _distance_2 (CallFunction|Vector2dDistance (LocalVariables|GetLineA) (LocalVariables|GetLineC)))
      (Utilities|Array|Add (Variables|Default|GetEdges) (Utilities|Struct|MakeEdge+Distance (LocalVariables|GetLineA) (LocalVariables|GetLineC) _distance_2)))
    (bind (_returnedges_3 _unique__3) (CallFunction|CheckifUniqueEdge (LocalVariables|GetUniqueEdges) (Utilities|Struct|MakeLine (LocalVariables|GetLineB) (LocalVariables|GetLineC))))
    (LocalVariables|SetUniqueEdges _returnedges_3)
    (if _unique__3
      (bind _distance_3 (CallFunction|Vector2dDistance (LocalVariables|GetLineB) (LocalVariables|GetLineC)))
      (Utilities|Array|Add (Variables|Default|GetEdges) (Utilities|Struct|MakeEdge+Distance (LocalVariables|GetLineB) (LocalVariables|GetLineC) _distance_3))))
  (return))

(fn DSUCreate
  (params (LastIndex :type Integer))
  (for _index (range 0 LastIndex)
    (Utilities|Array|Add (Variables|Default|GetDSU) (Utilities|Struct|MakeDSU _index 1)))
  (return))

(fn DSUFind
  (params (Node_Index :type Integer))
  (bind _dsu (Variables|Default|GetDSU))
  (bind _output (Utilities|Array|Get(acopy) _dsu Node_Index))
  (bind _parent (Utilities|Struct|BreakDSU _output))
  (if (== _parent Node_Index)
    (return _parent)
    (else
      (bind _parent_2 (CallFunction|DSUFind _parent))
      (return _parent_2))))

(fn CreateMSTEdges
  (params (Edges :type Array%20of%20Edge+Distance%20Structures))
  (bind _unique_vectormap (Variables|Default|GetUnique_VectorMap))
  (for _index (range 0 (Utilities|Array|LastIndex Edges))
    (Utilities|Array|AddUnique (Variables|Default|GetUnique_VectorMap) (.A (Utilities|Struct|BreakEdge+Distance (Utilities|Array|Get(acopy) Edges _index))))
    (Utilities|Array|AddUnique (Variables|Default|GetUnique_VectorMap) (.B (Utilities|Struct|BreakEdge+Distance (Utilities|Array|Get(acopy) Edges _index)))))
  (for _array_element Edges
    (Utilities|Array|Add (Variables|Default|GetIndex_Edges) (Utilities|Struct|MakeMST_Edge (Utilities|Array|FindItem _unique_vectormap (.A (Utilities|Struct|BreakEdge+Distance _array_element))) (Utilities|Array|FindItem _unique_vectormap (.B (Utilities|Struct|BreakEdge+Distance _array_element))) (.Distance (Utilities|Struct|BreakEdge+Distance _array_element)))))
  (return))

(fn Kruskal's
  (bind _output_get (LocalVariables|SetUniqueNode_Length (Utilities|Array|Length (Variables|Default|GetUnique_VectorMap))))
  (CallFunction|DSUCreate (- _output_get 1))
  (bind _array_element (Utilities|Array|ForEachLoopwithBreak (Variables|Default|GetIndex_Edges) :!label _label)
    (:LoopBody
      (bind _parent (CallFunction|DSUFind (.VectorA_Index (Utilities|Struct|BreakMST_Edge _array_element))))
      (bind _parent_2 (CallFunction|DSUFind (.VectorB_Index (Utilities|Struct|BreakMST_Edge _array_element))))
      (if (!= _parent _parent_2)
        (CallFunction|DSUUnion (.VectorA_Index (Utilities|Struct|BreakMST_Edge _array_element)) (.VectorB_Index (Utilities|Struct|BreakMST_Edge _array_element)))
        (Utilities|Array|Add (Variables|Default|GetMST_Edges) _array_element)
        (LocalVariables|SetCost (+ (LocalVariables|GetCost) (.Weight (Utilities|Struct|BreakMST_Edge _array_element))))
        (bind _result (Math|Integer|IncrementInt (LocalVariables|GetCount))
          (:%20%20
            (if (== _result (- (LocalVariables|GetUniqueNode_Length) 1))
              (goto _label Break))))))
    (:Completed
      (return (LocalVariables|GetCost)))))

(fn DSUUnion
  (params (index_x :type Integer) (index_y :type Integer))
  (bind _dsu (Variables|Default|GetDSU))
  (bind _dsu_2 (Variables|Default|GetDSU))
  (bind _dsu_3 (Variables|Default|GetDSU))
  (bind _dsu_4 (Variables|Default|GetDSU))
  (bind _dsu_5 (Variables|Default|GetDSU))
  (bind _dsu_6 (Variables|Default|GetDSU))
  (bind _parent (CallFunction|DSUFind index_x))
  (LocalVariables|SetS1 _parent)
  (bind _parent_2 (CallFunction|DSUFind index_y))
  (LocalVariables|SetS2 _parent_2)
  (if (!= (LocalVariables|GetS1) (LocalVariables|GetS2))
    (if (< (.Rank (Utilities|Struct|BreakDSU (Utilities|Array|Get(acopy) _dsu_3 (LocalVariables|GetS1)))) (.Rank (Utilities|Struct|BreakDSU (Utilities|Array|Get(acopy) _dsu_3 (LocalVariables|GetS2)))))
      (Utilities|Array|SetArrayElem _dsu_6 (LocalVariables|GetS1) (Utilities|Struct|MakeDSU (LocalVariables|GetS2) (.Rank (Utilities|Struct|BreakDSU (Utilities|Array|Get(acopy) _dsu_6 (LocalVariables|GetS1))))))
      (elif (> (.Rank (Utilities|Struct|BreakDSU (Utilities|Array|Get(acopy) _dsu_2 (LocalVariables|GetS1)))) (.Rank (Utilities|Struct|BreakDSU (Utilities|Array|Get(acopy) _dsu_2 (LocalVariables|GetS2)))))
        (Utilities|Array|SetArrayElem _dsu_5 (LocalVariables|GetS2) (Utilities|Struct|MakeDSU (LocalVariables|GetS1) (.Rank (Utilities|Struct|BreakDSU (Utilities|Array|Get(acopy) _dsu_5 (LocalVariables|GetS2))))))
        (else
          (Utilities|Array|SetArrayElem _dsu (LocalVariables|GetS2) (Utilities|Struct|MakeDSU (LocalVariables|GetS1) (.Rank (Utilities|Struct|BreakDSU (Utilities|Array|Get(acopy) _dsu (LocalVariables|GetS2))))))
          (Utilities|Array|SetArrayElem _dsu_4 (LocalVariables|GetS1) (Utilities|Struct|MakeDSU (.Parent (Utilities|Struct|BreakDSU (Utilities|Array|Get(acopy) _dsu_4 (LocalVariables|GetS1)))) (+ (.Rank (Utilities|Struct|BreakDSU (Utilities|Array|Get(acopy) _dsu_4 (LocalVariables|GetS1)))) 1))))))))

(fn FindExtraLoops
  (bind _nodeconnections (Variables|Default|GetNodeConnections))
  (bind _nodeconnections_2 (Variables|Default|GetNodeConnections))
  (bind _nodeconnections_3 (Variables|Default|GetNodeConnections))
  (bind _nodeconnections_4 (Variables|Default|GetNodeConnections))
  (bind _values (Utilities|Map|Values (Variables|Default|GetNodeConnections)))
  (bind _output_get (LocalVariables|SetValues _values))
  (for (_array_element _array_index) _output_get
    (if (== _array_element 1)
      (bind _keys (Utilities|Map|Keys (Variables|Default|GetNodeConnections)))
      (LocalVariables|SetVectorA_ArrayIndex _array_index)
      (LocalVariables|SetVectorA (Utilities|Array|Get(acopy) _keys _array_index))
      (LocalVariables|SetMinimumDistance 1e+07)
      (LocalVariables|SetFoundSingleNodeLoop false)
      (bind (_array_element_2 _array_index_2) (Utilities|Array|ForEachLoopwithBreak _output_get)
        (:LoopBody
          (if (== _array_element_2 1)
            (bind _keys_2 (Utilities|Map|Keys (Variables|Default|GetNodeConnections)))
            (if (Math|Vector|NotEqual(Vector) (LocalVariables|GetVectorA) (Utilities|Array|Get(acopy) _keys_2 _array_index_2) 0.0)
              (bind _distance (CallFunction|Vector2dDistance (LocalVariables|GetVectorA) (Utilities|Array|Get(acopy) _keys_2 _array_index_2)))
              (if (or (Utilities|Array|ContainsItem (Variables|Default|GetEdges) (Utilities|Struct|MakeEdge+Distance (LocalVariables|GetVectorA) (Utilities|Array|Get(acopy) _keys_2 _array_index_2) _distance)) (Utilities|Array|ContainsItem (Variables|Default|GetEdges) (Utilities|Struct|MakeEdge+Distance (Utilities|Array|Get(acopy) _keys_2 _array_index_2) (LocalVariables|GetVectorA) 0.0)))
                (LocalVariables|SetMinimumDistance (Math|Float|Min(Float) _distance (LocalVariables|GetMinimumDistance)))
                (if (== (Math|Float|Min(Float) _distance (LocalVariables|GetMinimumDistance)) _distance)
                  (LocalVariables|SetPotentialConnection (Utilities|Struct|MakeEdge+Distance (LocalVariables|GetVectorA) (Utilities|Array|Get(acopy) _keys_2 _array_index_2) _distance))
                  (LocalVariables|SetFoundSingleNodeLoop true)
                  (LocalVariables|SetVectorB_ArrayIndex _array_index_2)
                  (LocalVariables|SetPotentialVectorB (Utilities|Array|Get(acopy) _keys_2 _array_index_2)))))))
        (:Completed
          (if (LocalVariables|GetFoundSingleNodeLoop)
            (Utilities|Array|Add (Variables|Default|GetExtra_LoopEdges) (LocalVariables|GetPotentialConnection))
            (bind _output_get_2 (LocalVariables|SetNewLocalVar_0 (+ (.Value (Utilities|Map|Find _nodeconnections_2 (LocalVariables|GetVectorA))) 1)))
            (bind _returnvalue (Utilities|Map|Add _nodeconnections_2 (LocalVariables|GetVectorA) _output_get_2))
            (if _returnvalue
              (Development|PrintString "Added Array" true true "(R=0.000000,G=0.660000,B=1.000000,A=1.000000)" 1.2e+02))
            (Utilities|Array|SetArrayElem _output_get (LocalVariables|GetVectorA_ArrayIndex) _output_get_2)
            (bind _output_get_3 (LocalVariables|SetNewLocalVar_1 (+ (.Value (Utilities|Map|Find _nodeconnections_3 (LocalVariables|GetPotentialVectorB))) 1)))
            (bind _returnvalue_2 (Utilities|Map|Add _nodeconnections_3 (LocalVariables|GetPotentialVectorB) _output_get_3))
            (if _returnvalue_2
              (Development|PrintString "Added Array" true true "(R=0.000000,G=0.660000,B=1.000000,A=1.000000)" 1.2e+02))
            (Utilities|Array|SetArrayElem _output_get (LocalVariables|GetVectorB_ArrayIndex) _output_get_3)
            (else
              (bind _array_index_3 (Utilities|Array|ForEachLoopwithBreak _output_get)
                (:LoopBody
                  (bind _keys_3 (Utilities|Map|Keys (Variables|Default|GetNodeConnections)))
                  (if (Math|Vector|NotEqual(Vector) (LocalVariables|GetVectorA) (Utilities|Array|Get(acopy) _keys_3 _array_index_3) 0.0)
                    (bind _distance_2 (CallFunction|Vector2dDistance (LocalVariables|GetVectorA) (Utilities|Array|Get(acopy) _keys_3 _array_index_3)))
                    (if (or (Utilities|Array|ContainsItem (Variables|Default|GetEdges) (Utilities|Struct|MakeEdge+Distance (LocalVariables|GetVectorA) (Utilities|Array|Get(acopy) _keys_3 _array_index_3) _distance_2)) (Utilities|Array|ContainsItem (Variables|Default|GetEdges) (Utilities|Struct|MakeEdge+Distance (Utilities|Array|Get(acopy) _keys_3 _array_index_3) (LocalVariables|GetVectorA) _distance_2)))
                      (LocalVariables|SetMinimumDistance (Math|Float|Min(Float) _distance_2 (LocalVariables|GetMinimumDistance)))
                      (if (== _distance_2 (Math|Float|Min(Float) _distance_2 (LocalVariables|GetMinimumDistance)))
                        (LocalVariables|SetPotentialConnection (Utilities|Struct|MakeEdge+Distance (LocalVariables|GetVectorA) (Utilities|Array|Get(acopy) _keys_3 _array_index_3) _distance_2))
                        (LocalVariables|SetVectorB_ArrayIndex _array_index_3)
                        (LocalVariables|SetPotentialVectorB (Utilities|Array|Get(acopy) _keys_3 _array_index_3))
                        (LocalVariables|SetFoundSingleNodeLoop true)))))
                (:Completed
                  (if (LocalVariables|GetFoundSingleNodeLoop)
                    (Utilities|Array|Add (Variables|Default|GetExtra_LoopEdges) (LocalVariables|GetPotentialConnection))
                    (bind _output_get_4 (LocalVariables|SetNewLocalVar_0 (+ (.Value (Utilities|Map|Find _nodeconnections (LocalVariables|GetVectorA))) 1)))
                    (bind _returnvalue_3 (Utilities|Map|Add _nodeconnections (LocalVariables|GetVectorA) _output_get_4))
                    (if _returnvalue_3
                      (Development|PrintString "Added Array" true true "(R=0.000000,G=0.660000,B=1.000000,A=1.000000)" 1.2e+02))
                    (Utilities|Array|SetArrayElem _output_get (LocalVariables|GetVectorA_ArrayIndex) _output_get_4)
                    (bind _output_get_5 (LocalVariables|SetNewLocalVar_1 (+ (.Value (Utilities|Map|Find _nodeconnections_4 (LocalVariables|GetPotentialVectorB))) 1)))
                    (bind _returnvalue_4 (Utilities|Map|Add _nodeconnections_4 (LocalVariables|GetPotentialVectorB) _output_get_5))
                    (if _returnvalue_4
                      (Development|PrintString (Utilities|String|Append "added array at vector: " (Utilities|String|ToString(Vector2d) (LocalVariables|GetPotentialVectorB))) true true "(R=0.000000,G=0.660000,B=1.000000,A=1.000000)" 1.2e+02))
                    (Utilities|Array|SetArrayElem _output_get (LocalVariables|GetVectorB_ArrayIndex) _output_get_5)
                    (else
                      (Development|PrintString (Utilities|String|Append "Found no optoins! @ point: " (Utilities|String|ToString(Integer) (LocalVariables|GetVectorA_ArrayIndex)) "Vector: " (Utilities|String|ToString(Vector2d) (LocalVariables|GetVectorA))) true true "(R=1.000000,G=0.044531,B=0.000000,A=1.000000)" 1.2e+02)))))))))))
  (return _output_get))