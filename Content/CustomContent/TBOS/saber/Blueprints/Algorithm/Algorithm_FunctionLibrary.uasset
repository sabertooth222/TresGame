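; Blueprint function library of geometry and edge-list helpers for algorithm code.
; Vector2dDistance computes the straight-line distance between two 2D points.
; CheckIfUniqueEdge treats edges as undirected, appending a candidate only if neither it nor its reverse exists, and returns the list with a uniqueness flag.
; SortEdgesArray orders edges by ascending Distance with a swap-based selection sort, alongside unreachable leftovers of a map-based attempt.
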(fn Vector2dDistance
  (params (VectorA :type Vector%202D%20Structure) (VectorB :type Vector%202D%20Structure))
  (bind _returnvalue (- VectorA VectorB))
  (bind (_x _y) (Math|Vector2D|BreakVector2D _returnvalue))
  (return (Math|Float|Sqrt (+ (Math|Float|Square (Math|Float|Absolute(Float) _x)) (Math|Float|Square (Math|Float|Absolute(Float) _y))))))

(fn CheckifUniqueEdge
  (params (edges :type Array%20of%20Line%20Structures) (PotentialEdge :type Line%20Structure))
  (bind (_a _b) (Utilities|Struct|BreakLine PotentialEdge))
  (LocalVariables|Setlocal_edges edges)
  (if (or (Utilities|Array|ContainsItem (LocalVariables|Getlocal_edges) PotentialEdge) (Utilities|Array|ContainsItem (LocalVariables|Getlocal_edges) (Utilities|Struct|MakeLine _b _a)))
    (return (LocalVariables|Getlocal_edges) false)
    (else
      (Utilities|Array|Add (LocalVariables|Getlocal_edges) PotentialEdge)
      (return (LocalVariables|Getlocal_edges) true))))

(fn SortEdgesArray
  (params (Edges :type Array%20of%20Edge+Distance%20Structures))
  (bind _returnvalue (Utilities|Array|LastIndex Edges))
  (for _index (range 0 _returnvalue)
    (bind _output_get (LocalVariables|SetMinIndex _index))
    (for _index_2 (range (+ _output_get 1) _returnvalue)
      (if (< (.Distance (Utilities|Struct|BreakEdge+Distance (Utilities|Array|Get(acopy) Edges _index_2))) (.Distance (Utilities|Struct|BreakEdge+Distance (Utilities|Array|Get(acopy) Edges (LocalVariables|GetMinIndex)))))
        (LocalVariables|SetMinIndex _index_2)))
    (if (!= _index (LocalVariables|GetMinIndex))
      (LocalVariables|SetSwapA (Utilities|Array|Get(acopy) Edges _index))
      (LocalVariables|SetSwapB (Utilities|Array|Get(acopy) Edges (LocalVariables|GetMinIndex)))
      (Utilities|Array|SetArrayElem Edges (LocalVariables|GetMinIndex) (LocalVariables|GetSwapA))
      (Utilities|Array|SetArrayElem Edges _index (LocalVariables|GetSwapB))))
  (return))