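; Blueprint function library of shared helpers for the TBOS mod, built on the Tres player and item APIs.
; Seeded random helpers pick integers from weighted maps, including tables that double weight to favor higher numbers.
; Enemy selection redraws data table rows until role, size and difficulty match, without retry limit and ignoring the WorldCodes and SeaCompatible inputs.
; Other helpers fetch the game instance, strip Sora's items and toggle player abilities and restrictions.
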(fn RandomWeightedIntStream
  (params (IntTable :type Map%20of%20Integers%20to%20Float%20%28single-precision%29s) (Seed :type Random%20Stream%20Structure%20%28by%20ref%29))
  (bind _output_get (LocalVariables|SetTable IntTable))
  (bind _values (Utilities|Map|Values _output_get))
  (for _array_element _values
    (LocalVariables|SetRunningTotal (+ _array_element (LocalVariables|GetRunningTotal))))
  (LocalVariables|SetRandomValue (Math|Random|RandomFloatinRangefromStream 0.0 (LocalVariables|GetRunningTotal) Seed))
  (bind _keys (Utilities|Map|Keys (LocalVariables|GetTable)))
  (for _array_element_2 _keys
    (if (<= (LocalVariables|GetRandomValue) (.Value (Utilities|Map|Find (LocalVariables|GetTable) _array_element_2)))
      (return _array_element_2)
      (else
        (LocalVariables|SetRandomValue (- (LocalVariables|GetRandomValue) (.Value (Utilities|Map|Find (LocalVariables|GetTable) _array_element_2))))))))

(fn RandomEnemyPawns
  (params (NumberOfEnemyClasses :type Integer) (Stream :type Random%20Stream%20Structure%20%28by%20ref%29) (MinDifficultyLevel :type Integer) (MaxDifficultyLvl :type Integer) (WorldCodes :type Array%20of%20Saber_WorldCode%20Enums :default "NewEnumerator0") (SeaCompatible :type Boolean) (MaxEnemySize :type EnemySize%20Enum :default "NewEnumerator7") (Role :type BossType%20Enum :default "NewEnumerator0"))
  (for _index (range 1 NumberOfEnemyClasses)
    (bind _outrownames (DataTable|GetDataTableRowNames "/Game/CustomContent/TBOS/saber/DataTable/EnemyPawnsDataTable.EnemyPawnsDataTable"))
    (while (not (LocalVariables|GetMatchFound))
      (bind _returnvalue (Utilities|GetDataTableRow "/Game/CustomContent/TBOS/saber/DataTable/EnemyPawnsDataTable.EnemyPawnsDataTable" (Utilities|Array|Get(acopy) _outrownames (Math|Random|RandomIntegerinRangefromStream 0 (Utilities|Array|LastIndex _outrownames) Stream)))
        (:then
          (bind _between_ (CallFunction|IntBetween (.EnemyDIfficulty_Level (Utilities|Struct|BreakEnemyDTStruct _returnvalue)) MinDifficultyLevel MaxDifficultyLvl))
          (if (Math|Boolean|ANDBoolean (Utilities|Enum|Equal(Enum) (.Type (Utilities|Struct|BreakEnemyDTStruct _returnvalue)) Role) (<= (.Size (Utilities|Struct|BreakEnemyDTStruct _returnvalue)) MaxEnemySize) _between_)
            (Utilities|Array|Add (LocalVariables|GetLocalEnemyPawnSet) (.Pawn_SoftRef (Utilities|Struct|BreakEnemyDTStruct _returnvalue)))
            (LocalVariables|SetMatchFound true)
            (Utilities|Array|Add (LocalVariables|GetLocalEnemyName) (.EnemyName (Utilities|Struct|BreakEnemyDTStruct _returnvalue)))
            (Development|PrintString 0 (Utilities|String|ToString(Name) (.EnemyName (Utilities|Struct|BreakEnemyDTStruct _returnvalue))) true true "(R=0.000000,G=0.660000,B=1.000000,A=1.000000)" 1e+01)))))
    (LocalVariables|SetMatchFound false))
  (return (LocalVariables|GetLocalEnemyPawnSet) (LocalVariables|GetLocalEnemyName)))

(fn CreateWeightedIntTable(FavorHigher)
  (params (LowestNumber :type Integer) (HighestNumber :type Integer))
  (for _index (range LowestNumber HighestNumber)
    (bind _output_get (LocalVariables|SetWeight (* (LocalVariables|GetWeight) 2.0)))
    (Utilities|Map|Add (LocalVariables|GetLocalWeightedIntTable) _index _output_get))
  (return (LocalVariables|GetLocalWeightedIntTable)))

(fn GetTBOSGameInstance
  (bind _astbos_game_instance (Utilities|Casting|CastToTBOS_GameInstance (Game|GetGameInstance))
    (:then
      (return _astbos_game_instance))
    (:CastFailed
      (Development|PrintString 0 "GameInstance_CastFail" true true "(R=1.000000,G=0.000000,B=0.043706,A=1.000000)" 15.0)
      (return 0))))

(fn IntBetween
  (params (Number%28toCheck%29 :type Integer) (MinEquals :type Integer) (MaxEquals :type Integer))
  (return (and (>= Number%28toCheck%29 MinEquals) (<= Number%28toCheck%29 MaxEquals))))

(fn RemoveAllItems
  (Class|TresGameBlueprintLibrary|TresReturnCharEquipItems 0 "TRES_CHR_UID_SORA")
  (bind _outrownames (DataTable|GetDataTableRowNames "/Game/Load/Tres/TresItemData.TresItemData"))
  (for _array_element _outrownames
    (bind _returnvalue (Utilities|GetDataTableRow "/Game/Load/Tres/TresItemData.TresItemData" _array_element)
      (:then
        (for _index (range 1 99)
          (Class|TresGameBlueprintLibrary|TresDropBackyardItemOne 0 (Utilities|Struct|BreakTresItemDataTable _returnvalue))))))
  (return))

(fn PlayerEnableEverything
  (params (InEnable :type Boolean))
  (bind _returnvalue (Class|TresGameBlueprintLibrary|GetLocalTresPlayerControllerBase))
  (bind _returnvalue_2 (Class|TresGameBlueprintLibrary|GetLocalTresPlayerControllerBase))
  (bind _returnvalue_3 (not InEnable))
  (Class|TresPlayerControllerBase|SetAbilityAttack _returnvalue_2 InEnable)
  (Class|TresPlayerControllerBase|SetAbilityAttractionFlow _returnvalue_2 InEnable)
  (Class|TresPlayerControllerBase|SetAbilityMagic _returnvalue_2 InEnable)
  (Class|TresPlayerControllerBase|SetAbilityShootFlow _returnvalue_2 InEnable)
  (Class|TresPlayerControllerBase|SetAbilityShortCutMenu _returnvalue_2 InEnable)
  (Class|TresPlayerControllerBase|SetAbilityStyleChange _returnvalue_2 InEnable)
  (Class|TresPlayerControllerBase|SetRestrictAntiForm _returnvalue _returnvalue_3)
  (Class|TresPlayerControllerBase|SetRestrictAttack _returnvalue _returnvalue_3)
  (Class|TresPlayerControllerBase|SetRestrictAttraction _returnvalue _returnvalue_3)
  (Class|TresPlayerControllerBase|SetRestrictDiveFall _returnvalue _returnvalue_3)
  (Class|TresPlayerControllerBase|SetRestrictFriend _returnvalue _returnvalue_3)
  (Class|TresPlayerControllerBase|SetRestrictGuard _returnvalue _returnvalue_3)
  (Class|TresPlayerControllerBase|SetRestrictItem _returnvalue _returnvalue_3)
  (Class|TresPlayerControllerBase|SetRestrictJump _returnvalue _returnvalue_3)
  (Class|TresPlayerControllerBase|SetRestrictLink _returnvalue _returnvalue_3)
  (Class|TresPlayerControllerBase|SetRestrictMagic _returnvalue _returnvalue_3)
  (Class|TresPlayerControllerBase|SetRestrictRun _returnvalue _returnvalue_3)
  (Class|TresPlayerControllerBase|SetRestrictShootLock _returnvalue _returnvalue_3)
  (Class|TresPlayerControllerBase|SetRestrictSituation _returnvalue _returnvalue_3)
  (Class|TresPlayerControllerBase|SetRestrictStyle _returnvalue _returnvalue_3))