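; PartyReactor is a helper actor that follows an NPC, shows its proximity barks and lets the player recruit it into the party.
; Each tick it snaps to the NPC's center socket, and its collision overlaps show or end barks.
; The reactor command opens a join prompt: joining adds the NPC, shows party length and destroys this actor.
; Rejecting plays a rejection bark, then a timer re-enables bark overlaps.
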(event OnComponentBeginOverlap(BarkCollision)
  (params (OverlappedComponent :type Primitive%20Component%20Object%20Reference) (OtherActor :type Actor%20Object%20Reference) (OtherComp :type Primitive%20Component%20Object%20Reference) (OtherBodyIndex :type Integer) (bFromSweep :type Boolean) (SweepResult :type Hit%20Result%20Structure%20%28by%20ref%29))
  (CallFunction|PartyOverlapBark (Variables|Default|GetBark_String) (Variables|Default|GetnpcPawn) (Variables|Default|GetEnableBarks) OtherActor))

(event OnComponentEndOverlap(BarkCollision)
  (params (OverlappedComponent :type Primitive%20Component%20Object%20Reference) (OtherActor :type Actor%20Object%20Reference) (OtherComp :type Primitive%20Component%20Object%20Reference) (OtherBodyIndex :type Integer))
  (bind _astres_player_pawn_base (Utilities|Casting|CastToTresPlayerPawnBase OtherActor))
  (CallFunction|PartyOverlapEndBark (Variables|Default|GetEnableBarks) (Variables|Default|GetnpcPawn) _astres_player_pawn_base))

(event OnReactorDoCommand(npcReactor)
  (params (CommandCauser :type Tres%20Char%20Pawn%20Base%20Object%20Reference) (CommandID :type ETresCommandKind%20Enum :default "TRES_CMD_KIND_NONE") (ReactorComponent :type Tres%20Reactor%20Component%20Object%20Reference))
  (CallFunction|PartyChatSetup (Variables|Default|GetEnableBarks) (Variables|Default|GetPostBarkTimer) (Variables|Default|GetnpcPawn) (Variables|Default|GetBarkCollision))
  (bind _partyreplaceindex (Utilities|PartyUIJoinAsk)
    (:JoinParty
      (Utilities|PartyJoinSetup (Variables|Default|GetnpcPawn) _partyreplaceindex (Variables|Default|GetBarkCollision))
      (bind _astbos_game_instance (CallFunction|GetTBOSGameInstance))
      (Class|TresGameBlueprintLibrary|TresUIOpenInformation (Utilities|Struct|MakeTresLocText (Utilities|String|Append "Party Length:" (Utilities|String|ToString(Integer) (Utilities|Array|Length (Variables|/Game/CustomContent/TBOS/saber/TBOS_GameInstance.TBOS_GameInstance_C|GetParty _astbos_game_instance))))) false 5.0)
      (Actor|DestroyActor))
    (:Reject
      (CallFunction|PartyRejectionBark (Variables|Default|GetnpcPawn))
      (bind _returnvalue (Utilities|Time|SetTimerbyEvent (delegate Custom|PostRejectBarkCD) 3.0))
      (Variables|Default|SetPostBarkTimer _returnvalue))))

(event Custom|PostRejectBarkCD
  (Class|TresGameBlueprintLibrary|TresUICloseCenterInformation)
  (Variables|/Script/Engine.PrimitiveComponent|SetbGenerateOverlapEvents (Variables|Default|GetBarkCollision) true))

(event EventBeginPlay
  (Utilities|PartyBeginPlay (Variables|Default|GetnpcPawn) (Variables|Default|GetnpcReactor)))

(event EventTick
  (params (DeltaSeconds :type Float%20%28single-precision%29))
  (bind _npcpawn (Variables|Default|GetnpcPawn))
  (Transformation|SetActorLocationAndRotation (Transformation|GetSocketLocation (Variables|/Script/TresGame.TresCharPawnBase|GetMyMesh _npcpawn) "center") (Transformation|GetActorRotation _npcpawn)))

(fn ConstructionScript)