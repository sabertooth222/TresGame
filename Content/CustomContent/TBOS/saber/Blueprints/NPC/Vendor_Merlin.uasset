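; Merlin vendor NPC that offers the player a Blizzard magic upgrade, built on a parent vendor Blueprint.
; The reactor command event calls the parent, then opens a choice dialog, or a refusal if TransactionUsed is set, and ends cinematic mode.
; Choosing Blizzard grants the BLIZZA_03 victory bonus, sets its game flag and calls PostTransactionEvent with a farewell bark.
; The construction script sets Merlin's name and soul-shard bark; this graph checks no shard cost.
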(event EventBeginPlay
  (|CallParentFunction))

(event EventBndEvtTresComNpcReactorK2NodeComponentBoundEvent3TresReactorDoCommandSignatureDelegateSignature
  (params (CommandCauser :type Tres%20Char%20Pawn%20Base%20Object%20Reference) (CommandID :type ETresCommandKind%20Enum :default "TRES_CMD_KIND_NONE") (ReactorComponent :type Tres%20Reactor%20Component%20Object%20Reference))
  (bind _returnvalue (Utilities|Name|MakeLiteralName "gameflow_GET_MAGIC_BLIZZA_03"))
  (|CallParentFunction CommandCauser CommandID ReactorComponent)
  (if (Variables|Default|GetTransactionUsed?)
    (bind _returnvalue_2 (Class|TresGameBlueprintLibrary|TresUIOpenChoice (Utilities|Struct|MakeTresLocText "I don't have any magic to teach right now. I'm exhausted; come back another time, will you?") (Utilities|Array|MakeArray (Utilities|Struct|MakeTresLocText "Sure Thing")) (Utilities|Struct|MakeTresUIWindowSetting "WINDOW_WAIT_TYPE_WAIT" "WINDOW_POSITION_TYPE_NONE" "(X=0.000000,Y=0.000000)") 0 false false "World"))
    (Class|TresGameBlueprintLibrary|TresUICloseWindow _returnvalue_2)
    (Class|TresGameBlueprintLibrary|TresEndCinematicMode false false)
    (else
      (bind (_outselected _returnvalue_3) (Class|TresGameBlueprintLibrary|TresUIOpenChoice (Utilities|Struct|MakeTresLocText "Would you like to upgrade your magic, my boy?") (Utilities|Array|MakeArray (Utilities|Struct|MakeTresLocText "Blizzard") (Utilities|Struct|MakeTresLocText "Nope")) (Utilities|Struct|MakeTresUIWindowSetting "WINDOW_WAIT_TYPE_WAIT" "WINDOW_POSITION_TYPE_NONE" "(X=0.000000,Y=0.000000)") 0 false false "World"))
      (Class|TresGameBlueprintLibrary|TresUICloseWindow _returnvalue_3)
      (Class|TresGameBlueprintLibrary|TresEndCinematicMode false false)
      (if (== _outselected 0)
        (Class|TresGameBlueprintLibrary|TresGetVictoryBonus _returnvalue true)
        (Class|TresGameBlueprintLibrary|SetGameFlagBoolean _returnvalue true)
        (CallFunction|PostTransactionEvent "Same place same time tomorrow? Oh...right...that's very unlikely." 5.0)))))

(fn ConstructionScript
  (|CallParentFunction)
  (Variables|Default|SetBark_String "Oh where could I have left those darn soul shards? Sora, if you come across any soul shards, bring them to me. I can teach you some magic!")
  (Variables|Default|SetNPCName "Merlin"))