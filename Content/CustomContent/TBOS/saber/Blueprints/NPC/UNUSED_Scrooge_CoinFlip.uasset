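; An unused Scrooge NPC Blueprint for a munny coin-flip gamble, left unfinished.
; Interacting through the reactor command opens a bet menu, or a refusal line and cinematic-mode exit if the transaction is already used.
; The fixed bets only store the wager, while "bet it all" and decline have no handling.
; The random flip, chat-mode setup and post-transaction nodes are disconnected, so no munny changes hands.
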(event EventBeginPlay
  (|CallParentFunction))

(event EventBndEvtTresComNpcReactorK2NodeComponentBoundEvent3TresReactorDoCommandSignatureDelegateSignature
  (params (CommandCauser :type Tres%20Char%20Pawn%20Base%20Object%20Reference) (CommandID :type ETresCommandKind%20Enum :default "TRES_CMD_KIND_NONE") (ReactorComponent :type Tres%20Reactor%20Component%20Object%20Reference))
  (|CallParentFunction CommandCauser CommandID ReactorComponent)
  (if (Variables|Default|GetTransactionUsed?)
    (bind _returnvalue (Class|TresGameBlueprintLibrary|TresUIOpenChoice (Utilities|Struct|MakeTresLocText "Aye, I've already played ye lad. Patience and munny go hand in hand.") (Utilities|Array|MakeArray (Utilities|Struct|MakeTresLocText "Ok")) (Utilities|Struct|MakeTresUIWindowSetting "WINDOW_WAIT_TYPE_WAIT" "WINDOW_POSITION_TYPE_NONE" "(X=0.000000,Y=0.000000)") 0 false false "World"))
    (Class|TresGameBlueprintLibrary|TresUICloseWindow _returnvalue)
    (Class|TresGameBlueprintLibrary|TresEndCinematicMode false false)
    (else
      (bind _returnvalue_2 (Class|TresGameBlueprintLibrary|TresUIOpenChoice (Utilities|Struct|MakeTresLocText "How much will you bet? Heads, you double. Tails, I take your money. We got a deal lad?") (Utilities|Array|MakeArray (Utilities|Struct|MakeTresLocText "Bet 500") (Utilities|Struct|MakeTresLocText "Bet 5,000") (Utilities|Struct|MakeTresLocText "Bet 10,000") (Utilities|Struct|MakeTresLocText "Bet it all!") (Utilities|Struct|MakeTresLocText "No thanks. This is bad business advice.")) (Utilities|Struct|MakeTresUIWindowSetting "WINDOW_WAIT_TYPE_WAIT" "WINDOW_POSITION_TYPE_NONE" "(X=0.000000,Y=0.000000)") 0 false false "World"))
      (Class|TresGameBlueprintLibrary|TresUICloseWindow _returnvalue_2)
      (switch int _returnvalue_2
        (:0
          (Variables|Default|SetMunnyBidAmount 500))
        (:1
          (Variables|Default|SetMunnyBidAmount 5000))
        (:2
          (Variables|Default|SetMunnyBidAmount 10000))))))

(fn ConstructionScript
  (|CallParentFunction)
  (Variables|Default|SetBark_String "You could learn a thing or two about munny lad! I'll play you for some munny!")
  (Variables|Default|SetNPCName "Scrooge"))