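; Placeholder party-recruit NPC, named as unused, built on a parent NPC Blueprint and given a custom bark line at BeginPlay.
; Its reactor command runs the parent handler, opens a temporary choice window, then closes it and ends cinematic mode.
; Choosing to bring it aboard sets the player's friend party to n_ex001 through the friend manager and destroys the actor.
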(event EventBeginPlay
  (|CallParentFunction)
  (Variables|Default|SetBark_String "Soraaaaa! Over here you big palooka!!!!"))

(event EventBndEvtTresComNpcReactorK2NodeComponentBoundEvent3TresReactorDoCommandSignatureDelegateSignature
  (params (CommandCauser :type Tres%20Char%20Pawn%20Base%20Object%20Reference) (CommandID :type ETresCommandKind%20Enum :default "TRES_CMD_KIND_NONE") (ReactorComponent :type Tres%20Reactor%20Component%20Object%20Reference))
  (|CallParentFunction CommandCauser CommandID ReactorComponent)
  (bind (_outselected _returnvalue) (Class|TresGameBlueprintLibrary|TresUIOpenChoice (Utilities|Struct|MakeTresLocText "TEMP: PARTY MEMBER") (Utilities|Array|MakeArray (Utilities|Struct|MakeTresLocText "Come onboard!") "") (Utilities|Struct|MakeTresUIWindowSetting "WINDOW_WAIT_TYPE_WAIT" "WINDOW_POSITION_TYPE_NONE" "(X=0.000000,Y=0.000000)") 0 false false "World"))
  (Class|TresGameBlueprintLibrary|TresUICloseWindow _returnvalue)
  (Class|TresGameBlueprintLibrary|TresEndCinematicMode false false)
  (if (== _outselected 0)
    (Class|TresFriendComponent|SetFriendAll (Variables|/Script/TresGame.TresPlayerPawnBase|GetMyFrdMgr (Class|TresGameBlueprintLibrary|GetTresPlayerPawnBase)) "n_ex001" "None" "None" "None" "None" "None" false)
    (Actor|DestroyActor)))

(fn ConstructionScript
  (|CallParentFunction))