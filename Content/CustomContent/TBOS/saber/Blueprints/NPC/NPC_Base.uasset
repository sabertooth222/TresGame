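; Base NPC Blueprint that gives characters proximity barks and an interactable chat mode.
; Overlapping the bark volume shows bark text as center information, while the reactor command clears it and starts cinematic mode and chat with the player.
; SetName binds the NPC name to chat mode.
; The post-transaction event disables bark overlaps and shows a timed follow-up bark.
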(event OnReactorDoCommand(TresComNpcReactor)
  (params (CommandCauser :type Tres%20Char%20Pawn%20Base%20Object%20Reference) (CommandID :type ETresCommandKind%20Enum :default "TRES_CMD_KIND_NONE") (ReactorComponent :type Tres%20Reactor%20Component%20Object%20Reference))
  (Class|TresGameBlueprintLibrary|TresUICloseCenterInformation)
  (Class|TresGameBlueprintLibrary|TresStartCinematicModeforLevel false true true true true false false false true false false false false)
  (Class|TresGameBlueprintLibrary|BPTresSetupChatMode (Class|TresGameBlueprintLibrary|GetTresPlayerPawnBase) self))

(event OnComponentBeginOverlap(NPC_Bark)
  (params (OverlappedComponent :type Primitive%20Component%20Object%20Reference) (OtherActor :type Actor%20Object%20Reference) (OtherComp :type Primitive%20Component%20Object%20Reference) (OtherBodyIndex :type Integer) (bFromSweep :type Boolean) (SweepResult :type Hit%20Result%20Structure%20%28by%20ref%29))
  (Utilities|Casting|CastToTresPlayerPawnBase OtherActor)
  (Class|TresGameBlueprintLibrary|TresUIOpenCenterInformation (Utilities|Struct|MakeTresLocText (Variables|Default|GetBark_String))))

(event OnComponentEndOverlap(NPC_Bark)
  (params (OverlappedComponent :type Primitive%20Component%20Object%20Reference) (OtherActor :type Actor%20Object%20Reference) (OtherComp :type Primitive%20Component%20Object%20Reference) (OtherBodyIndex :type Integer))
  (if (not (Variables|Default|GetTransactionUsed?))
    (Utilities|Casting|CastToTresPlayerPawnBase OtherActor)
    (Class|TresGameBlueprintLibrary|TresUICloseCenterInformation)))

(event Custom|PostPurchaseBark
  (params (Bark :type String) (Delay :type Float%20%28single-precision%29))
  (Class|TresGameBlueprintLibrary|TresUIOpenCenterInformation (Utilities|Struct|MakeTresLocText Bark))
  (Utilities|FlowControl|Delay Delay)
  (Class|TresGameBlueprintLibrary|TresUICloseCenterInformation))

(event Custom|Post_Transaction_Event
  (params (Bark :type String) (MessageTime :type Float%20%28single-precision%29))
  (Variables|/Script/Engine.PrimitiveComponent|SetbGenerateOverlapEvents (Variables|Default|GetNPC_Bark) false)
  (Variables|Default|SetTransactionUsed? true)
  (CallFunction|PostPurchaseBark Bark MessageTime))

(event Custom|SetName
  (params (NPCName :type Name))
  (bind _output_get (Variables|Default|SetNPCName NPCName))
  (bind _output_get_2 (Variables|Default|Setm_RecordName _output_get))
  (Class|TresGameBlueprintLibrary|TresEnableComNpcChatMode true _output_get_2))

(event EventBeginPlay
  (Transformation|AttachComponentToComponent (Variables|Default|GetTresComNpcReactor) (Variables|Default|GetMyMesh) "center" "SnapToTarget" "SnapToTarget" "KeepRelative" true)
  (bind _astbos_game_instance (CallFunction|GetTBOSGameInstance))
  (Variables|Default|SetGameInstance _astbos_game_instance))

(fn ConstructionScript)