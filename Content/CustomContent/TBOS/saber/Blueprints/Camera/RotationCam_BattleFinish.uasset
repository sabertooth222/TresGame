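; Boss battle-finish camera actor that plays a slow-motion, multi-angle finishing sequence on spawn, then cleans up the fight.
; BeginPlay enters cinematic mode and staggers three rotating camera shots (enemy, party, enemy) through delayed Sequence pins.
; Each shot moves a spawned note actor to the subject's t_camera bone as the orbit target.
; A white fade hides camera reset, enemy and projectile removal and prize collection before the actor destroys itself.
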(event Custom|Rotation_Camera_Enemy1
  (bind _enemy (Variables|Default|GetEnemy))
  (bind _returnvalue (Class|TresGameBlueprintLibrary|GetBoneTranslationbyName (Variables|/Script/TresGame.TresCharPawnBase|GetMyMesh _enemy) "t_camera" "TBST_WorldSpace"))
  (Transformation|SetActorLocationAndRotation (Variables|Default|GetTresNote) _returnvalue (Transformation|GetActorRotation _enemy) true true)
  (bind _returnvalue_2 (Class|TresCameraRotTarget|SpawnTresCameraRotTarget self 0 "battle_finish"))
  (bind _output_get (Variables|Default|Setrotcam _returnvalue_2))
  (Class|TresCameraBase|SettingTresCamera _output_get (Variables|Default|GetTresNote) 0 self)
  (Class|TresCameraBase|SetPriority (Variables|Default|Getrotcam) 210)
  (Class|TresCameraRotTarget|SetTresCameraRotTargetParam (Variables|Default|Getrotcam) 2.5e+02 "-5.000000,-180.000000,0.000000" "0, 0, 0" "0,-50.000000,0.000000")
  (Class|TresCameraBase|StartTresCamera (Variables|Default|Getrotcam) false (Class|TresCameraBase|SetTresCameraTransitionParams 0.0 "VTBlend_EaseOut" 2.0 false "VTBInterp_LookRotationDistance" "VTBInterpYaw_None" false))
  (Class|TresCameraRotTarget|SetBaseRotation (Variables|Default|Getrotcam) "-10.000000,60.000000,0.000000" 0.5)
  (Class|TresCameraDistanceTarget|SetDistance (Variables|Default|Getrotcam) 3e+02 0.5))

(event Custom|Rotation_camera_Party
  (bind _party (Variables|Default|GetParty))
  (bind _returnvalue (Class|TresGameBlueprintLibrary|GetBoneTranslationbyName (Variables|/Script/TresGame.TresCharPawnBase|GetMyMesh _party) "t_camera" "TBST_WorldSpace"))
  (Transformation|SetActorLocationAndRotation (Variables|Default|GetTresNote) _returnvalue (Transformation|GetActorRotation _party) true true)
  (bind _returnvalue_2 (Class|TresCameraRotTarget|SpawnTresCameraRotTarget self 0 "battle_finish"))
  (bind _output_get (Variables|Default|Setrotcam _returnvalue_2))
  (Class|TresCameraBase|SettingTresCamera _output_get (Variables|Default|GetTresNote) 0 self)
  (Class|TresCameraBase|SetPriority (Variables|Default|Getrotcam) 210)
  (Class|TresCameraRotTarget|SetTresCameraRotTargetParam (Variables|Default|Getrotcam) 4e+02 "-10.000000,120.000000,10.000000" "0, 0, 0" "0, 0,50.000000")
  (Class|TresCameraTarget|EnableCollision (Variables|Default|Getrotcam) false)
  (Class|TresCameraBase|StartTresCamera (Variables|Default|Getrotcam) false (Class|TresCameraBase|SetTresCameraTransitionParams 0.0 "VTBlend_EaseOut" 2.0 false "VTBInterp_LookRotationDistance" "VTBInterpYaw_None" false))
  (Class|TresCameraRotTarget|SetBaseRotation (Variables|Default|Getrotcam) "-10.000000,210.000000,5.000000" 0.5)
  (Class|TresCameraDistanceTarget|SetDistance (Variables|Default|Getrotcam) 5e+02 0.5)
  (Class|TresGameBlueprintLibrary|StopAllCameraShake))

(event Custom|Rotation_Cam_Enemy2
  (bind _enemy (Variables|Default|GetEnemy))
  (bind _returnvalue (Class|TresGameBlueprintLibrary|GetBoneTranslationbyName (Variables|/Script/TresGame.TresCharPawnBase|GetMyMesh _enemy) "t_camera" "TBST_WorldSpace"))
  (Transformation|SetActorLocationAndRotation (Variables|Default|GetTresNote) _returnvalue (Transformation|GetActorRotation _enemy) true true)
  (bind _returnvalue_2 (Class|TresCameraRotTarget|SpawnTresCameraRotTarget self 0 "battle_finish"))
  (bind _output_get (Variables|Default|Setrotcam _returnvalue_2))
  (Class|TresCameraBase|SettingTresCamera _output_get (Variables|Default|GetTresNote) 0 self)
  (Class|TresCameraBase|SetPriority (Variables|Default|Getrotcam) 210)
  (Class|TresCameraRotTarget|SetTresCameraRotTargetParam (Variables|Default|Getrotcam) 8e+02 "-20.000000,45.000000,0.000000" "0, 0, 0" "0, 0, 0")
  (Class|TresCameraBase|StartTresCamera (Variables|Default|Getrotcam) false (Class|TresCameraBase|SetTresCameraTransitionParams 0.0 "VTBlend_EaseOut" 2.0 false "VTBInterp_LookRotationDistance" "VTBInterpYaw_None" false))
  (Class|TresCameraRotTarget|SetBaseRotation (Variables|Default|Getrotcam) "-30.000000,70.000000,0.000000" 0.5)
  (Class|TresCameraDistanceTarget|SetDistance (Variables|Default|Getrotcam) 9.5e+02 0.5))

(event EventBeginPlay
  ;[1 1 1] se00000_047
  (Audio|PlaySound2D "/Game/Sound/SE/common/00000/se00000_047.se00000_047")
  (Class|TresGameBlueprintLibrary|TresStartBossDefeatEffect)
  (Class|TresGameBlueprintLibrary|TresSetDisableGamePause true)
  (Utilities|FlowControl|Sequence
    (:then_0
      (Class|TresGameBlueprintLibrary|SetGlobalGameSpeed "CH_EVENT" 0.05 0.1)
      (bind _returnvalue (Class|TresGameState|GetSceneManager (Class|TresGameBlueprintLibrary|GetTresGameState)))
      (Class|TresSceneManager|SetScreenBlurDefault _returnvalue 0.001 "CH_EVENT" "ScreeneEffectPriority_Hi" true))
    (:then_1
      (Class|TresSoundStatics|TresSoundModeStart "BOSS_DEAD")
      (Class|TresGameBlueprintLibrary|TresStartCinematicMode false false true false false false false true false true false true true)
      (Class|TresGameBlueprintLibrary|TresCinematicPauseAI false true true false false true)
      (bind _returnvalue_2 (Game|SpawnActorfromClass "/Script/TresGame.TresNoteMovable" (Math|Transform|MakeTransform "0, 0, 0") "AdjustIfPossibleButDontSpawnIfColliding" 0 0))
      (Variables|Default|SetTresNote _returnvalue_2))
    (:then_2
      (Class|TresGameBlueprintLibrary|TresWaitCycle 1)
      (CallFunction|RotationCameraEnemy1))
    (:then_3
      (Class|TresGameBlueprintLibrary|TresWaitCycle 1)
      (Class|TresGameBlueprintLibrary|TresDelay 0.05)
      (CallFunction|RotationCameraParty))
    (:then_4
      (Class|TresGameBlueprintLibrary|TresWaitCycle 1)
      (Class|TresGameBlueprintLibrary|TresDelay 0.1)
      (CallFunction|RotationCamEnemy2))
    (:then_5
      (Class|TresGameBlueprintLibrary|TresWaitCycle 1)
      (Utilities|FlowControl|Delay 0.15)
      (Class|TresGameBlueprintLibrary|BPTresStartFadeOut "(R=1.000000,G=1.000000,B=1.000000,A=1.000000)" "SQEX_FADE_LAYER_FG" 0.08 false)
      (Class|TresGameBlueprintLibrary|WaitBPTresStartWhiteOut "SQEX_FADE_LAYER_FG" 0.08 true false)
      (Class|TresGameBlueprintLibrary|TresUIOpenSubtitle (Utilities|Struct|MakeTresLocText "Wait Fadeout Done!") "Cutscene")
      (Class|TresGameBlueprintLibrary|ResetGlobalGameSpeed "CH_EVENT" 0.0)
      (Class|TresGameBlueprintLibrary|TresWaitCycle 1)
      (Class|TresGameBlueprintLibrary|EndAllBPTresCamera false (Class|TresCameraBase|SetTresCameraTransitionParams 0.0 "VTBlend_EaseOut" 2.0 false "VTBInterp_LookRotationDistance" "VTBInterpYaw_None" false))
      (Class|TresGameBlueprintLibrary|TresDelay 1.0)
      (bind _outactors (Actor|GetAllActorsOfClass "/Script/TresGame.TresEnemyPawnBase"))
      (for _array_element _outactors
        ;[1 1 1] For some reason, I do need to destroy all pawns. idk why the aplpy damage doesn't work, maybe because cinematic mode?
        (Game|Damage|ApplyDamage _array_element 999999999.0 0 (Class|TresGameBlueprintLibrary|GetTresPlayerPawnBase)))
      (Class|TresGameBlueprintLibrary|DestroyAllEnemyPawn)
      (Class|TresGameBlueprintLibrary|AllPrizeCollection self (Class|TresGameBlueprintLibrary|GetLocalTresPlayerPawnBase))
      (Actor|DestroyActor (Variables|Default|GetTresNote))
      (Class|TresGameBlueprintLibrary|SetActorStopOff "CH_EVENT" true true false false false false false false false)
      (Class|TresGameBlueprintLibrary|DestroyAllProjectile)
      (Class|TresGameBlueprintLibrary|TresCinematicPlayerStateClear true false false)
      (bind _returnvalue_3 (Class|TresGameState|GetSceneManager (Class|TresGameBlueprintLibrary|GetTresGameState)))
      (Class|TresSceneManager|SetScreenBlurDefault _returnvalue_3 0.01 "CH_EVENT" "ScreeneEffectPriority_Hi" true)
      (Class|TresSoundStatics|TresSoundModeEnd "BOSS_DEAD")
      (Class|TresCameraBase|ResetCamera (Class|TresCameraManager|GetTresCameraNormal (Class|TresGameBlueprintLibrary|GetLocalTresCameraManager)) true)
      (Class|TresGameBlueprintLibrary|CancelFade 0.7 false)
      (Class|TresGameBlueprintLibrary|TresEndCinematicMode true false)
      (Utilities|FlowControl|Delay 0.7)
      (Class|TresGameBlueprintLibrary|SetActorStopOff "CH_EVENT" true true true true false true true true true)
      (Class|TresGameBlueprintLibrary|TresSetDisableGamePause false)
      (Actor|DestroyActor))))

(fn ConstructionScript)