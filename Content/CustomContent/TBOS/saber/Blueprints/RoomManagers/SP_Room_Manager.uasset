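; SP room manager Blueprint that extends a parent room manager and handles setup of "Sp" rooms for the dungeon.
; On BeginPlay it registers itself in the DungeonMaster's SpRoomManagers array.
; SetupRoom appends the room number to the NPC's name, tags the room name with an "Sp" suffix and prints it.
; It then passes that name and a color to the base room setup.
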(event EventSetupRoom
  (params (RoomNumber :type String) (Difficulty :type Integer))
  (bind _returnvalue (Utilities|String|Append RoomNumber "Sp"))
  (bind _npc (Variables|Default|GetNPC))
  ;[1 1 1] Setup Room
  (Default|SetName _npc (Utilities|String|StringToName (Utilities|String|Append (Utilities|String|ToString(Name) (Variables|/Game/CustomContent/TBOS/saber/Blueprints/NPC/NPC_Base.NPC_Base_C|GetNPCName _npc)) RoomNumber)))
  (Variables|Default|SetRoomName _returnvalue)
  (Development|PrintString _returnvalue true true "(R=0.000000,G=1.000000,B=0.146502,A=1.000000)" 1e+01)
  (Default|CallBaseSetupRoomED _returnvalue (Math|Color|MakeColor 150 255 0 255)))

(event EventBeginPlay
  (|CallParentFunction)
  (Utilities|Array|Add (Variables|/Game/CustomContent/TBOS/saber/saber_DungeonMaster.saber_DungeonMaster_C|GetSpRoomManagers (Variables|Default|GetDungeonMaster)) self))

(fn ConstructionScript
  (|CallParentFunction))