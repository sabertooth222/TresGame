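; Battle room manager for procedural dungeons that registers with the DungeonMaster and configures the room's enemy encounter.
; Room setup stores battle volumes and spawn points, randomizes unspecified enemy count and types, with tougher options for final rooms, then async-loads the classes.
; Wave creation chains a random number of follow-up waves after the first, each with a random spawn threshold.
; Randomness uses a seed stream borrowed from and returned to the GameInstance.
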(event Custom|setup_BattleRoom_Event
  (params (GroupName :type Name) (EnemyCount :type Integer) (EnemyStringOptions :type Array%20of%20Pawn%20Object%20References) (SpawnPoints :type Array%20of%20Enemy%20Spawn%20Point%20Object%20References) (StartBattleVolume :type Tres%20Battle%20Volume%20Object%20Reference) (BigBattleVolume :type Tres%20Battle%20Volume%20Object%20Reference) (MaxEnemySize :type EnemySize%20Enum :default "NewEnumerator8"))
  ;[1 1 1] Setup_Battle_variables
  (if (Variables|Default|GetFinalRoom)
    (Default|CallBaseSetupRoomED (Utilities|String|Append "Final" (Variables|Default|GetRoomName)) (Math|Color|MakeColor 50 50 255 255))
    (CallFunction|SetVariables GroupName EnemyCount EnemyStringOptions SpawnPoints StartBattleVolume BigBattleVolume MaxEnemySize)
    (if (== (Utilities|Array|Length EnemyStringOptions) 0)
      (bind (_enemypawnset _localenemyname1) (CallFunction|RandomEnemyPawns (Math|Random|RandomIntegerinRangefromStream 6 10 (Variables|Default|GetSeed)) (Variables|Default|GetSeed) 3 4 (Utilities|Array|MakeArray "NewEnumerator0") false (Variables|Default|GetMaxEnemySize)))
      (Variables|Default|SetEnemyPawnOptions _enemypawnset)
      (Variables|Default|SetEnemyNames _localenemyname1))
    (else
      (CallFunction|SetVariables GroupName EnemyCount EnemyStringOptions SpawnPoints StartBattleVolume BigBattleVolume MaxEnemySize)))
  (Default|GameReturnSeed (Variables|Default|GetGameInstance) (Variables|Default|GetSeed))
  (Utilities|AsyncLoadEnemyClasses (Variables|Default|GetEnemyPawnOptions)
    (:Complete
      (Default|CallFinishedLoadingPawnsED))))

(event Custom|CreateWaves
  ;[1 1 1] Create Normal Waves
  (bind _seed (Default|GameGetSeed (Variables|Default|GetGameInstance)))
  (Variables|Default|SetSeed _seed)
  (bind (_outwave _nextwavenumber) (Utilities|CreateFirstWave (Variables|Default|GetStartBattleVolume) (Variables|Default|GetGroupName) (Variables|Default|GetSpawnPoints) (Variables|Default|GetEnemyPawnOptions) "" (Variables|Default|GetCurrentWaveNumber) (Variables|Default|GetSeed) (Variables|Default|GetEnemyNames) "ETresLevelEntityAppearMode_Perform1" 0.0 0.0))
  (Variables|Default|SetCurrentWaveNumber _nextwavenumber)
  (Variables|Default|SetCurrentWaveName _outwave)
  (bind _output_get (Variables|Default|SetRandomWaveCount (Math|Random|RandomIntegerinRangefromStream 0 2 (Variables|Default|GetSeed))))
  (if (> _output_get 0)
    (for _index (range 1 _output_get)
      (Development|PrintString (Utilities|String|Append "NumBeforeSpawnWave: " (Utilities|String|ToString(Integer) (Math|Random|RandomIntegerinRangefromStream 0 3 (Variables|Default|GetSeed)))) true true "(R=0.000000,G=0.660000,B=1.000000,A=1.000000)" 1e+01)
      (bind _output_get_2 (Variables|Default|SetNumBeforeSpawnNextWave (Math|Random|RandomIntegerinRangefromStream 0 3 (Variables|Default|GetSeed))))
      (bind (_outwave_2 _nextwavenumber_2) (Utilities|CreateWaveNumSpawn (Variables|Default|GetBigBattleVolume) (Variables|Default|GetGroupName) (Variables|Default|GetSpawnPoints) (Variables|Default|GetEnemyPawnOptions) (Variables|Default|GetCurrentWaveName) (Variables|Default|GetCurrentWaveNumber) _output_get_2 (Variables|Default|GetSeed) (Variables|Default|GetEnemyNames) "ETresLevelEntityAppearMode_Perform1" 0.0 0.0))
      (Variables|Default|SetCurrentWaveNumber _nextwavenumber_2)
      (Variables|Default|SetCurrentWaveName _outwave_2))
    (Default|GameReturnSeed (Variables|Default|GetGameInstance) (Variables|Default|GetSeed))
    (else
      (Default|GameReturnSeed (Variables|Default|GetGameInstance) (Variables|Default|GetSeed)))))

(event EventSetupRoom
  (params (RoomNumber :type String) (Difficulty :type Integer))
  (bind _returnvalue (Utilities|String|Append RoomNumber "battle"))
  ;[1 1 1] Setup Room
  (Variables|Default|SetRoomName _returnvalue)
  (Development|PrintString _returnvalue true true "(R=0.000000,G=1.000000,B=0.146502,A=1.000000)" 1e+01)
  (Default|CallBaseSetupRoomED _returnvalue (Math|Color|MakeColor 255 195 104 255)))

(event EventBeginPlay
  ;[1 1 1] Begin Play
  (|CallParentFunction)
  (Utilities|Array|Add (Variables|/Game/CustomContent/TBOS/saber/saber_DungeonMaster.saber_DungeonMaster_C|GetBattleRoom_Managers (Variables|Default|GetDungeonMaster)) self))

(fn ConstructionScript
  (|CallParentFunction))

(fn SetVariables
  (params (GroupName :type Name) (enemyCount :type Integer) (EnemyPawnOptions :type Array%20of%20Pawn%20Object%20References) (SpawnPoints :type Array%20of%20Enemy%20Spawn%20Point%20Object%20References) (StartBattleVolume :type Tres%20Battle%20Volume%20Object%20Reference) (BigBattleVolume :type Tres%20Battle%20Volume%20Object%20Reference) (MaxEnemySize :type EnemySize%20Enum :default "NewEnumerator7"))
  (bind _astbos_game_instance (CallFunction|GetTBOSGameInstance))
  (bind _output_get (Variables|Default|SetGameInstance _astbos_game_instance))
  (bind _seed (Default|GameGetSeed _output_get))
  (Variables|Default|SetSeed _seed)
  (Variables|Default|SetMaxEnemySize MaxEnemySize)
  (Variables|Default|SetGroupName GroupName)
  (if (> enemyCount 0)
    (Variables|Default|SetenemyCount enemyCount)
    (else
      (bind _weightedinttable (CallFunction|CreateWeightedIntTable(FavorHigher) 1 (Utilities|Array|Length SpawnPoints)))
      (bind _randomint (CallFunction|RandomWeightedIntStream _weightedinttable (Variables|Default|GetSeed)))
      (Variables|Default|SetenemyCount _randomint)))
  (if (> (Utilities|Array|Length EnemyPawnOptions) 0)
    (Variables|Default|SetEnemyPawnOptions EnemyPawnOptions)
    (else
      (bind (_enemypawnset _localenemyname1) (CallFunction|RandomEnemyPawns (Math|Random|RandomIntegerinRangefromStream 1 6 (Variables|Default|GetSeed)) (Variables|Default|GetSeed) 1 4 (Utilities|Array|MakeArray "NewEnumerator0") false (Variables|Default|GetMaxEnemySize)))
      (Variables|Default|SetEnemyPawnOptions _enemypawnset)
      (Variables|Default|SetEnemyNames _localenemyname1)))
  (Variables|Default|SetSpawnPoints SpawnPoints)
  (Variables|Default|SetStartBattleVolume StartBattleVolume)
  (Variables|Default|SetBigBattleVolume BigBattleVolume)
  (return))