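; Base room manager Blueprint for the Saber dungeon system, registering each room with the level's dungeon master.
; On BeginPlay it finds the first Saber_DungeonMaster, adds itself to that actor's RoomManagers and caches the reference, printing an error if none is valid.
; SetupRoom forwards the room number and a fixed color through CallBaseSetupRoomED, while SetupRoom_ED_Event stores the number it receives as RoomName.
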(event Custom|SetupRoom_ED_Event
  (params (RoomNumber :type String))
  (Variables|Default|SetRoomName RoomNumber))

(event EventBeginPlay
  (bind _outactors (Actor|GetAllActorsOfClass "/Game/CustomContent/TBOS/saber/saber_DungeonMaster.saber_DungeonMaster_C"))
  (Utilities|IsValid (Utilities|Array|Get(acopy) _outactors)
    (:Is%20Valid
      (Utilities|Array|Add (Variables|/Game/CustomContent/TBOS/saber/saber_DungeonMaster.saber_DungeonMaster_C|GetRoomManagers (Utilities|Array|Get(acopy) _outactors)) self)
      (Variables|Default|SetDungeonMaster (Utilities|Array|Get(acopy) _outactors)))
    (:Is%20Not%20Valid
      (Development|PrintString "Dungeon master not valid!!!" true true "(R=1.000000,G=0.000000,B=0.000000,A=1.000000)" 1.2e+02))))

(event EventSetupRoom
  (params (RoomNumber :type String) (Difficulty :type Integer))
  (Default|CallBaseSetupRoomED RoomNumber (Math|Color|MakeColor 0 195 0 255)))

(fn ConstructionScript)