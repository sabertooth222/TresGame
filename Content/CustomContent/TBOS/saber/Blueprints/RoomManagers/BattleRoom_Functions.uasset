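; Battle room helper functions for wave naming and special-case enemy spawns.
; IterateWaveName builds a wave name from the group name and wave number, and returns the incremented number for the next wave.
; CheckSpecialSpawn flags "Puffball Stack" as special, returning a substitute pawn soft reference from the enemy pawn data table with a special appear mode.
; Other enemy names return non-special with immediate appearance.
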(fn IterateWaveName
  (params (GroupName :type Name) (waveNumber :type Integer))
  (return (Utilities|String|StringToName (Utilities|String|Append (Utilities|String|ToString(Name) GroupName) "Wave" (Utilities|String|ToString(Integer) waveNumber))) (+ waveNumber 1)))

(fn CheckSpecialSpawn
  (params (EnemyName :type Name))
  (switch name EnemyName
    (:Default
      (return false 0 "ETresLevelEntityAppearMode_Immediate"))
    (:PuffballStack
      (bind _returnvalue (Utilities|GetDataTableRow "/Game/CustomContent/TBOS/saber/DataTable/EnemyPawnsDataTable.EnemyPawnsDataTable" "e_ex013")
        (:then
          (return true (.Pawn_SoftRef (Utilities|Struct|BreakEnemyDTStruct _returnvalue)) "ETresLevelEntityAppearMode_Special1"))))))