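; Battle helper function library for the room managers, covering wave naming, special spawns, kill attribution and enemy difficulty.
; Builds numbered wave names, and gives Puffball Stack a special appear mode with its pawn looked up from the enemy data table.
; Resolves a killer to a character pawn via its owner or itself, falling back to player 0.
; Maps global difficulty to min/max enemy tiers, generally harder for final rooms.
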(fn IterateWaveName
  (params (GroupName :type Name) (waveNumber :type Integer))
  (return (Utilities|String|StringToName (Utilities|String|Append (Utilities|String|ToString(Name) GroupName) "Wave" (Utilities|String|ToString(Integer) waveNumber))) (+ waveNumber 1)))

(fn CheckSpecialSpawn
  (params (EnemyName :type Name))
  (switch name EnemyName
    (:Default
      (return false 0 "ETresLevelEntityAppearMode_Immediate"))
    (:PuffballStack
      (bind _returnvalue (Utilities|GetDataTableRow "/Game/CustomContent/TBOS/saber/DataTable/EnemyPawnsDataTable.EnemyPawnsDataTable" "e_ex013")
        (:then
          (return true (.Pawn_SoftRef (Utilities|Struct|BreakEnemyDTStruct _returnvalue)) "ETresLevelEntityAppearMode_Special1"))))))

(fn KilledbyCipher
  (params (KilledBy :type Actor%20Object%20Reference))
  (bind _astres_char_pawn_base (Utilities|Casting|CastToTresCharPawnBase (Components|GetOwner KilledBy))
    (:then
      (return _astres_char_pawn_base))
    (:CastFailed
      (bind _astres_char_pawn_base_2 (Utilities|Casting|CastToTresCharPawnBase KilledBy)
        (:then
          (return _astres_char_pawn_base_2))
        (:CastFailed
          (return (Class|TresGameBlueprintLibrary|GetTresPlayerPawnBase)))))))

(fn RegularEnemyDifficulty
  (params (GlobalDifficulty :type Integer))
  (switch int GlobalDifficulty
    (:1
      (LocalVariables|SetMinDiff 1)
      (LocalVariables|SetMaxDiff 2))
    (:2
      (LocalVariables|SetMinDiff 1)
      (LocalVariables|SetMaxDiff 3))
    (:3
      (LocalVariables|SetMinDiff 1)
      (LocalVariables|SetMaxDiff 4))
    (:4
      (LocalVariables|SetMinDiff 2)
      (LocalVariables|SetMaxDiff 4))
    (:5
      (LocalVariables|SetMinDiff 3)
      (LocalVariables|SetMaxDiff 4)))
  (return (LocalVariables|GetMinDiff) (LocalVariables|GetMaxDiff)))

(fn FinalRoomEnemyDifficulty
  (params (GlobalDifficulty :type Integer))
  (switch int GlobalDifficulty
    (:1
      (LocalVariables|SetMinDiff 1)
      (LocalVariables|SetMaxDiff 3))
    (:2
      (LocalVariables|SetMinDiff 2)
      (LocalVariables|SetMaxDiff 3))
    (:3
      (LocalVariables|SetMinDiff 2)
      (LocalVariables|SetMaxDiff 4))
    (:4
      (LocalVariables|SetMinDiff 3)
      (LocalVariables|SetMaxDiff 4))
    (:5
      (LocalVariables|SetMinDiff 4)
      (LocalVariables|SetMaxDiff 4)))
  (return (LocalVariables|GetMinDiff) (LocalVariables|GetMaxDiff)))