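; RoomFunctions holds helper functions for class-load checks and magic upgrade lookups, filed with the room managers.
; IsClassLoaded resolves a soft class reference and returns whether it is valid along with the class.
; FindNextMagicName&Level finds a magic type in the game instance's unlocked magic and increments its level.
; It then scans the magic data table for that type and level, returning the magic name and VBonus flag.
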(fn IsClassLoaded
  (params (Softclass :type Actor%20Object%20Reference))
  (bind _output (Utilities|ResolveSoftReference Softclass))
  (return (Utilities|IsValidClass _output) _output))

(fn FindNextMagicName&Level
  (params (MagicString :type String))
  (bind _astbos_game_instance (CallFunction|GetTBOSGameInstance))
  (LocalVariables|SetGameInstance _astbos_game_instance)
  (bind _array_element (Utilities|Array|ForEachLoopwithBreak (Variables|/Game/CustomContent/TBOS/saber/TBOS_GameInstance.TBOS_GameInstance_C|GetUnlockedMagic (LocalVariables|GetGameInstance)) :!label _label)
    (:LoopBody
      (if (Utilities|Enum|Equal(Enum) (.MagicType (Utilities|Struct|BreakMagicStruct _array_element)) MagicString)
        (LocalVariables|SetMagicStruct (Utilities|Struct|MakeMagicStruct (.MagicType (Utilities|Struct|BreakMagicStruct _array_element)) (Utilities|Enum|ByteToEnumMagicLevelEnum (+ (.Level (Utilities|Struct|BreakMagicStruct _array_element)) 1)) "" "None"))
        (goto _label Break)))
    (:Completed
      (bind _outrownames (DataTable|GetDataTableRowNames "/Game/CustomContent/TBOS/saber/DataTable/MagicDT.MagicDT"))
      (bind _array_element_2 (Utilities|Array|ForEachLoopwithBreak _outrownames :!label _label_2)
        (:LoopBody
          (bind _returnvalue (Utilities|GetDataTableRow "/Game/CustomContent/TBOS/saber/DataTable/MagicDT.MagicDT" _array_element_2)
            (:then
              (if (and (Utilities|Enum|Equal(Enum) (.MagicType (Utilities|Struct|BreakMagicStruct _returnvalue)) (.MagicType (Utilities|Struct|BreakMagicStruct (LocalVariables|GetMagicStruct)))) (Utilities|Enum|Equal(Enum) (.Level (Utilities|Struct|BreakMagicStruct _returnvalue)) (.Level (Utilities|Struct|BreakMagicStruct (LocalVariables|GetMagicStruct)))))
                (LocalVariables|SetMagicName (.MagicName (Utilities|Struct|BreakMagicStruct _returnvalue)))
                (LocalVariables|SetVBonus (.VBonusFlag (Utilities|Struct|BreakMagicStruct _returnvalue)))
                (goto _label_2 Break)))))
        (:Completed
          (return (LocalVariables|GetMagicName) (LocalVariables|GetVBonus)))))))