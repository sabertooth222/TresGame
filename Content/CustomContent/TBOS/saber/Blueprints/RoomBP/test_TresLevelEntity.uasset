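; Placeable test level entity that configures an enemy spawn from its exposed class, group names and appear settings.
; Its construction script copies these into the entity's spawn fields, building appear info from the actor's own location and rotation.
; For placement preview, it labels itself with the matching EnemyPawnsDataTable name and draws a long-lasting debug capsule.
; An asset-path "_C" suffix fixup is left disconnected.
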(fn ConstructionScript
  (bind _self self)
  (bind _groupnames_exposed (Variables|Default|GetGroupNames_Exposed))
  (bind _appearmode_exposed (Variables|Default|GetAppearMode_exposed))
  (bind _appearwaitmax (Variables|Default|GetAppearWaitMax))
  (bind _appearwaitmin (Variables|Default|GetAppearWaitMin))
  (bind _returnvalue (Transformation|GetActorRotation _self))
  (bind _returnvalue_2 (Transformation|GetActorLocation _self))
  (bind _treslevelentityappearinfo (Utilities|Struct|MakeTresLevelEntityAppearInfo _appearmode_exposed _appearwaitmin _appearwaitmax true 0 _returnvalue_2 _returnvalue))
  (bind _outrownames (DataTable|GetDataTableRowNames "/Game/CustomContent/TBOS/saber/DataTable/EnemyPawnsDataTable.EnemyPawnsDataTable"))
  (for _array_element _outrownames
    (bind _returnvalue_3 (Utilities|GetDataTableRow "/Game/CustomContent/TBOS/saber/DataTable/EnemyPawnsDataTable.EnemyPawnsDataTable" _array_element)
      (:then
        (if (Utilities|Enum|Equal(Enum) (.Pawn_SoftRef (Utilities|Struct|BreakEnemyDTStruct _returnvalue_3)) (Variables|Default|GetMyClass))
          (Rendering|Components|TextRender|SetText (Variables|Default|GetTresDebugTextRender) (Utilities|Text|ToText(Name) (.EnemyName (Utilities|Struct|BreakEnemyDTStruct _returnvalue_3))))))))
  (Rendering|Debug|DrawDebugCapsule (Transformation|GetActorLocation self) 9e+01 5e+01 "0, 0, 0" "(R=1.000000,G=0.937172,B=0.000000,A=1.000000)" 1e+03 0.0)
  (Variables|Default|Setm_ActorClass (Utilities|ResolveSoftReference (Variables|Default|GetMyClass)))
  (if (> (Utilities|Array|Length _groupnames_exposed) 0)
    (Variables|Default|Setm_GroupNames _groupnames_exposed))
  (Variables|Default|Setm_AppearInfo _self (Utilities|Array|MakeArray _treslevelentityappearinfo))
  (Variables|Default|Setm_CurrentAppearInfo _treslevelentityappearinfo))