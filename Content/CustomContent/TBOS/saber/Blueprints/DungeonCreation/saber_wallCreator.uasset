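; Dungeon-creation actor that spawns walls around each segment in its Corridors array at BeginPlay.
; CreateWalls offsets both sides of a segment and closes its two ends, running TraceTestsV2 on each edge.
; Forward and reverse line traces, ignoring battle volumes and spawned walls, split edges at obstructions, leaving gaps where corridors intersect.
; Clear spans become stretched Test_SplineWall actors; debug drawing remains on, while TraceTests and OverlapCheck are never called.
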(event EventBeginPlay
  (bind _outactors (Actor|GetAllActorsOfClass "/Script/TresGame.TresBattleVolume"))
  (Variables|Default|SetIgnored_Actors _outactors)
  (for _array_element (Variables|Default|GetCorridors)
    (Variables|Default|SetStartPoint (.StartPoint (Utilities|Struct|BreakPathStruct _array_element)))
    (Variables|Default|SetEndPoint (.Endpoint (Utilities|Struct|BreakPathStruct _array_element)))
    (CallFunction|CreateWalls (Variables|Default|GetStartPoint) (Variables|Default|GetEndPoint))))

(fn ConstructionScript)

(fn SpawnIndividualSplineWall
  (params (Start :type Vector) (Target :type Vector))
  (bind _returnvalue (Game|SpawnActorfromClass "/Game/CustomContent/TBOS/saber/Test/Test_SplineWall.Test_SplineWall_C" (Math|Transform|MakeTransform Start) "Undefined" 0 0))
  (Transformation|SetWorldRotation (Variables|/Game/CustomContent/TBOS/saber/Test/Test_SplineWall.Test_SplineWall_C|GetSplineMesh _returnvalue) (Math|Rotator|FindLookatRotation Start Target) false false)
  (SplineMesh|SetEndPosition (Variables|/Game/CustomContent/TBOS/saber/Test/Test_SplineWall.Test_SplineWall_C|GetSplineMesh _returnvalue) (Math|Vector|MakeVector (Math|Vector|VectorLength (- Target Start)) 0.0 0.0) true)
  (Utilities|Array|Add (Variables|Default|GetIgnored_Actors) _returnvalue)
  (return))

(fn TraceTests
  (params (start :type Vector) (end :type Vector))
  (bind _output_get (LocalVariables|SetLocalStart start))
  (LocalVariables|SetInitialStart _output_get)
  (bind _output_get_2 (LocalVariables|SetLocalEnd end))
  (LocalVariables|SetLineDir (Math|Vector|GetUnitDirection(Vector) _output_get _output_get_2))
  (LocalVariables|SetCorridor_Length (Math|Float|Absolute(Float) (Math|Vector|VectorLength (- (LocalVariables|GetLocalStart) (LocalVariables|GetLocalEnd)))))
  (bind (_outhits _returnvalue) (Class|KismetSystemLibrary|LineTraceMultiforObjects (LocalVariables|GetLocalStart) (LocalVariables|GetLocalEnd) (Utilities|Array|MakeArray "ObjectTypeQuery1" "ObjectTypeQuery2") false (Variables|Default|GetIgnored_Actors) "Persistent" true))
  (if _returnvalue
    (for _array_element _outhits
      (if (>= (Math|Vector|VectorLength (- (LocalVariables|GetLocalStart) (.ImpactPoint (Collision|BreakHitResult _array_element)))) 1.0)
        (CallFunction|SpawnIndividualSplineWall (LocalVariables|GetLocalStart) (.ImpactPoint (Collision|BreakHitResult _array_element))))
      (if (> (.X (Math|Vector|BreakVector (* "0, 0, 0" (LocalVariables|GetLineDir)))) (.Y (Math|Vector|BreakVector (* "0, 0, 0" (LocalVariables|GetLineDir)))))
        (LocalVariables|Setre-center%20for%20axis (Math|Vector|MakeVector (.X (Math|Vector|BreakVector (* "0, 0, 0" (LocalVariables|GetLineDir)))) (.Y (Math|Vector|BreakVector (.ImpactPoint (Collision|BreakHitResult _array_element)))) -1e+01))
        (else
          (LocalVariables|Setre-center%20for%20axis (Math|Vector|MakeVector (.X (Math|Vector|BreakVector (.ImpactPoint (Collision|BreakHitResult _array_element)))) (.Y (Math|Vector|BreakVector (* "0, 0, 0" (LocalVariables|GetLineDir)))) 0.0))))
      (LocalVariables|SetLocalStart (+ (.ImpactPoint (Collision|BreakHitResult _array_element)) (* (LocalVariables|GetLineDir) (Math|Vector|VectorLength (* "0, 0, 0" (LocalVariables|GetLineDir)))))))
    (if (< (Math|Float|Absolute(Float) (Math|Vector|VectorLength (- (LocalVariables|GetInitialStart) (LocalVariables|GetLocalStart)))) (LocalVariables|GetCorridor_Length))
      (CallFunction|SpawnIndividualSplineWall (LocalVariables|GetLocalStart) (LocalVariables|GetLocalEnd)))
    (else
      (CallFunction|SpawnIndividualSplineWall (LocalVariables|GetLocalStart) (LocalVariables|GetLocalEnd)))))

(fn TraceTestsV2
  (params (start :type Vector) (end :type Vector))
  (bind _output_get (LocalVariables|SetLocalStart start))
  (bind _output_get_2 (LocalVariables|SetInitialStart _output_get))
  (bind _output_get_3 (LocalVariables|SetLocalEnd end))
  ;[1 1 1] This checks to see if there are stopping points (ie wall collides with an intersecting path)
  (LocalVariables|SetLineDir (Math|Vector|GetUnitDirection(Vector) _output_get_2 _output_get_3))
  (LocalVariables|SetCorridor_Length (Math|Float|Absolute(Float) (Math|Vector|VectorLength (- (LocalVariables|GetLocalStart) (LocalVariables|GetLocalEnd)))))
  (bind (_outhits _returnvalue) (Class|KismetSystemLibrary|LineTraceMultiforObjects (LocalVariables|GetLocalStart) (LocalVariables|GetLocalEnd) (Utilities|Array|MakeArray "ObjectTypeQuery1" "ObjectTypeQuery2") false (Variables|Default|GetIgnored_Actors) "Persistent" true))
  (if _returnvalue
    ;[1 1 1] This traces from the opposite end for collisions
    (bind (_outhits_2 _returnvalue_2) (Class|KismetSystemLibrary|LineTraceMultiforObjects (LocalVariables|GetLocalEnd) (LocalVariables|GetLocalStart) (Utilities|Array|MakeArray "ObjectTypeQuery1" "ObjectTypeQuery2") false (Variables|Default|GetIgnored_Actors) "Persistent" true "(R=1.000000,G=0.000000,B=0.600456,A=1.000000)" "(R=0.000000,G=0.219207,B=1.000000,A=1.000000)"))
    (for (_array_element _array_index) _outhits
      ;[1 1 1] This stops walls from spawning on first collision that =0 lenght (ie if a wall/corridor starts inside another corridor)
      (if (>= (Math|Float|Absolute(Float) (Math|Vector|VectorLength (- (LocalVariables|GetLocalStart) (.ImpactPoint (Collision|BreakHitResult _array_element))))) 1.0)
        ;[1 0.3794 0] Not sure what the point of this is...
        (if (Math|Vector|Equal(Vector) (Math|Vector|GetUnitDirection(Vector) (LocalVariables|GetLocalStart) (.ImpactPoint (Collision|BreakHitResult _array_element))) (LocalVariables|GetLineDir) 0.0001)
          (CallFunction|SpawnIndividualSplineWall (LocalVariables|GetLocalStart) (.ImpactPoint (Collision|BreakHitResult _array_element)))))
      (if _returnvalue_2
        ;[1 1 1] Sets last trace hit from opposite end as next start point
        (Rendering|Debug|DrawDebugBox (.ImpactPoint (Collision|BreakHitResult _array_element)) "50.000000,50.000000,50.000000" "(R=0.000000,G=1.000000,B=0.950728,A=1.000000)" "0, 0, 0" 1.2e+02 3.0)
        (LocalVariables|SetLocalStart (.Location (Collision|BreakHitResult (Utilities|Array|Get(acopy) _outhits_2 (- (Utilities|Array|LastIndex _outhits_2) _array_index)))))
        (Rendering|Debug|DrawDebugBox (.Location (Collision|BreakHitResult (Utilities|Array|Get(acopy) _outhits_2 (- (Utilities|Array|LastIndex _outhits_2) _array_index)))) "50.000000,50.000000,50.000000" "(R=1.000000,G=0.000000,B=0.367432,A=1.000000)" "0, 0, 0" 1.2e+02 3.0)
        (else
          (LocalVariables|SetLocalStart (.ImpactPoint (Collision|BreakHitResult _array_element))))))
    ;[1 1 1] If the length of the last reverse impact hit to the end would be greater than 1, spawn a wall (if it's 1 or less, that means the reverse line started inside another corridor or mesh)
    (if (>= (Math|Float|Absolute(Float) (Math|Vector|VectorLength (- (LocalVariables|GetLocalStart) (LocalVariables|GetLocalEnd)))) 1.0)
      (CallFunction|SpawnIndividualSplineWall (LocalVariables|GetLocalStart) (LocalVariables|GetLocalEnd)))
    (elif (>= (Math|Float|Absolute(Float) (Math|Vector|VectorLength (- (LocalVariables|GetLocalStart) (LocalVariables|GetLocalEnd)))) 1.0)
      (CallFunction|SpawnIndividualSplineWall (LocalVariables|GetLocalStart) (LocalVariables|GetLocalEnd)))))

(fn OverlapCheck
  (params (Start+OverlapPoint :type Vector) (Target%28forLookAtRotation%29 :type Vector))
  (bind _returnvalue (Game|SpawnActorfromClass "/Game/CustomContent/TBOS/saber/Blueprints/DungeonCreation/Wall_CollisionTrigger.Wall_CollisionTrigger_C" (Math|Transform|MakeTransform Start+OverlapPoint (Math|Rotator|FindLookatRotation Start+OverlapPoint Target%28forLookAtRotation%29)) "Undefined" 0 0))
  (Development|PrintString (Utilities|String|ToString(Integer) (Utilities|Array|Length (Collision|GetOverlappingActors (Variables|/Game/CustomContent/TBOS/saber/Blueprints/DungeonCreation/Wall_CollisionTrigger.Wall_CollisionTrigger_C|GetBox _returnvalue) 0 :!class /Script/Engine.PrimitiveComponent))) true true "(R=0.000000,G=0.660000,B=1.000000,A=1.000000)" 3e+01)
  (return (> (Utilities|Array|Length (Collision|GetOverlappingActors (Variables|/Game/CustomContent/TBOS/saber/Blueprints/DungeonCreation/Wall_CollisionTrigger.Wall_CollisionTrigger_C|GetBox _returnvalue) 0 :!class /Script/Engine.PrimitiveComponent)) 0)))

(fn FindRightOffset
  (params (StartPoint :type Vector) (Endpoint%28ForDirection%29 :type Vector) (Offest :type Integer))
  (bind _returnvalue (Math|Vector|GetUnitDirection(Vector) StartPoint Endpoint%28ForDirection%29))
  (return (- (+ StartPoint (* (Math|Vector|CrossProduct _returnvalue "0, 0,1.000000") Offest) (* _returnvalue -1)) "0, 0,10.000000") (- (+ Endpoint%28ForDirection%29 (* (Math|Vector|CrossProduct _returnvalue "0, 0,1.000000") Offest) (* _returnvalue 1)) "0, 0,10.000000")))

(fn CreateWalls
  (params (StartPoint :type Vector) (Endpoint%28ForDirection%29 :type Vector))
  ;[1 1 1] Creates walls on "right" side
  (bind (_offset_location_start _offset_location_end) (CallFunction|FindRightOffset StartPoint Endpoint%28ForDirection%29 201))
  (LocalVariables|SetRight_Offset_Start _offset_location_start)
  (LocalVariables|SetRight_Offset_end _offset_location_end)
  (CallFunction|TraceTestsV2 (LocalVariables|GetRight_Offset_Start) (LocalVariables|GetRight_Offset_end))
  ;[1 1 1] Creates walls on "left" side
  (bind (_offset_location_start_2 _offset_location_end_2) (CallFunction|FindRightOffset StartPoint Endpoint%28ForDirection%29 -201))
  (LocalVariables|SetLeft_Offset_Start _offset_location_start_2)
  (LocalVariables|SetLeft_Offset_end _offset_location_end_2)
  (CallFunction|TraceTestsV2 (LocalVariables|GetLeft_Offset_Start) (LocalVariables|GetLeft_Offset_end))
  ;[1 1 1] Creates walls on front/back
  (CallFunction|TraceTestsV2 (LocalVariables|GetLeft_Offset_Start) (LocalVariables|GetRight_Offset_Start))
  (CallFunction|TraceTestsV2 (LocalVariables|GetLeft_Offset_end) (LocalVariables|GetRight_Offset_end)))