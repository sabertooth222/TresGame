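; Seeded dungeon floor layout generator that fills TileMap with a spawn room plus random counts of battle and special rooms.
; On BeginPlay it takes the DungeonMaster's random stream, draws rooms from RoomDT by type in mixed order, then hands the stream back.
; Placement uses rejection sampling against room extents plus padding, enlarging the grid's maximum bounds after too many failed attempts.
; Level-instance loading and older generation passes are unused.
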(event EventBeginPlay
  (bind _seed (Default|GetFloorSeed (Variables|Default|GetDungeonMaster)))
  (Variables|Default|SetSeed _seed)
  (bind _outrownames (DataTable|GetDataTableRowNames "/Game/CustomContent/TBOS/saber/DataTable/RoomDT.RoomDT"))
  (while (not (Variables|Default|GetSpawnFound?))
    (bind _returnvalue (Utilities|GetDataTableRow "/Game/CustomContent/TBOS/saber/DataTable/RoomDT.RoomDT" (Utilities|Array|Get(acopy) _outrownames (Math|Random|RandomIntegerinRangefromStream 0 (Utilities|Array|LastIndex _outrownames) (Variables|Default|GetSeed))))
      (:then
        (if (Utilities|Enum|Equal(Enum) (.RoomType (Utilities|Struct|BreakRoomStruct _returnvalue)) "NewEnumerator0")
          (Variables|Default|SetSpawnRoom _returnvalue)
          (Variables|Default|SetSpawnFound? true)))))
  ;[1 0.8991 0.2581] Room Amount and Grid Size are instanced variables set in dungeon master!!!
  (Utilities|Array|Add (Variables|Default|GetTileMap) (Variables|Default|GetSpawnRoom))
  (bind _output_get (Variables|Default|SetFinalBattleRoomAmount (Math|Random|RandomIntegerinRangefromStream (Variables|Default|GetMinBRoomAmount) (Variables|Default|GetMaxbattleRoomAmount) (Variables|Default|GetSeed))))
  (Variables|Default|SetFinalSpecialRoomAmount (Math|Random|RandomIntegerinRangefromStream (Variables|Default|GetMinSpRoom) (Variables|Default|GetMaxSpRoom) (Variables|Default|GetSeed)))
  (Development|PrintString (Utilities|String|ToString(Integer) _output_get) true true "(R=0.000000,G=1.000000,B=0.268722,A=1.000000)" 3e+01)
  (for _index (range 1 (+ (Variables|Default|GetFinalBattleRoomAmount) (Variables|Default|GetFinalSpecialRoomAmount)))
    (bind _sproom_ (CallFunction|RandomRoomType))
    (if _sproom_
      (bind _room1 (CallFunction|FindRandomSpRoom))
      (Variables|Default|SetNewRoomSize (.RoomSizefromCenter (Utilities|Struct|BreakRoomStruct _room1)))
      (CallFunction|Generate+AddRoom (.RoomPath (Utilities|Struct|BreakRoomStruct _room1)))
      (else
        (bind _room1_2 (CallFunction|FindRandomBattleRoom))
        (Variables|Default|SetNewRoomSize (.RoomSizefromCenter (Utilities|Struct|BreakRoomStruct _room1_2)))
        (CallFunction|Generate+AddRoom (.RoomPath (Utilities|Struct|BreakRoomStruct _room1_2))))))
  (Default|ReturnFloorSeed (Variables|Default|GetDungeonMaster) (Variables|Default|GetSeed))
  (Development|PrintString (Utilities|String|Append "attempts" (Utilities|String|ToString(Integer) (Variables|Default|GetAttempts))) true true "(R=1.000000,G=0.000000,B=0.833106,A=1.000000)" 3e+01)
  (Development|PrintString (Utilities|String|Append "Resets: " (Utilities|String|ToString(Integer) (Variables|Default|GetResets))) true true "(R=0.463340,G=0.331302,B=1.000000,A=1.000000)" 3e+01))

(fn ConstructionScript)

(fn RoomCheckDistance
  (params (CenterVec :type Vector) (OldRoomSize :type Vector%202D%20Structure) (CheckRandVector :type Vector) (CheckRoomSize :type Vector%202D%20Structure))
  (bind (_x _y) (Math|Vector|BreakVector CheckRandVector))
  (bind (_x_2 _y_2) (Math|Vector|BreakVector CenterVec))
  (bind (_x_3 _y_3) (Math|Vector2D|BreakVector2D OldRoomSize))
  (bind (_x_4 _y_4) (Math|Vector2D|BreakVector2D CheckRoomSize))
  (return (or (> (Math|Float|Absolute(Float) (- _x_2 _x)) (+ _x_3 1e+03 _x_4)) (> (Math|Float|Absolute(Float) (- _y_2 _y)) (+ _y_3 1e+03 _y_4)))))

(fn UNUSEDOLDGenerateRooms
  (params (NumberOfRooms :type Integer) (RoomType :type String) (MinX :type Integer) (MaxX :type Integer) (MinY :type Integer) (MaxY :type Integer))
  (bind _seed (Variables|Default|GetSeed))
  (for _index (range 1 NumberOfRooms)
    (LocalVariables|SetPotentialVector (Math|Vector|MakeVector (Math|Conversions|ToFloat(Integer) (Math|Random|RandomIntegerinRangefromStream MinX MaxX _seed)) (Math|Conversions|ToFloat(Integer) (Math|Random|RandomIntegerinRangefromStream MinY MaxY _seed)) 0.0) :!label _label)
    (bind _array_element (Utilities|Array|ForEachLoopwithBreak (Variables|Default|GetTileMap) :!label _label_2)
      (:LoopBody
        (if (Math|Vector|Equal(Vector) (LocalVariables|GetPotentialVector) (.MidPointVector (Utilities|Struct|BreakRoomStruct _array_element)) 0.0)
          (LocalVariables|SetDupedVector true)
          (goto _label_2 Break)))
      (:Completed
        (if (LocalVariables|GetDupedVector)
          (LocalVariables|SetDupedVector false)
          (goto _label)
          (else
            (Utilities|Array|Add (Variables|Default|GetTileMap) (Utilities|Struct|MakeRoomStruct (LocalVariables|GetPotentialVector) (Variables|Default|GetNewRoomSize) RoomType))
            (LocalVariables|SetDupedVector false))))))
  (return))

(fn UNUSEDOLDCheckRooms
  (bind _tilemap (Variables|Default|GetTileMap))
  (bind (_arrayindex _arrayelement) (Utilities|Array|ReverseforEachLoop (Variables|Default|GetTileMap))
    (:LoopBody
      (if (Utilities|Enum|NotEqual(Enum) (.RoomPath (Utilities|Struct|BreakRoomStruct _arrayelement)) (Variables|Default|GetStartCell))
        (LocalVariables|SetVectorCheck (.MidPointVector (Utilities|Struct|BreakRoomStruct _arrayelement)))
        (LocalVariables|SetVectorCheckLength (.RoomSizefromCenter (Utilities|Struct|BreakRoomStruct _arrayelement)))
        (bind _index (Utilities|FlowControl|ForLoopwithBreak (* (Utilities|Array|LastIndex _tilemap) -1) 0 :!label _label)
          (:LoopBody
            (if (not (== (* _index -1) _arrayindex))
              (bind _distance_combinedroomsize_ (CallFunction|RoomCheckDistance (.MidPointVector (Utilities|Struct|BreakRoomStruct (Utilities|Array|Get(acopy) _tilemap (* _index -1)))) (.RoomSizefromCenter (Utilities|Struct|BreakRoomStruct (Utilities|Array|Get(acopy) _tilemap (* _index -1)))) (LocalVariables|GetVectorCheck) (LocalVariables|GetVectorCheckLength)))
              (if (== (Variables|Default|GetAttempts) 1021)
                (if (not _distance_combinedroomsize_)
                  (Utilities|Array|RemoveIndex (Variables|Default|GetTileMap) _arrayindex :!label _label_2)
                  (goto _label Break))
                (elif (not _distance_combinedroomsize_)
                  (goto _label_2))))))))
    (:Completed
      (return))))

(fn UNUSEDOLDDeleteExtraRooms
  (params (MaxRoomAmount :type Integer))
  (bind _tilemap (Variables|Default|GetTileMap))
  (if (> (Utilities|Array|Length (Variables|Default|GetTileMap)) MaxRoomAmount) :!label _label
    (LocalVariables|SetRandomIndex (Class|KismetMathLibrary|RandomIntegerfromStream (Utilities|Array|Length (Variables|Default|GetTileMap)) (Variables|Default|GetSeed)))
    (if (Utilities|Enum|NotEqual(Enum) (.RoomPath (Utilities|Struct|BreakRoomStruct (Utilities|Array|Get(acopy) _tilemap (LocalVariables|GetRandomIndex)))) (Variables|Default|GetStartCell))
      (Utilities|Array|RemoveIndex _tilemap (LocalVariables|GetRandomIndex))
      (goto _label)
      (else
        (goto _label)))
    (else
      (return))))

(fn Generate+AddRoom
  (params (RoomType :type String))
  (bind _seed (Variables|Default|GetSeed))
  (Variables|Default|SetVIableVector (Math|Vector|MakeVector (Math|Conversions|ToFloat(Integer) (Math|Random|RandomIntegerinRangefromStream (Variables|Default|GetGrid_MinX) (Variables|Default|GetGridMax_X) _seed)) (Math|Conversions|ToFloat(Integer) (Math|Random|RandomIntegerinRangefromStream (Variables|Default|GetGrid_MinY) (Variables|Default|GetGrid_MaxY) _seed)) 0.0) :!label _label)
  (bind _array_element (Utilities|Array|ForEachLoopwithBreak (Variables|Default|GetTileMap) :!label _label_2)
    (:LoopBody
      (bind _result (Math|Integer|IncrementInt (Variables|Default|GetAttempts))
        (:%20%20
          (bind _distance_combinedroomsize_ (CallFunction|RoomCheckDistance (.MidPointVector (Utilities|Struct|BreakRoomStruct _array_element)) (.RoomSizefromCenter (Utilities|Struct|BreakRoomStruct _array_element)) (Variables|Default|GetVIableVector) (Variables|Default|GetNewRoomSize)))
          (if _distance_combinedroomsize_
            (Variables|Default|SetFoundPossible_roomVector true)
            (else
              (Variables|Default|SetFoundPossible_roomVector false)
              (goto _label_2 Break))))))
    (:Completed
      (if (Variables|Default|GetFoundPossible_roomVector)
        (Utilities|Array|Add (Variables|Default|GetTileMap) (Utilities|Struct|MakeRoomStruct (Math|Vector|MakeVector (.X (Math|Vector|BreakVector (Variables|Default|GetVIableVector))) (.Y (Math|Vector|BreakVector (Variables|Default|GetVIableVector))) 0.0) (Variables|Default|GetNewRoomSize) RoomType))
        (Variables|Default|SetFoundPossible_roomVector false)
        (return)
        (elif (> (Variables|Default|GetAttempts) 10000)
          (Math|Integer|IncrementInt (Variables|Default|GetAttempts)
            (:%20%20
              (Variables|Default|SetGridMax_X (Math|Float|Truncate (* (Variables|Default|GetGridMax_X) 1.5)))
              (Variables|Default|SetGrid_MaxY (Math|Float|Truncate (* (Variables|Default|GetGrid_MaxY) 1.5)))
              (Math|Integer|IncrementInt (Variables|Default|GetResets)
                (:%20%20
                  (Variables|Default|SetAttempts 1)
                  (goto _label)))))
          (else
            (Math|Integer|IncrementInt (Variables|Default|GetAttempts)
              (:%20%20
                (goto _label)))))))))

(fn FindRandomBattleRoom
  (bind _outrownames (DataTable|GetDataTableRowNames "/Game/CustomContent/TBOS/saber/DataTable/RoomDT.RoomDT"))
  (while (not (LocalVariables|GetRoomFound))
    (bind _returnvalue (Utilities|GetDataTableRow "/Game/CustomContent/TBOS/saber/DataTable/RoomDT.RoomDT" (Utilities|Array|Get(acopy) _outrownames (Math|Random|RandomIntegerinRangefromStream 0 (Utilities|Array|LastIndex _outrownames) (Variables|Default|GetSeed))))
      (:then
        (if (Utilities|Enum|Equal(Enum) (.RoomType (Utilities|Struct|BreakRoomStruct _returnvalue)) "NewEnumerator1")
          (LocalVariables|SetRoom _returnvalue)
          (LocalVariables|SetRoomFound true)))))
  (return (LocalVariables|GetRoom)))

(fn FindRandomSpRoom
  (bind _outrownames (DataTable|GetDataTableRowNames "/Game/CustomContent/TBOS/saber/DataTable/RoomDT.RoomDT"))
  (while (not (LocalVariables|GetRoomFound))
    (bind _returnvalue (Utilities|GetDataTableRow "/Game/CustomContent/TBOS/saber/DataTable/RoomDT.RoomDT" (Utilities|Array|Get(acopy) _outrownames (Math|Random|RandomIntegerinRangefromStream 0 (Utilities|Array|LastIndex _outrownames) (Variables|Default|GetSeed))))
      (:then
        (if (Math|Boolean|ORBoolean (Utilities|Enum|Equal(Enum) (.RoomType (Utilities|Struct|BreakRoomStruct _returnvalue)) "NewEnumerator3") (Utilities|Enum|Equal(Enum) (.RoomType (Utilities|Struct|BreakRoomStruct _returnvalue)) "NewEnumerator2") (Utilities|Enum|Equal(Enum) (.RoomType (Utilities|Struct|BreakRoomStruct _returnvalue)) "NewEnumerator4"))
          (LocalVariables|SetRoom _returnvalue)
          (LocalVariables|SetRoomFound true)))))
  (return (LocalVariables|GetRoom)))

(fn RandomRoomType
  (if (== (Variables|Default|GetFinalBattleRoomAmount) (Variables|Default|GetTotalCreatedBattleRooms))
    _
    (elif (== (Variables|Default|GetFinalSpecialRoomAmount) (Variables|Default|GetTotalCreatedSpRoom))
      (Math|Integer|IncrementInt (Variables|Default|GetTotalCreatedBattleRooms)
        (:%20%20
          (return false)))
      (else
        (bind _output_get (LocalVariables|SetRandomCreateSpRoom? (Math|Random|RandomBoolfromStream (Variables|Default|GetSeed))))
        (if _output_get
          _
          (else
            (Math|Integer|IncrementInt (Variables|Default|GetTotalCreatedBattleRooms)
              (:%20%20
                (return false))))))))
  (Math|Integer|IncrementInt (Variables|Default|GetTotalCreatedSpRoom)
    (:%20%20
      (return true))))