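; Dungeon level loader that streams in room levels from a tile map, one after another, to build a dungeon.
; On BeginPlay it walks TileMap, instancing each RoomPath level at its MidPointVector with no rotation.
; Each instance's OnLevelLoaded event advances the index and loads the next room, so loading stays sequential.
; After the last room it calls LoadingLevelsFinished on the DungeonMaster.
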(event Custom|LevelLoaded
  (EventDispatchers|UnbindEventfromOnLevelLoaded (stale Custom|LoadNextLevel _returnvalue) (delegate Custom|LevelLoaded))
  (bind _outactors (Actor|GetAllActorsOfClass "/Game/CustomContent/TBOS/saber/Blueprints/RoomManagers/Room_Manager_Base.Room_Manager_Base_C"))
  (if (== (Variables|Default|GetTileMap_FinalIndex) (Variables|Default|GetTilemap_CurrentIndex))
    (Default|LoadingLevelsFinished (Variables|Default|GetDungeonMaster))
    (else
      (Math|Integer|IncrementInt (Variables|Default|GetTilemap_CurrentIndex)
        (:%20%20
          (CallFunction|LoadNextLevel))))))

(event Custom|LoadNextLevel
  (bind _tilemap (Variables|Default|GetTileMap))
  (bind _tilemap_currentindex (Variables|Default|GetTilemap_CurrentIndex))
  (bind _output (Utilities|Array|Get(acopy) _tilemap _tilemap_currentindex))
  (bind (_midpointvector _roomsizefromcenter _roompath) (Utilities|Struct|BreakRoomStruct _output))
  (bind _returnvalue (Class|LevelStreamingKismet|LoadLevelInstance _roompath _midpointvector (Math|Rotator|MakeRotator 0.0 0.0 0.0)))
  (EventDispatchers|BindEventtoOnLevelLoaded _returnvalue (delegate Custom|LevelLoaded)))

(event EventBeginPlay
  (Variables|Default|SetTileMap_FinalIndex (Utilities|Array|LastIndex (Variables|Default|GetTileMap)))
  (Variables|Default|SetTilemap_CurrentIndex 0)
  (bind _returnvalue (Class|LevelStreamingKismet|LoadLevelInstance (.RoomPath (Utilities|Struct|BreakRoomStruct (Utilities|Array|Get(acopy) (Variables|Default|GetTileMap) (Variables|Default|GetTilemap_CurrentIndex)))) (.MidPointVector (Utilities|Struct|BreakRoomStruct (Utilities|Array|Get(acopy) (Variables|Default|GetTileMap) (Variables|Default|GetTilemap_CurrentIndex)))) (Math|Rotator|MakeRotator 0.0 0.0 0.0)))
  (EventDispatchers|BindEventtoOnLevelLoaded _returnvalue (delegate Custom|LevelLoaded)))

(fn ConstructionScript)