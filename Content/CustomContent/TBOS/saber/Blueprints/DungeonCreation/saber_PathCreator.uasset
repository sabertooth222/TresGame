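; Dungeon corridor generator that links room centers along MST edges on BeginPlay, or to their nearest unlinked rooms when no edges exist.
; Each edge joins the closest entry point pair, opens their doors and lays axis-aligned spline segments in seeded random X/Y order.
; Line traces stop segments short of obstacles, with doubling sidesteps checked against tile-map room bounds when blocked.
; Recorded corridor segments then go to a spawned Saber_wallCreator.
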(event EventBeginPlay
  (bind _astbos_game_instance (CallFunction|GetTBOSGameInstance))
  (bind _output_get (Variables|Default|SetGameInstance _astbos_game_instance))
  (bind _seed (Default|GameGetSeed _output_get))
  (Variables|Default|SetRoomSeed _seed)
  (if (== (Utilities|Array|Length (Variables|Default|GetEdges)) 0)
    ;[1 1 1] If MST is empty (ie - rooms are straight line), then this draws lines between each room
    (CallFunction|NoMSTCreateLinksBetweenClosestRooms))
  (for _array_element (Variables|Default|GetEdges)
    (Variables|Default|SetRoomCenterCount 0)
    ;[1 1 1] Finds matching room center with MST edge, then breaks once it finds the 2 matching room centers
    (bind _array_element_2 (Utilities|Array|ForEachLoopwithBreak (Variables|Default|GetRoomCenters) :!label _label)
      (:LoopBody
        (if (Math|Vector|Equal(Vector) (Math|Conversions|ToVector2D(Vector) (Transformation|GetActorLocation _array_element_2)) (.A (Utilities|Struct|BreakEdge+Distance _array_element)) 0.0)
          (Variables|Default|SetRoom_CenterA _array_element_2)
          (bind _result (Math|Integer|IncrementInt (Variables|Default|GetRoomCenterCount) :!label _label_2)
            (:%20%20
              (if (== _result 2)
                (goto _label Break))))
          (elif (Math|Vector|Equal(Vector) (Math|Conversions|ToVector2D(Vector) (Transformation|GetActorLocation _array_element_2)) (.B (Utilities|Struct|BreakEdge+Distance _array_element)) 0.0)
            (Variables|Default|SetRoom_CenterB _array_element_2)
            (goto _label_2))))
      (:Completed
        (CallFunction|GeneratePathBetween2Rooms))))
  (Default|GameReturnSeed (Variables|Default|GetGameInstance) (Variables|Default|GetRoomSeed))
  (Game|SpawnActorfromClass "/Game/CustomContent/TBOS/saber/Blueprints/DungeonCreation/saber_wallCreator.saber_wallCreator_C" (Math|Transform|MakeTransform "0, 0, 0") "Undefined" 0 (Variables|Default|GetCorridors) 0))

(fn ConstructionScript)

(fn GeneratePathBetween2Rooms
  ;[1 0.1621 0] TO DO: weighted randomize for B, Weighted randomize of continuing A
  (LocalVariables|SetClosest_Entry_Point_Distance 1e+06)
  (for _array_element (Variables|/Game/CustomContent/TBOS/saber/Blueprints/RoomBP/Room_Center.Room_Center_C|GetRoomEntryPoints (Variables|Default|GetRoom_CenterA))
    ;;[1 1 1] find closest B entry point (in the connecting room)
    (for _array_element_2 (Variables|/Game/CustomContent/TBOS/saber/Blueprints/RoomBP/Room_Center.Room_Center_C|GetRoomEntryPoints (Variables|Default|GetRoom_CenterB))
      (if (< (Transformation|GetHorizontalDistanceTo _array_element_2 _array_element) 0.0)
        (Development|PrintString (Utilities|String|Append "NegativeDistance: " (Utilities|String|ToString(Float) (Transformation|GetHorizontalDistanceTo _array_element_2 _array_element))) true true "(R=0.969245,G=1.000000,B=0.151953,A=1.000000)" 3e+01))
      (bind _output_get (LocalVariables|SetClosest_Entry_Point_Distance (Math|Float|Min(Float) (Transformation|GetHorizontalDistanceTo _array_element_2 _array_element) (LocalVariables|GetClosest_Entry_Point_Distance))))
      (if (== _output_get (Transformation|GetHorizontalDistanceTo _array_element_2 _array_element))
        (LocalVariables|SetClosest_EntryPointB _array_element_2)
        (LocalVariables|SetEntryPointA _array_element))))
  ;[1 1 1] Extends start/endpoint past room entry point a bit
  (CallFunction|SpawnIndividualSpline (+ (Transformation|GetActorLocation (LocalVariables|GetClosest_EntryPointB)) (* (Transformation|GetActorForwardVector (LocalVariables|GetClosest_EntryPointB)) 400)) (Transformation|GetActorLocation (LocalVariables|GetClosest_EntryPointB)) "/Game/CustomContent/TBOS/saber/Test/Test_SplinePath_End.Test_SplinePath_End_C")
  (Utilities|Array|Add (Variables|Default|GetCorridors) (Utilities|Struct|MakePathStruct (+ (Transformation|GetActorLocation (LocalVariables|GetClosest_EntryPointB)) (* (Transformation|GetActorForwardVector (LocalVariables|GetClosest_EntryPointB)) 400)) (Transformation|GetActorLocation (LocalVariables|GetClosest_EntryPointB))))
  (Rendering|Debug|DrawDebugBox (+ (Transformation|GetActorLocation (LocalVariables|GetClosest_EntryPointB)) (* (Transformation|GetActorForwardVector (LocalVariables|GetClosest_EntryPointB)) 400)) "10.000000,10.000000,100.000000" "(R=0.157399,G=1.000000,B=0.000000,A=1.000000)" "0, 0, 0" 1.2e+02 3.0)
  (bind _output_get_2 (Variables|Default|Setendpoint_global (+ (Transformation|GetActorLocation (LocalVariables|GetClosest_EntryPointB)) (* (Transformation|GetActorForwardVector (LocalVariables|GetClosest_EntryPointB)) 400))))
  (Variables|Default|SetX%20Target (.X (Math|Vector|BreakVector _output_get_2)))
  (Variables|Default|SetY%20Target (.Y (Math|Vector|BreakVector _output_get_2)))
  (bind _output_get_3 (Variables|Default|SetCurrent_StopPoint (Transformation|GetActorLocation (LocalVariables|GetEntryPointA))))
  (CallFunction|SpawnIndividualSpline _output_get_3 (+ _output_get_3 (* (Transformation|GetActorForwardVector (LocalVariables|GetEntryPointA)) 400)) "/Game/CustomContent/TBOS/saber/Test/Test_SplinePath_Start.Test_SplinePath_Start_C")
  (Utilities|Array|Add (Variables|Default|GetCorridors) (Utilities|Struct|MakePathStruct _output_get_3 (+ _output_get_3 (* (Transformation|GetActorForwardVector (LocalVariables|GetEntryPointA)) 400))))
  (bind _output_get_4 (Variables|Default|SetCurrent_StopPoint (+ _output_get_3 (* (Transformation|GetActorForwardVector (LocalVariables|GetEntryPointA)) 400))))
  (Rendering|Debug|DrawDebugBox _output_get_4 "10.000000,10.000000,100.000000" "(R=0.157399,G=1.000000,B=0.000000,A=1.000000)" "0, 0, 0" 1.2e+02 3.0)
  (Variables|Default|SetCurrent_YStopPoint (.Y (Math|Vector|BreakVector _output_get_4)))
  (Variables|Default|SetCurrent_XStopPoint (.X (Math|Vector|BreakVector _output_get_4)))
  (Default|OpenEntryDoors (LocalVariables|GetEntryPointA))
  (while (Math|Vector|NotEqual(Vector) (Variables|Default|GetCurrent_StopPoint) (Variables|Default|Getendpoint_global) 0.0)
    ;[1 1 1] Random works towards x or Y
    (if (== (Variables|Default|GetX%20Target) (Variables|Default|GetCurrent_XStopPoint))
      (CallFunction|FindNextPathLine-Y :!label _label)
      (else
        (if (== (Variables|Default|GetCurrent_YStopPoint) (Variables|Default|GetY%20Target))
          _
          (else
            (switch int (Math|Random|RandomIntegerinRangefromStream 0 1 (Variables|Default|GetRoomSeed))
              (:0
                _)
              (:1
                (goto _label)))))
        (CallFunction|FindNextPathLine-X)))))

(fn SpawnIndividualSpline
  (params (StartPoint1 :type Vector) (EndPoint1 :type Vector) (Class :type Actor%20Class%20Reference))
  (LocalVariables|SetStartPoint StartPoint1)
  (LocalVariables|SetEndPoint EndPoint1)
  (Rendering|Debug|DrawDebugLine (LocalVariables|GetStartPoint) (LocalVariables|GetEndPoint) "(R=0.966223,G=0.021443,B=1.000000,A=1.000000)" 1.2e+02 5.0)
  (if (< (Math|Float|Absolute(Float) (Math|Vector|VectorLength (- (LocalVariables|GetStartPoint) (LocalVariables|GetEndPoint)))) 1.0)
    (return)
    (else
      (bind _returnvalue (Game|SpawnActorfromClass Class (Math|Transform|MakeTransform (LocalVariables|GetStartPoint)) "Undefined" 0 0))
      (bind _astest_spline_path (Utilities|Casting|CastToTest_SplinePath _returnvalue))
      (Transformation|SetWorldRotation (Variables|/Game/CustomContent/TBOS/saber/Test/Test_SplinePath.Test_SplinePath_C|GetSplineMesh _astest_spline_path) (Math|Rotator|FindLookatRotation (LocalVariables|GetStartPoint) (LocalVariables|GetEndPoint)) false false)
      (SplineMesh|SetEndPosition (Variables|/Game/CustomContent/TBOS/saber/Test/Test_SplinePath.Test_SplinePath_C|GetSplineMesh _astest_spline_path) (Math|Vector|MakeVector (Math|Vector|VectorLength (- (LocalVariables|GetEndPoint) (LocalVariables|GetStartPoint))) 0.0 0.0) true)
      (Utilities|Array|Add (Variables|Default|GetPathSplines) _astest_spline_path)
      (return))))

(fn FindNextPathLine-Y
  (bind _y_target (Variables|Default|GetY%20Target))
  ;[1 1 1] Check if Path would Hit something
  (bind (_outhit _returnvalue) (Collision|LineTraceForObjects (Variables|Default|GetCurrent_StopPoint) (Math|Vector|MakeVector (.X (Math|Vector|BreakVector (Variables|Default|GetCurrent_StopPoint))) _y_target (.Z (Math|Vector|BreakVector (Variables|Default|GetCurrent_StopPoint)))) (Utilities|Array|MakeArray "ObjectTypeQuery1") false (Variables|Default|GetPathSplines) "None"))
  (if _returnvalue
    ;[1 0.1709 0.1012] Checks if Path would not move forward at all
    (if (Math|Vector|Equal(Vector) (+ (* (Math|Vector|GetUnitDirection(Vector) (.Location (Collision|BreakHitResult _outhit)) (Variables|Default|GetCurrent_StopPoint)) 250) (.Location (Collision|BreakHitResult _outhit))) (Variables|Default|GetCurrent_StopPoint) 0.0001)
      (CallFunction|FindOverextension (.Location (Collision|BreakHitResult _outhit)))
      (else
        (Variables|Default|SetCurrentTarget (+ (* (Math|Vector|GetUnitDirection(Vector) (.Location (Collision|BreakHitResult _outhit)) (Variables|Default|GetCurrent_StopPoint)) 250) (.Location (Collision|BreakHitResult _outhit))))
        (Variables|Default|SetCurrent_YStopPoint (.Y (Math|Vector|BreakVector (+ (* (Math|Vector|GetUnitDirection(Vector) (.Location (Collision|BreakHitResult _outhit)) (Variables|Default|GetCurrent_StopPoint)) 250) (.Location (Collision|BreakHitResult _outhit))))))
        ;[0.8829 1 0.2782] If path can move forward, move forward until 250 steps away from hit location, then go other way
        (CallFunction|SpawnIndividualSpline (Variables|Default|GetCurrent_StopPoint) (Variables|Default|GetCurrentTarget) "/Game/CustomContent/TBOS/saber/Test/Test_SplinePath.Test_SplinePath_C")
        (Utilities|Array|Add (Variables|Default|GetCorridors) (Utilities|Struct|MakePathStruct (Variables|Default|GetCurrent_StopPoint) (Variables|Default|GetCurrentTarget)))
        (Variables|Default|SetCurrent_StopPoint (Variables|Default|GetCurrentTarget))
        (CallFunction|FindNextPathLine-X)))
    (else
      (Variables|Default|SetCurrentTarget (Math|Vector|MakeVector (.X (Math|Vector|BreakVector (Variables|Default|GetCurrent_StopPoint))) _y_target (.Z (Math|Vector|BreakVector (Variables|Default|GetCurrent_StopPoint)))))
      ;[0.4437 1 0.3343] Path can move forward all the way to goal
      (Variables|Default|SetCurrent_YStopPoint _y_target)
      (CallFunction|SpawnIndividualSpline (Variables|Default|GetCurrent_StopPoint) (Variables|Default|GetCurrentTarget) "/Game/CustomContent/TBOS/saber/Test/Test_SplinePath.Test_SplinePath_C")
      (Utilities|Array|Add (Variables|Default|GetCorridors) (Utilities|Struct|MakePathStruct (Variables|Default|GetCurrent_StopPoint) (Variables|Default|GetCurrentTarget)))
      (Variables|Default|SetCurrent_StopPoint (Variables|Default|GetCurrentTarget))
      (return))))

(fn FindNextPathLine-X
  (bind _x_target (Variables|Default|GetX%20Target))
  ;[1 1 1] Check if Path would Hit something
  (bind (_outhit _returnvalue) (Collision|LineTraceForObjects (Variables|Default|GetCurrent_StopPoint) (Math|Vector|MakeVector _x_target (.Y (Math|Vector|BreakVector (Variables|Default|GetCurrent_StopPoint))) (.Z (Math|Vector|BreakVector (Variables|Default|GetCurrent_StopPoint)))) (Utilities|Array|MakeArray "ObjectTypeQuery1" "ObjectTypeQuery2") false (Variables|Default|GetPathSplines) "None"))
  (if _returnvalue
    ;[1 0.1709 0.1012] Checks if Path would not move forward at all
    (if (Math|Vector|Equal(Vector) (+ (* (Math|Vector|GetUnitDirection(Vector) (.Location (Collision|BreakHitResult _outhit)) (Variables|Default|GetCurrent_StopPoint)) 250) (.Location (Collision|BreakHitResult _outhit))) (Variables|Default|GetCurrent_StopPoint) 0.0001)
      (Variables|Default|SetOverExtend? true)
      (CallFunction|FindOverextension (.Location (Collision|BreakHitResult _outhit)))
      (else
        (Variables|Default|SetCurrentTarget (+ (* (Math|Vector|GetUnitDirection(Vector) (.Location (Collision|BreakHitResult _outhit)) (Variables|Default|GetCurrent_StopPoint)) 250) (.Location (Collision|BreakHitResult _outhit))))
        ;[0.8829 1 0.2782] If path can move forward, move forward until 250 steps away from hit location, then go other way
        (Variables|Default|SetCurrent_XStopPoint (.X (Math|Vector|BreakVector (+ (* (Math|Vector|GetUnitDirection(Vector) (.Location (Collision|BreakHitResult _outhit)) (Variables|Default|GetCurrent_StopPoint)) 250) (.Location (Collision|BreakHitResult _outhit))))))
        (CallFunction|SpawnIndividualSpline (Variables|Default|GetCurrent_StopPoint) (Variables|Default|GetCurrentTarget) "/Game/CustomContent/TBOS/saber/Test/Test_SplinePath.Test_SplinePath_C")
        (Utilities|Array|Add (Variables|Default|GetCorridors) (Utilities|Struct|MakePathStruct (Variables|Default|GetCurrent_StopPoint) (Variables|Default|GetCurrentTarget)))
        (Variables|Default|SetCurrent_StopPoint (Variables|Default|GetCurrentTarget))
        (CallFunction|FindNextPathLine-Y)))
    (else
      ;[0.4437 1 0.3343] Path can move forward all the way to goal
      (Variables|Default|SetCurrentTarget (Math|Vector|MakeVector _x_target (.Y (Math|Vector|BreakVector (Variables|Default|GetCurrent_StopPoint))) (.Z (Math|Vector|BreakVector (Variables|Default|GetCurrent_StopPoint)))))
      (Variables|Default|SetCurrent_XStopPoint _x_target)
      (CallFunction|SpawnIndividualSpline (Variables|Default|GetCurrent_StopPoint) (Variables|Default|GetCurrentTarget) "/Game/CustomContent/TBOS/saber/Test/Test_SplinePath.Test_SplinePath_C")
      (Utilities|Array|Add (Variables|Default|GetCorridors) (Utilities|Struct|MakePathStruct (Variables|Default|GetCurrent_StopPoint) (Variables|Default|GetCurrentTarget)))
      (Variables|Default|SetCurrent_StopPoint (Variables|Default|GetCurrentTarget))
      (return))))

(fn CreateOverExtend
  (bind _currenttarget (Variables|Default|GetCurrentTarget))
  (bind _currenttarget_2 (Variables|Default|GetCurrentTarget))
  (bind (_x _y) (Math|Vector|BreakVector _currenttarget))
  (Variables|Default|SetCurrent_YStopPoint _y)
  (Variables|Default|SetCurrent_XStopPoint _x)
  (CallFunction|SpawnIndividualSpline (Variables|Default|GetCurrent_StopPoint) _currenttarget_2 "/Game/CustomContent/TBOS/saber/Test/Test_SplinePath.Test_SplinePath_C")
  (Utilities|Array|Add (Variables|Default|GetCorridors) (Utilities|Struct|MakePathStruct (Variables|Default|GetCurrent_StopPoint) _currenttarget_2))
  (Variables|Default|SetCurrent_StopPoint (Variables|Default|GetCurrentTarget))
  (return))

(fn FindOverextension
  (params (LineHitLocation :type Vector))
  (bind _output_get (LocalVariables|SetinitialHitLoc LineHitLocation))
  ;[1 1 1] Check to see if there is anything colliding 2000 to the opposite axis in order to go around hit object
  (bind _returnvalue (Collision|LineTraceForObjects (Variables|Default|GetCurrent_StopPoint) (+ (* (Math|Vector|CrossProduct (Math|Vector|GetUnitDirection(Vector) (Variables|Default|GetCurrent_StopPoint) _output_get) "0, 0,1.000000") 2000) (Variables|Default|GetCurrent_StopPoint)) (Utilities|Array|MakeArray "ObjectTypeQuery1" "ObjectTypeQuery2") false (Variables|Default|GetPathSplines) "None"))
  (if _returnvalue
    ;[1 1 1] What happens if there is stuff to both the left and right of hit room? Excellent question...hopefully rooms can't be generated that close enough
    (LocalVariables|Setsidemove -200)
    (bind _isinroom (CallFunction|RoomBoundariesCheck (+ (* (Math|Vector|CrossProduct (Math|Vector|GetUnitDirection(Vector) (Variables|Default|GetCurrent_StopPoint) (LocalVariables|GetinitialHitLoc)) "0, 0,1.000000") (LocalVariables|Getsidemove)) (Variables|Default|GetCurrent_StopPoint) (* (Math|Vector|GetUnitDirection(Vector) (Variables|Default|GetCurrent_StopPoint) (LocalVariables|GetinitialHitLoc)) 2.5e+02)) :!label _label))
    (if _isinroom
      (LocalVariables|Setsidemove (+ (LocalVariables|Getsidemove) (LocalVariables|Getsidemove)))
      (goto _label)
      (else
        (Variables|Default|SetCurrentTarget (+ (* (Math|Vector|CrossProduct (Math|Vector|GetUnitDirection(Vector) (Variables|Default|GetCurrent_StopPoint) (LocalVariables|GetinitialHitLoc)) "0, 0,1.000000") (LocalVariables|Getsidemove)) (Variables|Default|GetCurrent_StopPoint) ""))
        (CallFunction|CreateOverExtend)))
    (else
      (LocalVariables|Setsidemove 200)
      ;[1 1 1] Checks to see if you can go forward from current point. If still stuck, move point to the "right" again, then check. Once you can move forward, go back to normal routine
      (bind _isinroom_2 (CallFunction|RoomBoundariesCheck (+ (* (Math|Vector|CrossProduct (Math|Vector|GetUnitDirection(Vector) (Variables|Default|GetCurrent_StopPoint) (LocalVariables|GetinitialHitLoc)) "0, 0,1.000000") (LocalVariables|Getsidemove)) (Variables|Default|GetCurrent_StopPoint) (* (Math|Vector|GetUnitDirection(Vector) (Variables|Default|GetCurrent_StopPoint) (LocalVariables|GetinitialHitLoc)) 2.5e+02)) :!label _label_2))
      (if _isinroom_2
        (LocalVariables|Setsidemove (+ (LocalVariables|Getsidemove) (LocalVariables|Getsidemove)))
        (goto _label_2)
        (else
          (Variables|Default|SetCurrentTarget (+ (* (Math|Vector|CrossProduct (Math|Vector|GetUnitDirection(Vector) (Variables|Default|GetCurrent_StopPoint) (LocalVariables|GetinitialHitLoc)) "0, 0,1.000000") (LocalVariables|Getsidemove)) (Variables|Default|GetCurrent_StopPoint) ""))
          (CallFunction|CreateOverExtend))))))

(fn RoomBoundariesCheck
  (params (Point :type Vector))
  (bind _array_element (Utilities|Array|ForEachLoopwithBreak (Variables|Default|GetTileMap) :!label _label)
    (:LoopBody
      (if (Math|Geometry|IsPointinBox Point (.MidPointVector (Utilities|Struct|BreakRoomStruct _array_element)) (Math|Vector|MakeVector (+ (.X (Math|Vector|BreakVector (Math|Vector|MakeVector (.X (Math|Vector2D|BreakVector2D (.RoomSizefromCenter (Utilities|Struct|BreakRoomStruct _array_element)))) (.Y (Math|Vector2D|BreakVector2D (.RoomSizefromCenter (Utilities|Struct|BreakRoomStruct _array_element)))) 0.0))) 5e+02) (+ (.Y (Math|Vector|BreakVector (Math|Vector|MakeVector (.X (Math|Vector2D|BreakVector2D (.RoomSizefromCenter (Utilities|Struct|BreakRoomStruct _array_element)))) (.Y (Math|Vector2D|BreakVector2D (.RoomSizefromCenter (Utilities|Struct|BreakRoomStruct _array_element)))) 0.0))) 5e+02) 0.0))
        (LocalVariables|SetIsInRoom? true)
        (goto _label Break)))
    (:Completed
      (return (LocalVariables|GetIsInRoom?)))))

(fn NoMSTCreateLinksBetweenClosestRooms
  (for _array_element (Variables|Default|GetRoomCenters)
    (LocalVariables|SetNO_MST_Distance 1e+05)
    (for _array_element_2 (Variables|Default|GetRoomCenters)
      (LocalVariables|SetAlreadyMatched false)
      (bind _array_element_3 (Utilities|Array|ForEachLoopwithBreak (Variables|Default|GetEdges) :!label _label)
        (:LoopBody
          (if (or (and (Math|Vector|Equal(Vector) (.A (Utilities|Struct|BreakEdge+Distance _array_element_3)) (Math|Conversions|ToVector2D(Vector) (Transformation|GetActorLocation _array_element)) 0.0001) (Math|Vector|Equal(Vector) (.B (Utilities|Struct|BreakEdge+Distance _array_element_3)) (Math|Conversions|ToVector2D(Vector) (Transformation|GetActorLocation _array_element_2)) 0.0001)) (and (Math|Vector|Equal(Vector) (.A (Utilities|Struct|BreakEdge+Distance _array_element_3)) (Math|Conversions|ToVector2D(Vector) (Transformation|GetActorLocation _array_element_2)) 0.0001) (Math|Vector|Equal(Vector) (.B (Utilities|Struct|BreakEdge+Distance _array_element_3)) (Math|Conversions|ToVector2D(Vector) (Transformation|GetActorLocation _array_element)) 0.0001)))
            (LocalVariables|SetAlreadyMatched true)
            (goto _label Break)))
        (:Completed
          (if (not (LocalVariables|GetAlreadyMatched))
            (if (!= _array_element_2 _array_element)
              (if (== (Math|Float|Absolute(Float) (Transformation|GetDistanceTo _array_element _array_element_2)) (Math|Float|Min(Float) (LocalVariables|GetNO_MST_Distance) (Math|Float|Absolute(Float) (Transformation|GetDistanceTo _array_element _array_element_2))))
                (LocalVariables|SetNO_MST_Distance (Math|Float|Min(Float) (LocalVariables|GetNO_MST_Distance) (Math|Float|Absolute(Float) (Transformation|GetDistanceTo _array_element _array_element_2))))
                (LocalVariables|SetRoomCenterB _array_element_2)))))))
    (Utilities|Array|Add (Variables|Default|GetEdges) (Utilities|Struct|MakeEdge+Distance (Math|Conversions|ToVector2D(Vector) (Transformation|GetActorLocation _array_element)) (Math|Conversions|ToVector2D(Vector) (Transformation|GetActorLocation (LocalVariables|GetRoomCenterB))) 0.0)))
  (return))